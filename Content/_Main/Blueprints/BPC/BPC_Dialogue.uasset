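; Dialogue component that plays timed NPC conversation lines and world quips in a W_Dialogue widget.
; A forward line trace reads the hit actor's WorldStats dialogue tag as a DT_Dialogue row, and a looping timer with delays advances its text.
; Finishing stores the response tag on the actor and can spawn a BP_ItemSpawner for quest lines.
; Quip paths match player status tags against DT_F_Traits1 traits to pick random rows.
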(event `Reset`
  ;[0 0 0] World Quip
  (`self.SetRandomQuip` (stale `reset2` _returnvalue) :!label _label))

(event `reset2`
  ;[0 0 0] World Quip
  (`self.SetDialouge` (stale `WorldDialouge` _output_get) :!label _label_2)
  (bind _returnvalue (`self.PlayerWorldStatus` (stale `WorldDialouge` WorldStat)))
  (goto _label :!via `execute`))

(event `WorldDialouge`
  (params (WorldStat :type "WorldStats Object Reference") (Target :type "Actor Object Reference"))
  ;[0 0 0] World Quip
  (if (not (`self.Quest`))
    (bind _output_get (`self.DoesWidgetExist` Target))
    (goto _label_2 :!via `execute`)))

(event `DIa`
  (bind _player (`self.Player`))
  (bind _returnvalue (`Actor.K2_GetActorLocation` _player))
  ;[0 0 0] Line Trace Event For Interaction
  (bind _outhit (`KismetSystemLibrary.LineTraceSingle` _returnvalue (+ _returnvalue (* (`SceneComponent.GetForwardVector` (`Actor.RootComponent` _player)) 1700.0)) "TraceTypeQuery1"))
  ;;[0.2396 0.1158 0.06747] Grab Tag from actor and find reff in DT
  (bind _output_get (set `self.Hit Actor` (`.HitActor` (`GameplayStatics.BreakHitResult` _outhit))))
  (bind _returnvalue_2 (`Actor.GetComponentByClass` _output_get "/Game/_Main/Blueprints/BPC/WorldStats.WorldStats_C"))
  (`/Engine/EditorBlueprintResources/StandardMacros.IsValid` _returnvalue_2
    (:`Is Valid`
      (bind ((`Dialogue` _dialogue)) (break `PlayerVariables` (`WorldStats.PlayerVariables` _returnvalue_2)))
      (if (`BlueprintGameplayTagLibrary.IsGameplayTagValid` _dialogue)
        (set `self.Row Name` (`BlueprintGameplayTagLibrary.GetTagName` _dialogue))
        (`self.InitlizeDialouge`)))))

(event `Key|E`
  (params (Key :type "Key Structure"))
  ;[0 0 0] Line Trace Event For Interaction
)

(event `InitlizeDialouge`
  ;[0 0 0] Runs The Lines of Dialouge
  (`/Engine/EditorBlueprintResources/StandardMacros.DoOnce` false :!label _label_3
    (:`Completed`
      (bind _returnvalue (`|GetDataTableRow` "/Game/_Main/Data/DT/DT_Dialogue/DT_Dialogue.DT_Dialogue" (`self.Row Name`))
        (:`then`
          (bind _returnvalue_2 (`KismetSystemLibrary.K2_SetTimerDelegate` (`|CreateDelegate` :!event `StartDIlouge`) 0.01 true))
          (set `self.Timer` _returnvalue_2)
          (bind _returnvalue_3 (`|CreateWidget` "/Game/UltimateSurvivalPack/Widget/W_Dialogue.W_Dialogue_C"))
          (set `self.DialougeUI` _returnvalue_3)
          (`UserWidget.AddToViewport` _returnvalue_3 0))))))

(event `Reset_d`
  ;[0 0 0] Runs The Lines of Dialouge
  (goto _label_3 :!via `Reset`))

(event `StartDIlouge`
  ;[0 0 0] Runs The Lines of Dialouge
  (`KismetSystemLibrary.Delay` (`self.Time`))
  (bind ((`Text_22_401F119E4F0E44204DBE8095DFE69311` _text) (`ResponceTag_53_DDD78E534C4C572115308C931D55AD91` _responcetag) (`HasQuest_47_F1514D4B4B78929C6CE7FF9E1C7E3906` _hasquest)) (break `/Game/_Main/Data/Struc/S_dialogue` (stale `InitlizeDialouge` _returnvalue)))
  (bind _output (`self.Dialouge` _text _responcetag _hasquest)
    (:`Completed`
      (if _output
        (`|SpawnActorFromClass` "/Game/UltimateSurvivalPack/Blueprints/BP_ItemSpawner.BP_ItemSpawner_C" (`KismetMathLibrary.MakeTransform` (+ (`Actor.K2_GetActorLocation` (`self.Hit Actor`)) (0.0 50.0 50.0))) "Undefined" "MultiplyWithRoot" null 120.0 null false null)))))