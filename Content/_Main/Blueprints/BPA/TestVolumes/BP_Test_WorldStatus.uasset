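; Test trigger volume that gives the player a world-status gameplay tag and reports whether they have been there before.
; On overlap it reads the WordStatus tags from the character's world stats component, then checks for GiveWorldStatus.
; A new tag is added to PlayerVariables, all tags are debug-printed and a W_TestStatChange widget names it.
; An existing tag shows a "been here before" widget instead; leaving the box removes the widget.
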(event `Explor`
  (if (`BlueprintGameplayTagLibrary.HasTag` (`self.Word Status`) (`self.GiveWorldStatus`) true)
    (`KismetSystemLibrary.Delay` 0.1)
    (bind _returnvalue (`|CreateWidget` "/Game/_Main/UI/TestValue/W_TestStatChange.W_TestStatChange_C" null (`KismetTextLibrary.Conv_StringToText` (`KismetStringLibrary.Concat_StrStr` (`KismetStringLibrary.Conv_NameToString` (`BlueprintGameplayTagLibrary.GetTagName` (`self.GiveWorldStatus`))) "/" "You have been here before"))))
    (bind _output_get (set `self.TestUI` _returnvalue))
    (`UserWidget.AddToViewport` _output_get 0)
    (else
      (`BlueprintGameplayTagLibrary.AddGameplayTag` (`self.Word Status`) (`self.GiveWorldStatus`))
      (bind _structout (setmembers `PlayerVariables` :`StructRef` (`WorldStats.PlayerVariables` (`WorldStats.FindWorldStatsComponent` (`self.As Third Person Character`))) :`WordStatus` (`self.Word Status`)))
      (for _array_element (`BlueprintGameplayTagLibrary.BreakGameplayTagContainer` (`.WordStatus` (break `PlayerVariables` _structout)))
        (`KismetSystemLibrary.PrintString` (`KismetStringLibrary.Conv_NameToString` (`BlueprintGameplayTagLibrary.GetTagName` (`BlueprintGameplayTagLibrary.MakeLiteralGameplayTag` _array_element))) true true (struct :`R` 1.0 :`G` 0.987288 :`A` 1.0) 55.0)
        (`KismetSystemLibrary.Delay` 0.1)
        (`self.ShowWidget`)))))

(event `ShowWidget`
  (bind _returnvalue (`|CreateWidget` "/Game/_Main/UI/TestValue/W_TestStatChange.W_TestStatChange_C" null (`KismetTextLibrary.Conv_NameToText` (`BlueprintGameplayTagLibrary.GetTagName` (`self.GiveWorldStatus`)))))
  (bind _output_get (set `self.TestUI` _returnvalue))
  (`UserWidget.AddToViewport` _output_get 0))

(event `self.Box.OnComponentBeginOverlap`
  (params (OverlappedComponent :type "PrimitiveComponent Object Reference") (OtherActor :type "Actor Object Reference") (OtherComp :type "PrimitiveComponent Object Reference") (OtherBodyIndex :type Integer) (bFromSweep :type Boolean) (SweepResult :type "HitResult Structure (by ref)"))
  (bind _asthird_person_character (cast `/Game/UltimateSurvivalPack/Blueprints/ThirdPersonCharacter` OtherActor))
  (set `self.As Third Person Character` _asthird_person_character)
  (set `self.Word Status` (`.WordStatus` (break `PlayerVariables` (`WorldStats.PlayerVariables` (`WorldStats.FindWorldStatsComponent` (`self.As Third Person Character`))))))
  (`KismetSystemLibrary.Delay` 0.2)
  (`self.Explor`))

(event `self.Box.OnComponentEndOverlap`
  (params (OverlappedComponent :type "PrimitiveComponent Object Reference") (OtherActor :type "Actor Object Reference") (OtherComp :type "PrimitiveComponent Object Reference") (OtherBodyIndex :type Integer))
  (cast `/Game/UltimateSurvivalPack/Blueprints/ThirdPersonCharacter` OtherActor)
  (`Widget.RemoveFromParent` (`self.TestUI`)))

(fn `UserConstructionScript`)