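; Test trigger volume that shows a W_TestChoice UI widget while a ThirdPersonCharacter is inside it.
; Box begin overlap creates the widget, stores it as TestUI and adds it to the viewport; end overlap removes it.
; Leftover, unconnected nodes for granting and clearing a gameplay ability on the player never run, and the timer and BeginPlay events are empty.
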(event `StartTimer`)

(event `ShowWidget`
  (bind _returnvalue (`|CreateWidget` "/Game/_Main/UI/TestValue/W_TestChoice.W_TestChoice_C"))
  (bind _output_get (set `self.TestUI` _returnvalue))
  (`UserWidget.AddToViewport` _output_get 0))

(event `self.Box.OnComponentBeginOverlap`
  (params (OverlappedComponent :type "PrimitiveComponent Object Reference") (OtherActor :type "Actor Object Reference") (OtherComp :type "PrimitiveComponent Object Reference") (OtherBodyIndex :type Integer) (bFromSweep :type Boolean) (SweepResult :type "HitResult Structure (by ref)"))
  (cast `/Game/UltimateSurvivalPack/Blueprints/ThirdPersonCharacter` OtherActor)
  (`self.ShowWidget`))

(event `self.Box.OnComponentEndOverlap`
  (params (OverlappedComponent :type "PrimitiveComponent Object Reference") (OtherActor :type "Actor Object Reference") (OtherComp :type "PrimitiveComponent Object Reference") (OtherBodyIndex :type Integer))
  (cast `/Game/UltimateSurvivalPack/Blueprints/ThirdPersonCharacter` OtherActor)
  (`Widget.RemoveFromParent` (`self.TestUI`)))

(fn `UserConstructionScript`)