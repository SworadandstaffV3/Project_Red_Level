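; Test trigger volume that records exploration and decision gameplay tags on the player and shows on-screen feedback.
; On box overlap it copies both tag containers from the ThirdPersonCharacter's WorldStats component, then runs the exploration and decision checks.
; Missing tags are written back to PlayerVariables; existing ones produce "already visited" or "choice made" messages.
; Messages use delayed W_TestStatChange widgets, with only the last stored one removed on exit; ability-granting nodes are unconnected.
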(event `Dec`
  (bind _decision_made (`self.Decision Made`))
  (if (or (`BlueprintGameplayTagLibrary.HasTag` _decision_made (`self.Positive`) true) (`BlueprintGameplayTagLibrary.HasTag` _decision_made (`self.NegitiveTag`) true))
    (`KismetSystemLibrary.Delay` 3.0)
    (bind _returnvalue (`|CreateWidget` "/Game/_Main/UI/TestValue/W_TestStatChange.W_TestStatChange_C" null "You have made your choice"))
    (bind _output_get (set `self.TestUI` _returnvalue))
    (`UserWidget.AddToViewport` _output_get 0)
    (else
      (`BlueprintGameplayTagLibrary.AddGameplayTag` (`self.Decision Made`) (`self.Positive`))
      (setmembers `PlayerVariables` :`StructRef` (`WorldStats.PlayerVariables` (`WorldStats.FindWorldStatsComponent` (`self.As Third Person Character`))) :`DecisionMade` (`self.Decision Made`))
      (`KismetSystemLibrary.Delay` 1.0)
      (`self.ShowWidget`))))

(event `Explor`
  (if (`BlueprintGameplayTagLibrary.HasTag` (`self.Explored Areas`) (`self.Explored`) true)
    (`KismetSystemLibrary.Delay` 0.1)
    (bind _returnvalue (`|CreateWidget` "/Game/_Main/UI/TestValue/W_TestStatChange.W_TestStatChange_C" null (`KismetTextLibrary.Conv_StringToText` (`KismetStringLibrary.Concat_StrStr` (`KismetStringLibrary.Conv_NameToString` (`BlueprintGameplayTagLibrary.GetTagName` (`self.Explored`))) "/" "You have been here before"))))
    (bind _output_get (set `self.TestUI` _returnvalue))
    (`UserWidget.AddToViewport` _output_get 0)
    (else
      (`BlueprintGameplayTagLibrary.AddGameplayTag` (`self.Explored Areas`) (`self.Explored`))
      (bind _structout (setmembers `PlayerVariables` :`StructRef` (`WorldStats.PlayerVariables` (`WorldStats.FindWorldStatsComponent` (`self.As Third Person Character`))) :`ExploredAreas` (`self.Explored Areas`)))
      (for _array_element (`BlueprintGameplayTagLibrary.BreakGameplayTagContainer` (`.ExploredAreas` (break `PlayerVariables` _structout)))
        (`KismetSystemLibrary.PrintString` (`KismetStringLibrary.Conv_NameToString` (`BlueprintGameplayTagLibrary.GetTagName` (`BlueprintGameplayTagLibrary.MakeLiteralGameplayTag` _array_element))) true true (struct :`R` 1.0 :`G` 0.987288 :`A` 1.0) 55.0)
        (`KismetSystemLibrary.Delay` 0.1)
        (`self.ShowWidget`)))))

(event `StartTimer`)

(event `ShowWidget`
  (bind _returnvalue (`|CreateWidget` "/Game/_Main/UI/TestValue/W_TestStatChange.W_TestStatChange_C" null (`KismetTextLibrary.Conv_NameToText` (`BlueprintGameplayTagLibrary.GetTagName` (`self.Positive`)))))
  (bind _output_get (set `self.TestUI` _returnvalue))
  (`UserWidget.AddToViewport` _output_get 0))

(event `self.Box.OnComponentBeginOverlap`
  (params (OverlappedComponent :type "PrimitiveComponent Object Reference") (OtherActor :type "Actor Object Reference") (OtherComp :type "PrimitiveComponent Object Reference") (OtherBodyIndex :type Integer) (bFromSweep :type Boolean) (SweepResult :type "HitResult Structure (by ref)"))
  (bind ((`DecisionMade` _decisionmade) (`ExploredAreas` _exploredareas)) (break `PlayerVariables` (`WorldStats.PlayerVariables` (`WorldStats.FindWorldStatsComponent` (`self.As Third Person Character`)))))
  (bind _asthird_person_character (cast `/Game/UltimateSurvivalPack/Blueprints/ThirdPersonCharacter` OtherActor))
  (set `self.As Third Person Character` _asthird_person_character)
  (set `self.Decision Made` _decisionmade)
  (set `self.Explored Areas` _exploredareas)
  (`KismetSystemLibrary.Delay` 0.2)
  (`self.Explor`)
  (`self.Dec`))

(event `self.Box.OnComponentEndOverlap`
  (params (OverlappedComponent :type "PrimitiveComponent Object Reference") (OtherActor :type "Actor Object Reference") (OtherComp :type "PrimitiveComponent Object Reference") (OtherBodyIndex :type Integer))
  (cast `/Game/UltimateSurvivalPack/Blueprints/ThirdPersonCharacter` OtherActor)
  (`Widget.RemoveFromParent` (`self.TestUI`)))

(fn `UserConstructionScript`)