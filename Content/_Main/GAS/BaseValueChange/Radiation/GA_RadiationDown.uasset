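; Gameplay ability that steadily lowers the player's radiation level, with a test widget showing the value.
; On activation it commits and starts a looping short-interval timer for the decrement logic.
; RadiationStuff decrements RadiationLevel in the player pawn's WorldStats component BaseValues, then writes the text to the first W_TestStatChange widget found.
; The ability never clears the timer or ends itself, and applies no lower limit.
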(event `self.K2_ActivateAbility`
  (`self.K2_CommitAbility`)
  (`KismetSystemLibrary.K2_SetTimerDelegate` (`|CreateDelegate` :!event `RadiationStuff`) 0.1 true))

(event `RadiationStuff`
  (bind _basevalues (`WorldStats.BaseValues` (`WorldStats.FindWorldStatsComponent` (`GameplayStatics.GetPlayerPawn` 0))))
  (bind _result (`/Engine/EditorBlueprintResources/StandardMacros.DecrementFloat` (`.RadiationLevel` (break `BaseValues` _basevalues)))
    (:`  `
      (bind _structout (setmembers `BaseValues` :`StructRef` _basevalues :`RadiationLevel` _result))
      (bind _foundwidgets (`WidgetBlueprintLibrary.GetAllWidgetsOfClass` "/Game/_Main/UI/TestValue/W_TestStatChange.W_TestStatChange_C"))
      (set `/Game/_Main/UI/TestValue/W_TestStatChange.Textstuff` (`KismetTextLibrary.Conv_StringToText` (`KismetStringLibrary.Concat_StrStr` "Radiation:  " (`KismetStringLibrary.Conv_DoubleToString` (`.RadiationLevel` (break `BaseValues` _structout))))) (`|GetArrayItem` _foundwidgets)))))