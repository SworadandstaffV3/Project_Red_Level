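; Base AI character Blueprint for enemies, handling damage, death, team ID and target marker info.
; Damage goes through CAIDataComponent; on death a one-shot multicast ragdolls the mesh from the pelvis and sets a short lifespan, crediting the instigator via BPTargetComponent for point damage.
; Local proximity overlap toggles the info widget and target component.
; On the server it registers as a navigation invoker and asks its spawner to respawn it when destroyed.
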(event `/Game/UltimateSurvivalPack/Blueprints/Interface/BPI_InventorySystem.Local Overlap`
  (params (Overlap :type Boolean))
  (bind _returnvalue (`GameplayStatics.GetPlayerCharacter` 0))
  (bind _c_ai_datacomponent (`self.C_AI_DataComponent`))
  (bind _bp_targetcomponent (`self.BP_TargetComponent`))
  ;[0 0 0] Show/Hide Enemy Info Widget
  (if Overlap
    (`/Game/UltimateSurvivalPack/Blueprints/Components/BP_AI_DataComponent.Widget Visibility` _c_ai_datacomponent "NewEnumerator0")
    (`/Game/UltimateSurvivalPack/Blueprints/Components/BP_TargetComponent.Overlap` _bp_targetcomponent _returnvalue true)
    (else
      (`/Game/UltimateSurvivalPack/Blueprints/Components/BP_AI_DataComponent.Widget Visibility` _c_ai_datacomponent "NewEnumerator1")
      (`/Game/UltimateSurvivalPack/Blueprints/Components/BP_TargetComponent.Overlap` _bp_targetcomponent _returnvalue false))))

(event `self.ReceiveBeginPlay`
  ;[0 0 0] Refresh Collision Overlaps At Beggining
  (`/Engine/EditorBlueprintResources/ActorMacros.Switch Has Authority`
    (:`Authority`
      (`NavigationSystemV1.RegisterNavigationInvoker` (`NavigationSystemV1.GetNavigationSystem`) self 2500.0 4000.0))))

(event `MULTICAST Play Montage`
  (params (AnimMontage :type "AnimMontage Object Reference"))
  ;[1 1 1] Multicast Play Anim Montage
  (`self.PlayAnimMontage` AnimMontage))

(event `/Game/UltimateSurvivalPack/Blueprints/Interface/BPI_AI.On Dead`
  ;[1 1 1] On Enemy Death Call, stop movement and logic
  (`MovementComponent.StopMovementImmediately` (`self.CharacterMovement`))
  (`BrainComponent.StopLogic` (`AIController.BrainComponent` (`AIBlueprintHelperLibrary.GetAIController` self)) "Death"))

(event `self.ReceivePointDamage`
  (params (Damage :type "Float (single-precision)") (DamageType :type "DamageType Object Reference") (HitLocation :type "Vector Structure") (HitNormal :type "Vector Structure") (HitComponent :type "PrimitiveComponent Object Reference") (BoneName :type Name) (ShotFromDirection :type "Vector Structure") (InstigatedBy :type "Controller Object Reference") (DamageCauser :type "Actor Object Reference") (HitInfo :type "HitResult Structure (by ref)"))
  ;[0 0 0] Handle Damage Event
  (`/Game/UltimateSurvivalPack/Blueprints/Components/BP_AI_DataComponent.On Point Damage` (`self.C_AI_DataComponent`) Damage DamageType InstigatedBy DamageCauser HitInfo)
  (if (not (`/Game/UltimateSurvivalPack/Blueprints/Components/BP_AI_DataComponent.Is Alive` (`self.C_AI_DataComponent`))) :!label _label
    (`/Engine/EditorBlueprintResources/StandardMacros.DoOnce` false
      (:`Completed`
        (`/Engine/EditorBlueprintResources/StandardMacros.IsValid` (stale `self.ReceiveAnyDamage` InstigatedBy)
          (:`Is Valid`
            (`/Game/UltimateSurvivalPack/Blueprints/Components/BP_TargetComponent.Interacted` (`self.BP_TargetComponent`) (stale `self.ReceiveAnyDamage` InstigatedBy)))
          (:`Is Not Valid`
            _))
        (`self.SetLifeSpan` 3.0)
        (`self.MULTICAST On Dead`)))))

(event `self.ReceiveAnyDamage`
  (params (Damage :type "Float (single-precision)") (DamageType :type "DamageType Object Reference") (InstigatedBy :type "Controller Object Reference") (DamageCauser :type "Actor Object Reference"))
  ;[0 0 0] Handle Damage Event
  (goto _label))

(event `MULTICAST On Dead`
  (bind _capsulecomponent (`self.CapsuleComponent`))
  (bind _mesh (`self.Mesh`))
  ;[0.3932 0.8798 1] On Enemy Dead (MULTICAST)
  (`SkeletalMeshComponent.SetAllBodiesBelowSimulatePhysics` (`self.Mesh`) "Pelvis" true true)
  (`PrimitiveComponent.SetCollisionObjectType` _mesh "ECC_PhysicsBody")
  (`PrimitiveComponent.SetCollisionResponseToChannel` _mesh "ECC_GameTraceChannel1" "ECR_Ignore")
  (`PrimitiveComponent.SetCollisionResponseToChannel` _mesh "ECC_Vehicle" "ECR_Block")
  (`PrimitiveComponent.SetCollisionResponseToChannel` _mesh "ECC_GameTraceChannel4" "ECR_Ignore")
  (`PrimitiveComponent.SetCollisionResponseToAllChannels` _capsulecomponent "ECR_Ignore")
  (`PrimitiveComponent.SetCollisionResponseToChannel` _capsulecomponent "ECC_WorldStatic" "ECR_Block")
  (set `SkinnedMeshComponent.bComponentUseFixedSkelBounds` false (`self.Mesh`))
  (`CharacterMovementComponent.SetAvoidanceEnabled` (`self.CharacterMovement`) false))

(event `self.ReceiveDestroyed`
  ;[1 1 1] Inform Spawner when Destroyed
  (`parent.ReceiveDestroyed`)
  (`/Engine/EditorBlueprintResources/ActorMacros.Switch Has Authority`
    (:`Authority`
      (bind _spawner_reference (`self.Spawner Reference`)
        (:`then`
          (message `/Game/UltimateSurvivalPack/Blueprints/Interface/BPI_Spawning.Request Respawn` _spawner_reference))
        (:`else`)))))

(fn `Get Interaction Data`
  (returns (`Interaction Text` :type Text))
  (return ""))

(fn `Get Team ID`
  (returns (`Team ID` :type Byte))
  (return (`/Game/UltimateSurvivalPack/Blueprints/Components/BP_AI_DataComponent.Team ID` (`self.C_AI_DataComponent`))))

(fn `Local Can Overlap`
  (returns (Success :type Boolean))
  (return (and (< (`self.GetSquaredDistanceTo` (`Controller.K2_GetPawn` (`GameplayStatics.GetPlayerController` 0))) 640000.0) (> (`/Game/UltimateSurvivalPack/Blueprints/Components/BP_AI_DataComponent.Health` (`self.C_AI_DataComponent`)) 0.0))))

(fn `Perform AI Action`
  (params (Action :type Name))
  (returns (Success :type Boolean))
  (return false))

(fn `UserConstructionScript`
  (bind (_returnvalue_location _returnvalue_rotation _returnvalue_scale) (`KismetMathLibrary.BreakTransform` (`self.GetTransform`)))
  (bind _bp_targetcomponent (`self.BP_TargetComponent`))
  (bind (_target_information_targettype _target_information_uniqueid _target_information_amount _target_information_marker) (break `/Game/UltimateSurvivalPack/Blueprints/Structs/S_TargetInformation` (`/Game/UltimateSurvivalPack/Blueprints/Components/BP_TargetComponent.Target Information` _bp_targetcomponent)))
  (bind (_markertype _markermaterial _markertexture _alwaysonscreen _padding) (break `/Game/UltimateSurvivalPack/Blueprints/Structs/Mission/S_Marker` _target_information_marker))
  ;[1 1 1] Set Target Info Inside Construction Event
  (set `/Game/UltimateSurvivalPack/Blueprints/Components/BP_TargetComponent.Target Information` (make `/Game/UltimateSurvivalPack/Blueprints/Structs/S_TargetInformation` _target_information_targettype (`self.Unique ID`) _target_information_amount (make `/Game/UltimateSurvivalPack/Blueprints/Structs/Mission/S_Marker` _markertype _markermaterial _markertexture _alwaysonscreen (* _padding _returnvalue_scale)) self) _bp_targetcomponent))