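; Behavior tree service that turns an AI pawn, by its name a zombie, to face its current enemy target at close range.
; Each tick it reads the target from the pawn's BP_AI_DataComponent, which it looks up and caches when not yet valid.
; When the target passes a squared-distance check, it smoothly interpolates the pawn's yaw toward it, keeping pitch and roll unchanged.
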(event `self.ReceiveTickAI`
  (params (OwnerController :type "AIController Object Reference") (ControlledPawn :type "Pawn Object Reference") (DeltaSeconds :type "Float (single-precision)"))
  (bind _returnvalue (`Actor.K2_GetActorRotation` ControlledPawn))
  (`self.AI Component`
    (:`then`
      (bind _current_enemy_target (`/Game/UltimateSurvivalPack/Blueprints/Components/BP_AI_DataComponent.Current Enemy Target` (`self.AI Component`))
        (:`then`
          (if (< (`Actor.GetSquaredDistanceTo` ControlledPawn _current_enemy_target) 10000.0)
            (bind (_returnvalue_roll _returnvalue_pitch _returnvalue_yaw) (`KismetMathLibrary.BreakRotator` (`KismetMathLibrary.FindLookAtRotation` (`Actor.K2_GetActorLocation` ControlledPawn) (`Actor.K2_GetActorLocation` _current_enemy_target))))
            (`Actor.K2_SetActorRotation` ControlledPawn (`KismetMathLibrary.RInterpTo` _returnvalue (`KismetMathLibrary.MakeRotator` (.roll _returnvalue) (.pitch _returnvalue) _returnvalue_yaw) (`GameplayStatics.GetWorldDeltaSeconds`) 10.0) false)))
        (:`else`)))
    (:`else`
      (set `self.AI Component` (`Actor.GetComponentByClass` ControlledPawn "/Game/UltimateSurvivalPack/Blueprints/Components/BP_AI_DataComponent.BP_AI_DataComponent_C")))))