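; Behavior tree decorator that passes when the AI pawn is facing its blackboard Target and is close enough to it.
; It compares the pawn's yaw with the look-at yaw against TargetForwardAngle, using a raw difference without angle wrapping.
; It also checks squared distance against TargetDistance, or against a fixed 250-unit range to the attach parent when the target is attached.
; An invalid target fails the check.
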(fn `PerformConditionCheckAI`
  (params (OwnerController :type "AIController Object Reference") (ControlledPawn :type "Pawn Object Reference"))
  (returns (ReturnValue :type Boolean))
  (bind (_returnvalue_roll _returnvalue_pitch _returnvalue_yaw) (`KismetMathLibrary.BreakRotator` (`Actor.K2_GetActorRotation` ControlledPawn)))
  (bind _target_distance (`self.Target Distance`))
  (bind _returnvalue (`BTFunctionLibrary.GetBlackboardValueAsActor` (`self.Target`)))
  (bind _returnvalue_2 (`Actor.GetAttachParentActor` _returnvalue))
  (bind (_returnvalue_roll_2 _returnvalue_pitch_2 _returnvalue_yaw_2) (`KismetMathLibrary.BreakRotator` (`KismetMathLibrary.FindLookAtRotation` (`Actor.K2_GetActorLocation` ControlledPawn) (`Actor.K2_GetActorLocation` _returnvalue))))
  (bind _returnvalue_3 (`KismetSystemLibrary.IsValid` _returnvalue_2))
  (`/Engine/EditorBlueprintResources/StandardMacros.IsValid` _returnvalue
    (:`Is Valid`
      (return (and (< (`KismetMathLibrary.Abs` (- _returnvalue_yaw _returnvalue_yaw_2)) (`self.Target Forward Angle`)) (< (`Actor.GetSquaredDistanceTo` ControlledPawn (select `bool` _returnvalue_3 :`false` _returnvalue :`true` _returnvalue_2)) (select `bool` _returnvalue_3 :`false` (* _target_distance _target_distance) :`true` 62500.0)))))
    (:`Is Not Valid`
      (return false))))