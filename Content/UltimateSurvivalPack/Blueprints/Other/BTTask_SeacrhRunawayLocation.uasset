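; Behavior Tree task that picks a blackboard destination for an AI running away from the StartingFrom actor or location.
; It samples random reachable navmesh points directly away, left, right, then toward the threat, failing if none passes the path check.
; While running, it searches again when the pawn nears the destination or has no move destination.
; Each check re-rolls the random point, so the stored location can differ from the validated one.
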(event `self.ReceiveExecuteAI`
  (params (OwnerController :type "AIController Object Reference") (ControlledPawn :type "Pawn Object Reference"))
  (bind _starting_from (`self.Starting From`))
  (`self.Search for Location` ControlledPawn)
  (if (not (or (`KismetSystemLibrary.IsValid` (`BTFunctionLibrary.GetBlackboardValueAsActor` _starting_from)) (`AIBlueprintHelperLibrary.IsValidAILocation` (`BTFunctionLibrary.GetBlackboardValueAsVector` _starting_from))))
    (`self.FinishExecute` true)))

(event `self.ReceiveTickAI`
  (params (OwnerController :type "AIController Object Reference") (ControlledPawn :type "Pawn Object Reference") (DeltaSeconds :type "Float (single-precision)"))
  (if (or (< (`KismetMathLibrary.Vector_Distance` (`BTFunctionLibrary.GetBlackboardValueAsVector` (`self.Desired Location Key`)) (`Actor.K2_GetActorLocation` ControlledPawn)) 200.0) (== (`AIController.GetImmediateMoveDestination` OwnerController) (0.0 0.0 0.0)))
    (`self.Search for Location` ControlledPawn)))

(fn `Search for Location`
  (params (`Controlled Pawn` :type "Actor Object Reference (by ref)"))
  (locals (`L Target Loc` :type "Vector Structure"))
  (bind _returnvalue (`Actor.K2_GetActorLocation` `Controlled Pawn`))
  (bind _returnvalue_2 (`Actor.K2_GetActorLocation` `Controlled Pawn`))
  (bind _returnvalue_3 (`Actor.K2_GetActorLocation` `Controlled Pawn`))
  (bind _starting_from (`self.Starting From`))
  (bind _desired_getaway_distance (`self.Desired Getaway Distance`))
  (bind _returnvalue_4 (`BTFunctionLibrary.GetBlackboardValueAsActor` _starting_from))
  (bind _returnvalue_5 (`KismetMathLibrary.FindLookAtRotation` (`Actor.K2_GetActorLocation` `Controlled Pawn`) (`local.L Target Loc`)))
  (bind _returnvalue_6 (`KismetMathLibrary.GetRightVector` _returnvalue_5))
  (bind (_randomlocation _returnvalue_7) (`NavigationSystemV1.K2_GetRandomReachablePointInRadius` (+ _returnvalue (* _returnvalue_6 (* (`self.Desired Getaway Distance`) -1.25))) _desired_getaway_distance null null))
  (bind (_randomlocation_2 _returnvalue_8) (`NavigationSystemV1.K2_GetRandomReachablePointInRadius` (+ (`Actor.K2_GetActorLocation` `Controlled Pawn`) (* (`KismetMathLibrary.GetForwardVector` _returnvalue_5) (* (`self.Desired Getaway Distance`) 1.25))) _desired_getaway_distance null null))
  (bind (_randomlocation_3 _returnvalue_9) (`NavigationSystemV1.K2_GetRandomReachablePointInRadius` (+ _returnvalue_2 (* _returnvalue_6 (* (`self.Desired Getaway Distance`) 1.25))) _desired_getaway_distance null null))
  (bind (_randomlocation_4 _returnvalue_10) (`NavigationSystemV1.K2_GetRandomReachablePointInRadius` (+ _returnvalue_3 (* (`KismetMathLibrary.GetForwardVector` _returnvalue_5) (* (`self.Desired Getaway Distance`) -1.25))) _desired_getaway_distance null null))
  (if (`KismetSystemLibrary.IsValid` _returnvalue_4)
    (set `local.L Target Loc` (`Actor.K2_GetActorLocation` _returnvalue_4))
    (else
      (set `local.L Target Loc` (`BTFunctionLibrary.GetBlackboardValueAsVector` _starting_from))))
  (if _returnvalue_10
    (if (`|EnumEquality` (`.ReturnValue` (`NavigationSystemV1.GetPathCost` _returnvalue_3 _randomlocation_4 null null)) "Success")
      (`BTFunctionLibrary.SetBlackboardValueAsVector` (`self.Desired Location Key`) _randomlocation_4)
      (return)
      (else
        _)))
  (if _returnvalue_7
    (if (`|EnumEquality` (`.ReturnValue` (`NavigationSystemV1.GetPathCost` _returnvalue _randomlocation null null)) "Success")
      (`BTFunctionLibrary.SetBlackboardValueAsVector` (`self.Desired Location Key`) _randomlocation)
      (return)
      (else
        _)))
  (if _returnvalue_9
    (if (`|EnumEquality` (`.ReturnValue` (`NavigationSystemV1.GetPathCost` _returnvalue_2 _randomlocation_3 null null)) "Success")
      (`BTFunctionLibrary.SetBlackboardValueAsVector` (`self.Desired Location Key`) _randomlocation_3)
      (return)
      (else
        _)))
  (if _returnvalue_8
    (if (`|EnumEquality` (`.ReturnValue` (`NavigationSystemV1.GetPathCost` _returnvalue_2 _randomlocation_2 null null)) "Success")
      (`BTFunctionLibrary.SetBlackboardValueAsVector` (`self.Desired Location Key`) _randomlocation_2)
      (return)
      (else
        _)))
  (`self.FinishExecute` false)
  (return))