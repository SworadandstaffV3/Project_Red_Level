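; Blueprint function library for the Ultimate Survival Pack, providing shared lookup helpers.
; Validity-checked getters return a player's or object's mission, leveling, skill tree, inventory and player components via GetComponentByClass.
; Cast-based getters fetch an AI's nametag info and the human character stored on the controller's inventory component.
; Other helpers centralise the player class, save slot names and a hard-coded list of non-saveable levels.
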(fn `Get Customization Slot Name`
  (returns (ReturnValue :type String))
  (return "SAVE_Customization"))

(fn `Get Enemy Nametag`
  (params (Object :type "Object Object Reference"))
  (returns (`Name Tag` :type "WidgetComponent Object Reference"))
  (bind _asbp_aibase (cast `/Game/UltimateSurvivalPack/Blueprints/AI/BP_AIBase` Object)
    (:`then`
      (return (`/Game/UltimateSurvivalPack/Blueprints/AI/BP_AIBase.Info` _asbp_aibase)))
    (:`CastFailed`
      (return null))))

(fn `Get Human Player Character`
  (params (Controller :type "Actor Object Reference"))
  (returns (`Human Player Character` :type "Character Object Reference"))
  (locals (NewLocalVar_0 :type "Actor Object Reference"))
  (bind _asbp_player_controller (cast `/Game/UltimateSurvivalPack/Blueprints/BP_PlayerController` Controller))
  (return (`/Game/UltimateSurvivalPack/Blueprints/Components/BP_PlayerInventoryComponent.Huma Player Character` (`/Game/UltimateSurvivalPack/Blueprints/BP_PlayerController.BP_PlayerInventoryComponent` _asbp_player_controller))))

(fn `Get Inventory Component`
  (params (`Player Controller` :type "Actor Object Reference (by ref)"))
  (returns (ReturnValue :type "/Game/UltimateSurvivalPack/Blueprints/Components/BP_PlayerInventoryComponent Object Reference"))
  (`/Engine/EditorBlueprintResources/StandardMacros.IsValid` `Player Controller`
    (:`Is Valid`
      (return (`Actor.GetComponentByClass` `Player Controller` "/Game/UltimateSurvivalPack/Blueprints/Components/BP_PlayerInventoryComponent.BP_PlayerInventoryComponent_C")))
    (:`Is Not Valid`
      (return null))))

(fn `Get Leveling Component`
  (params (Object :type "Actor Object Reference"))
  (returns (`Leveling Component` :type "/Game/UltimateSurvivalPack/Blueprints/Components/BP_Player_ExperienceComponent Object Reference"))
  (`/Engine/EditorBlueprintResources/StandardMacros.IsValid` Object
    (:`Is Valid`
      (return (`Actor.GetComponentByClass` Object "/Game/UltimateSurvivalPack/Blueprints/Components/BP_Player_ExperienceComponent.BP_Player_ExperienceComponent_C")))
    (:`Is Not Valid`
      (return null))))

(fn `Get Mission Component`
  (params (Player :type "Actor Object Reference"))
  (returns (MissionComponent :type "/Game/UltimateSurvivalPack/Blueprints/Components/BP_MissionComponent Object Reference"))
  (`/Engine/EditorBlueprintResources/StandardMacros.IsValid` Player
    (:`Is Valid`
      (return (`Actor.GetComponentByClass` Player "/Game/UltimateSurvivalPack/Blueprints/Components/BP_MissionComponent.BP_MissionComponent_C")))
    (:`Is Not Valid`
      (return null))))

(fn `Get Option Slot Name`
  (returns (ReturnValue :type String))
  (return "SAVE_Options"))

(fn `Get Player Class`
  (returns (`Player Class` :type "Character Class Reference"))
  (return "/Game/UltimateSurvivalPack/Blueprints/ThirdPersonCharacter.ThirdPersonCharacter_C"))

(fn `Get Player Component`
  (params (Character :type "Actor Object Reference"))
  (returns (ReturnValue :type "/Game/UltimateSurvivalPack/Blueprints/Components/BP_PlayerComponent Object Reference"))
  (`/Engine/EditorBlueprintResources/StandardMacros.IsValid` Character
    (:`Is Valid`
      (return (`Actor.GetComponentByClass` Character "/Game/UltimateSurvivalPack/Blueprints/Components/BP_PlayerComponent.BP_PlayerComponent_C")))
    (:`Is Not Valid`
      (return null))))

(fn `Get Skill Component`
  (params (Player :type "Actor Object Reference"))
  (returns (ReturnValue :type "/Game/UltimateSurvivalPack/Blueprints/Components/BP_SkillTreeComponent Object Reference"))
  (`/Engine/EditorBlueprintResources/StandardMacros.IsValid` Player
    (:`Is Valid`
      (return (`Actor.GetComponentByClass` Player "/Game/UltimateSurvivalPack/Blueprints/Components/BP_SkillTreeComponent.BP_SkillTreeComponent_C")))
    (:`Is Not Valid`
      (return null))))

(fn `Is Current Level Saveable`
  (returns (ReturnValue :type Boolean))
  (bind _returnvalue (`GameplayStatics.GetCurrentLevelName` null))
  (return (not (`KismetArrayLibrary.Array_Contains` (`|MakeArray` "L_Demo") _returnvalue))))