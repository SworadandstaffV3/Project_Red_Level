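; Arrow projectile actor for the survival pack that deals damage on impact and can then be picked up.
; On stop it attaches to the hit component, plays blood or smoke effects by target type, and becomes interactable.
; The authority applies point damage with random variance and doubled headshots, and destroys the arrow when its target is destroyed.
; Interacting adds an Arrow to the executor's inventory; selection toggles a custom-depth highlight.
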(event `self.ProjectileMovement.OnProjectileStop`
  (params (ImpactResult :type "HitResult Structure (by ref)"))
  (bind (_bblockinghit _binitialoverlap _time _distance _location _impactpoint _normal _impactnormal _physmat _hitactor _hitcomponent _hitbonename) (`GameplayStatics.BreakHitResult` ImpactResult))
  (bind (_bblockinghit_2 _binitialoverlap_2 _time_2 _distance_2 _location_2 _impactpoint_2 _normal_2 _impactnormal_2 _physmat_2 _hitactor_2) (`GameplayStatics.BreakHitResult` ImpactResult))
  (set `self.Interactable` true)
  (`PrimitiveComponent.SetCollisionResponseToAllChannels` (`self.Sphere`) "ECR_Ignore")
  (`self.K2_AttachToComponent` _hitcomponent _hitbonename "KeepWorld" "KeepWorld" "KeepWorld" false)
  (cast `SkeletalMeshComponent` _hitcomponent
    (:`then`
      (`NiagaraFunctionLibrary.SpawnSystemAttached` "/Game/UltimateSurvivalPack/Demo/Particles/Niagara/NS_BloodSplash.NS_BloodSplash" (`self.Sphere`) "None" (0.0 0.0 0.0) (struct) "KeepRelativeOffset")
      (`GameplayStatics.SpawnSoundAttached` "/Game/UltimateSurvivalPack/Demo/Audio/SFX/CUE_BodyHit.CUE_BodyHit" (`self.Sphere`) "None" (0.0 0.0 0.0) (struct) "KeepRelativeOffset" false 1.0 1.0 0.0 "/Game/UltimateSurvivalPack/Blueprints/Attenuation/SA_Footsteps.SA_Footsteps" null))
    (:`CastFailed`
      (`GameplayStatics.SpawnEmitterAttached` "/Game/UltimateSurvivalPack/Demo/Particles/P_ImpactSmoke.P_ImpactSmoke" (`self.Sphere`))
      (`GameplayStatics.SpawnSoundAttached` "/Game/UltimateSurvivalPack/Demo/Audio/Impact/CUE_HitImpact.CUE_HitImpact" (`self.Sphere`) "None" (0.0 0.0 0.0) (struct) "KeepRelativeOffset" false 0.5 1.0 0.0 "/Game/UltimateSurvivalPack/Blueprints/Attenuation/SA_Footsteps.SA_Footsteps" null)))
  (`/Engine/EditorBlueprintResources/ActorMacros.Switch Has Authority`
    (:`Authority`
      (add `self.OnDestroyed` _hitactor (delegate `Target Destroyed`))
      (`GameplayStatics.ApplyPointDamage` _hitactor_2 (`self.Get Damage` ImpactResult) (- (`self.K2_GetActorLocation` _hitactor_2) (`self.K2_GetActorLocation` (`self.Instigator`))) ImpactResult (cast `Controller` (`self.GetOwner`) :!pure true) self "/Game/UltimateSurvivalPack/Blueprints/DamageType/DT_Projectile.DT_Projectile_C"))))

(event `Target Destroyed` :!signature `self.OnDestroyed`
  (params (DestroyedActor :type "Actor Object Reference"))
  (`self.K2_DestroyActor`))

(event `/Game/UltimateSurvivalPack/Blueprints/Interface/BPI_InventorySystem.Toggle Selected`
  (params (Toggle :type Boolean))
  (bind _staticmesh (`self.StaticMesh`))
  (bind _staticmesh_2 (`self.StaticMesh`))
  (if (`self.Interactable`)
    (if Toggle
      (`PrimitiveComponent.SetRenderCustomDepth` _staticmesh_2 true)
      (`PrimitiveComponent.SetCustomDepthStencilValue` _staticmesh_2 1)
      (else
        (`PrimitiveComponent.SetRenderCustomDepth` _staticmesh false :!label _label)
        (`PrimitiveComponent.SetCustomDepthStencilValue` _staticmesh 0)))
    (else
      (goto _label))))

(event `/Game/UltimateSurvivalPack/Blueprints/Interface/BPI_InventorySystem.On Interacted`
  (params (Executor :type "Controller Object Reference"))
  (if (`self.Interactable`)
    (`/Game/UltimateSurvivalPack/Blueprints/Components/BP_MasterInventoryComponent.Add Item` (`/Game/UltimateSurvivalPack/Blueprints/BFL_UMSPack.Get Inventory Component` Executor) (make `/Game/UltimateSurvivalPack/Blueprints/Structs/S_InventoryItem` "Arrow" 1))
    (`self.K2_DestroyActor`)))

(fn `Get Damage`
  (params (Hit :type "HitResult Structure (by ref)"))
  (returns (ReturnValue :type "Float (double-precision)"))
  (return (* (`self.Damage`) (`KismetMathLibrary.RandomFloatInRange` (- 1.0 (`self.Random Damage Delta Multiplier`)) (+ (`self.Random Damage Delta Multiplier`) 1.0)) (select `bool` (`KismetStringLibrary.Contains` (`KismetStringLibrary.Conv_NameToString` (`.HitBoneName` (`GameplayStatics.BreakHitResult` Hit))) "Head") :`false` 1.0 :`true` 2.0 :!type "Float (single-precision)"))))

(fn `Get Interaction Data`
  (returns (`Interaction Text` :type Text))
  (return (select `bool` (`self.Interactable`) :`true` "Pick up Arrow." :!type "Text")))

(fn `Get Team ID`
  (returns (`Team ID` :type Byte))
  (return 0))

(fn `Local Can Overlap`
  (returns (Success :type Boolean))
  (return false))

(fn `UserConstructionScript`
  (`parent.UserConstructionScript`))