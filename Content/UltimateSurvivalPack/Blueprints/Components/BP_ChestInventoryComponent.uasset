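; Inventory component for storage chests in the survival game, optionally filling slots with random items from DT_ItemData on creation.
; On updates, it refreshes players viewing the chest, prunes stale viewers, and saves contents through SurvivalGamemode when the owner is a building.
; When the owner is destroyed, it closes the local player's open storage menu, and the authority moves any items into a spawned BP_StorageStash with extra slots.
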(event `Reinitialize`
  ;[1 0.1552 0.195] Initialization
  (`self.Create Inventory` :!label _label)
  (add `Actor.OnDestroyed` (`self.GetOwner`) (delegate `Event Destroyed`)))

(event `self.ReceiveBeginPlay`
  ;[1 0.1552 0.195] Initialization
  (goto _label))

(event `Event Destroyed`
  (params (DestroyedActor :type "Actor Object Reference"))
  (bind _returnvalue (`GameplayStatics.GetPlayerController` 0))
  ;[1 1 1] On Destroyed
  (if (== self (`/Game/UltimateSurvivalPack/Blueprints/Components/BP_PlayerInventoryComponent.Current Opened Storage` (`/Game/UltimateSurvivalPack/Blueprints/BFL_UMSPack.Get Inventory Component` _returnvalue)))
    (`/Game/UltimateSurvivalPack/Blueprints/Components/BP_MissionComponent.Close Inventory Menu` (`/Game/UltimateSurvivalPack/Blueprints/BFL_UMSPack.Get Mission Component` _returnvalue))))

(event `Update All Clients Inventory`
  (bind _returnvalue (`Actor.GetComponentByClass` (`self.GetOwner`) "/Game/UltimateSurvivalPack/Blueprints/Buildings/Parent/BP_BuildingComponent.BP_BuildingComponent_C"))
  (bind _build_id (`/Game/UltimateSurvivalPack/Blueprints/Buildings/Parent/BP_BuildingComponent.Build ID` _returnvalue))
  ;[1 1 1] Update Chest
  ;;[1 1 1] Update On All Clients
  (`self.Update Inventory To All Clients`)
  ;;[1 1 1] Save New Chest Data to Save Component
  (`/Engine/EditorBlueprintResources/StandardMacros.IsValid` _returnvalue
    (:`Is Valid`
      (bind _assurvival_gamemode (cast `/Game/UltimateSurvivalPack/Blueprints/SurvivalGamemode` (`GameplayStatics.GetGameMode`)))
      (bind (_saved_data _returnvalue_2) (`/Game/UltimateSurvivalPack/Blueprints/SurvivalGamemode.Get Saved Build Data` _assurvival_gamemode _build_id))
      (if _returnvalue_2
        (bind ((`BuildData_2_700EB4E148DBEF7281188785324662CA` _builddata) (`Transform_6_227D833D45720C2C90F11EB731C1BBAA` _transform) (`OnAttachedActor_9_07069BCA4FEF9223D5BEC6BA5C09F0C5` _onattachedactor) (`WorldName_11_6840022640BD07C9638712B3FDD0588F` _worldname) (`CustomFloat_21_2B1EE62141F1CF01B611A4BB124FA5E8` _customfloat) (`CustomString_25_358AA98E4F4B4693E56F5CB4422E5AF2` _customstring) (`Cupboard_28_E77CCD52410AEBABC31F47A904A01FB2` _cupboard)) (break `/Game/UltimateSurvivalPack/Blueprints/Structs/S_BuildSave` _saved_data))
        (`/Game/UltimateSurvivalPack/Blueprints/SurvivalGamemode.Save Existing Building` _assurvival_gamemode _build_id (make `/Game/UltimateSurvivalPack/Blueprints/Structs/S_BuildSave` _builddata _transform _onattachedactor _worldname (`self.Inventory`) _customfloat _customstring _cupboard (`/Game/UltimateSurvivalPack/Blueprints/Buildings/Parent/BP_BuildingComponent.Health` _returnvalue)))))))

(event `self.ReceiveEndPlay`
  (params (EndPlayReason :type "EEndPlayReason Enum" :default "Destroyed"))
  ;[1 1 1] On End Play
  (`parent.ReceiveEndPlay` EndPlayReason)
  (switch `EEndPlayReason` EndPlayReason
    (:`Destroyed`
      ;;[1 1 1] Switch on Authority
      (if (`Actor.HasAuthority` (`self.GetOwner`))
        (`self.Spawn Destroyed Items`)))))

(fn `Create Inventory`
  (bind _inventory (`self.Inventory`))
  (`parent.Create Inventory`)
  (if (> (`self.Random Loot Spawn Count`) 0)
    (bind _outrownames (`DataTableFunctionLibrary.GetDataTableRowNames` "/Game/UltimateSurvivalPack/Blueprints/Datatable/Inventory/DT_ItemData.DT_ItemData"))
    (for _index (range (`self.Random Loot Spawn Count`))
      (if (`KismetArrayLibrary.Array_IsValidIndex` _inventory _index)
        (bind _output (`|GetArrayItem` _outrownames (`KismetMathLibrary.RandomIntegerInRange` 0 (`KismetArrayLibrary.Array_LastIndex` _outrownames))))
        (`KismetArrayLibrary.Array_Set` _inventory _index (make `/Game/UltimateSurvivalPack/Blueprints/Structs/S_InventoryItem` _output (`KismetMathLibrary.RandomIntegerInRange` 1 (`.MaximumStack_21_39EA4E634AD2ADBC0EA36C92000AFBC7` (break `/Game/UltimateSurvivalPack/Blueprints/Structs/S_InventoryItemData` (`.Item Data` (`/Game/UltimateSurvivalPack/Blueprints/BFL_Inventory.Get Item Data from ID` _output))))) _index self))))))

(fn `Spawn Destroyed Items`
  ;[1 1 1] Can create death bag
  (if (`self.Has Any Items in Inventory`)
    ;[1 1 1] Spawn Storage on Controlled Pawn Loc
    (bind _returnvalue (`|SpawnActorFromClass` "/Game/UltimateSurvivalPack/Blueprints/Buildings/BP_StorageStash.BP_StorageStash_C" (`KismetMathLibrary.MakeTransform` (`Actor.K2_GetActorLocation` (`self.GetOwner`))) "AdjustIfPossibleButAlwaysSpawn" "OverrideRootScale" null null))
    (bind _bp_chestinventorycomponent (`/Game/UltimateSurvivalPack/Blueprints/Buildings/BP_StorageStash.BP_ChestInventoryComponent` _returnvalue))
    ;[1 1 1] Initialize and replace inventory
    (set `/Game/UltimateSurvivalPack/Blueprints/Components/BP_MasterInventoryComponent.Inventory Size` (+ (`self.Inventory Size`) 4) _bp_chestinventorycomponent)
    (`self.Reinitialize` _bp_chestinventorycomponent)
    (for (_array_element _array_index) (`self.Inventory`)
      (`KismetArrayLibrary.Array_Set` (`/Game/UltimateSurvivalPack/Blueprints/Components/BP_MasterInventoryComponent.Inventory` _bp_chestinventorycomponent) _array_index (make `/Game/UltimateSurvivalPack/Blueprints/Structs/S_InventoryItem` (break `/Game/UltimateSurvivalPack/Blueprints/Structs/S_InventoryItem` _array_element) (`.Amount_5_1F2975454CE296A7C7033BA39535256F` (break `/Game/UltimateSurvivalPack/Blueprints/Structs/S_InventoryItem` _array_element)) _array_index _bp_chestinventorycomponent (`.CustomInteger_14_C4B91C704D98E5A3B3B6D1B77CFE476E` (break `/Game/UltimateSurvivalPack/Blueprints/Structs/S_InventoryItem` _array_element)) (`.Durability_17_EACE862B4A67C4626DE918B12D7D20BB` (break `/Game/UltimateSurvivalPack/Blueprints/Structs/S_InventoryItem` _array_element))) true))))

(fn `Update Inventory To All Clients`
  (locals (`L Player Components` :type "Array of /Game/UltimateSurvivalPack/Blueprints/Components/BP_PlayerInventoryComponent Object Reference"))
  (bind _output_get (set `local.L Player Components` (`self.Controlling Components`)))
  ;[1 1 1] Loop each client that has interacted with chest, dump if not valid (disconnected)
  (for _array_element _output_get
    (`/Engine/EditorBlueprintResources/StandardMacros.IsValid` _array_element
      (:`Is Valid`
        (if (== (`/Game/UltimateSurvivalPack/Blueprints/Components/BP_PlayerInventoryComponent.Current Opened Storage` _array_element) self)
          (`/Game/UltimateSurvivalPack/Blueprints/Components/BP_PlayerInventoryComponent.Open Chest Inventory` _array_element self false (`self.Inventory`))
          (else
            (`KismetArrayLibrary.Array_RemoveItem` (`self.Controlling Components`) _array_element :!label _label))))
      (:`Is Not Valid`
        (goto _label))))
  (return))