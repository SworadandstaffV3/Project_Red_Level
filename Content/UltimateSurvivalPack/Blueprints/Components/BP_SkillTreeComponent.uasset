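; Controller component that runs the player's skill tree, with separate XP, levels and skill points for Survivor, Agility and Power.
; XP raises levels along a growing curve, each granting a point to unlock DataTable skills, gated by parent and cost, that set ability multipliers.
; Changes are computed locally, then pushed through server events, with saving delegated to the inventory component.
; On BeginPlay, the server restores saved data by player ID and mirrors it to the client.
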(event `SERVER Set Data`
  (params (`Current Skill Abilities` :type "/Game/UltimateSurvivalPack/Blueprints/Structs/S_CurrentSkills Structure") (`Unlocked Skills` :type "Array of /Game/UltimateSurvivalPack/Blueprints/Structs/S_SkillDatabase Structure"))
  ;[0 0 0 1 100] Skill System
  ;;[0.625 0.555 1] Update Data On Server
  (set `self.Current Skill Abilities` `Current Skill Abilities`)
  (set `self.Unlocked Skills` `Unlocked Skills`)
  (`self.Save Player Data`))

(event `Unlock Skill`
  (params (Datatable :type "DataTable Object Reference") (`Skill ID` :type Name))
  (bind _s_skilldatabase (make `/Game/UltimateSurvivalPack/Blueprints/Structs/S_SkillDatabase` Datatable `Skill ID`))
  ;[0 0 0 1 100] Skill System
  ;;[0.4471 1 0.1875] Unlock Skill
  ;;;[1 0.3646 0.3646] Can Be skill Unlocked ?
  (if (`self.Can Be Skill Unlocked?` _s_skilldatabase)
    (bind _returnvalue (`|GetDataTableRow` Datatable `Skill ID`)
      (:`then`
        (bind (_skilltype _skillpointsrequired) (break `/Game/UltimateSurvivalPack/Blueprints/Structs/S_Skill_Settings` (`.SkillSettings_5_2784FA144838FB861B8955ACE1560BFB` (break `/Game/UltimateSurvivalPack/Blueprints/Structs/S_SkillTreeMaster` _returnvalue))))
        ;;;[0.6458 0.2683 0.2554] Decrease Skill Points After Unlocking
        (`self.Add Skill Points` _skilltype (* _skillpointsrequired -1))
        ;;;[0.295 0.8495 1] Add Skill to database
        (`KismetArrayLibrary.Array_Add` (`self.Unlocked Skills`) _s_skilldatabase)
        ;;;[0.436 1 0.2545] Update Skill Abilities
        (`self.Update Skill Abilities` _returnvalue)
        ;;;[1 1 1] Update Changed Data on Server
        (`self.SERVER Set Data` (`self.Current Skill Abilities`) (`self.Unlocked Skills`))
        (`/Game/UltimateSurvivalPack/Blueprints/Components/BP_MissionComponent.CLIENT Add Notification` (`/Game/UltimateSurvivalPack/Blueprints/BFL_UMSPack.Get Mission Component` (cast `Controller` (`self.GetOwner`) :!pure true)) (make `/Game/UltimateSurvivalPack/Blueprints/Structs/S_Notification` "New Ability" "You Have Unlocked New Skill"))))))

(event `Add Skill Points`
  (params (`Skill Type` :type "/Game/UltimateSurvivalPack/Blueprints/Enum/E_SkillType Enum" :default "NewEnumerator0") (Amount :type Integer))
  (bind _returnvalue (`self.Get Skill Points` `Skill Type`))
  ;[0 0 0 1 100] Skill System
  ;;[0.224 0.9671 1 1 50] Add Skill Points
  ;;;[0.08714 0.1667 0.4427] Add Experience Points For Selected Skill Type
  (`self.Set Skill Points` `Skill Type` (+ _returnvalue Amount))
  ;;;;[1 0.7786 0.2552] Update On Server
  (`self.SERVER Set Skill Points` `Skill Type` _returnvalue))

(event `SERVER Set Skill Points`
  (params (`Skill Type` :type "/Game/UltimateSurvivalPack/Blueprints/Enum/E_SkillType Enum" :default "NewEnumerator0") (`Skill Points` :type Integer))
  ;[0 0 0 1 100] Skill System
  ;;[0.224 0.9671 1 1 50] Add Skill Points
  ;;;[0 0 0] Update Skill Points On Server
  (`self.Set Skill Points` `Skill Type` `Skill Points`)
  (`self.Save Player Data`))

(event `Add Experience`
  (params (`Skill Type` :type "/Game/UltimateSurvivalPack/Blueprints/Enum/E_SkillType Enum" :default "NewEnumerator0") (`Experience Points` :type Integer))
  ;[0 0 0 1 100] Experience System
  ;;[0.4113 0.8695 1] Add Experience Points
  (`/Game/UltimateSurvivalPack/Blueprints/Components/BP_MissionComponent.CLIENT Add Notification` (`/Game/UltimateSurvivalPack/Blueprints/BFL_UMSPack.Get Mission Component` (cast `Controller` (`self.GetOwner`) :!pure true)) (make `/Game/UltimateSurvivalPack/Blueprints/Structs/S_Notification` (`KismetTextLibrary.Conv_TextToString` (select `/Game/UltimateSurvivalPack/Blueprints/Enum/E_SkillType` `Skill Type` :`NewEnumerator0` "Survivor Experience Points" :`NewEnumerator1` "Agility Experience Points" :`NewEnumerator2` "Power Experience Points" :!type "Text")) (`KismetTextLibrary.Conv_TextToString` (`|FormatText` "+ {Amount} XP" `Experience Points`))))
  (`self.Update Experience` `Skill Type` `Experience Points`)
  ;;;[1 1 1] Update XP On Server
  (`self.SERVER Set Experience Points` `Skill Type` (`self.Get Total Experience Points` `Skill Type`)))

(event `SERVER Set Experience Points`
  (params (`Skill Type` :type "/Game/UltimateSurvivalPack/Blueprints/Enum/E_SkillType Enum" :default "NewEnumerator0") (`Experience Points` :type Integer))
  ;[0 0 0 1 100] Experience System
  ;;[1 1 1] Set Experience Point On Server
  (`self.Set Skill Experience Points` `Skill Type` `Experience Points`))

(event `SERVER Set Level`
  (params (`Skill Type` :type "/Game/UltimateSurvivalPack/Blueprints/Enum/E_SkillType Enum" :default "NewEnumerator0") (Level :type Integer))
  ;[0 0 0 1 100] Experience System
  ;;[1 1 1] Set Level On Server
  (`self.Set Skill Level` `Skill Type` Level))

(event `Event On Level Up`
  (params (`Skill Type` :type "/Game/UltimateSurvivalPack/Blueprints/Enum/E_SkillType Enum" :default "NewEnumerator0"))
  ;[0 0 0 1 100] Experience System
  ;;[1 1 1] Event On Level Up
  (`self.Add Skill Points` `Skill Type` 1) ; Add 1 Skill Point
  (`self.SERVER Set Level` `Skill Type` (`self.Get Skill Level` `Skill Type`))
  (`/Game/UltimateSurvivalPack/Blueprints/Components/BP_MissionComponent.CLIENT Add Notification` (`/Game/UltimateSurvivalPack/Blueprints/BFL_UMSPack.Get Mission Component` (cast `Controller` (`self.GetOwner`) :!pure true)) (make `/Game/UltimateSurvivalPack/Blueprints/Structs/S_Notification` (`KismetTextLibrary.Conv_TextToString` (select `/Game/UltimateSurvivalPack/Blueprints/Enum/E_SkillType` `Skill Type` :`NewEnumerator0` "Survivor Rank Up" :`NewEnumerator1` "Agility Rank Up" :`NewEnumerator2` "Power Rank Up" :!type "Text")) (`KismetTextLibrary.Conv_TextToString` (select `/Game/UltimateSurvivalPack/Blueprints/Enum/E_SkillType` `Skill Type` :`NewEnumerator0` "+ 1 Survivor Point" :`NewEnumerator1` "+ 1 Agility Point" :`NewEnumerator2` "+ 1 Power Point" :!type "Text")))))

(event `SERVER Load Skill Data`
  (bind _asbp_game_instance_umsp (cast `/Game/UltimateSurvivalPack/Blueprints/BP_GameInstance_UMSP` (`GameplayStatics.GetGameInstance`)))
  (bind (_value _returnvalue) (`BlueprintMapLibrary.Map_Find` (`/Game/UltimateSurvivalPack/Blueprints/Save/SAV_ServerData.Players Save` (`/Game/UltimateSurvivalPack/Blueprints/BP_GameInstance_UMSP.Player Save` _asbp_game_instance_umsp)) (`/Game/UltimateSurvivalPack/LobbySystem/Blueprints/BFL_LobbySystem.Get Player Unique ID` (cast `PlayerController` (`self.GetOwner`) :!pure true))))
  (if _returnvalue
    (bind ((`UnlockedSkills_41_B8BCB5884BDF059288328FAA84AC6893` _unlockedskills) (`CurrentSkillAbilities_45_15FEF461452D277B0FFC7C8602E5860E` _currentskillabilities) (`SurvivorSkillData_48_EF30E8544B42C5EC77B86194B874BA18` _survivorskilldata) (`AgilitySkillData_50_E5487CA2427A4E14DA0E0589269EAE8A` _agilityskilldata) (`PowerSkillData_52_DD714B4E417C7197B37160937B3A77EC` _powerskilldata)) (break `/Game/UltimateSurvivalPack/Blueprints/Structs/S_PlayerSave` _value))
    ;[0.6457 0.9901 1] Replicate To Owning Client
    (`self.CLIENT Load Skill Data` _unlockedskills _currentskillabilities _survivorskilldata _agilityskilldata _powerskilldata)
    ;[1 1 1] Set  General Data
    (set `self.Unlocked Skills` _unlockedskills)
    (set `self.Current Skill Abilities` _currentskillabilities)
    (bind (_skillpoints _experience _level) (break `/Game/UltimateSurvivalPack/Blueprints/Structs/S_SkillDataSave` _survivorskilldata))
    ;[1 1 1] Set Survivor Data
    (set `self.Survivor Skill Points` _skillpoints)
    (set `self.Survivor Experience Points` _experience)
    (set `self.Survivor Level` _level)
    (bind (_skillpoints_2 _experience_2 _level_2) (break `/Game/UltimateSurvivalPack/Blueprints/Structs/S_SkillDataSave` _agilityskilldata))
    ;[1 1 1] Set Agility Data
    (set `self.Agility Skill Points` _skillpoints_2)
    (set `self.Agility Experience Points` _experience_2)
    (set `self.Agility Level` _level_2)
    (bind (_skillpoints_3 _experience_3 _level_3) (break `/Game/UltimateSurvivalPack/Blueprints/Structs/S_SkillDataSave` _powerskilldata))
    ;[1 1 1] Set Power Data
    (set `self.Power Skill Points` _skillpoints_3)
    (set `self.Power Experience Points` _experience_3)
    (set `self.Power Level` _level_3)))

(event `self.ReceiveBeginPlay`
  (if (`Controller.IsLocalController` (cast `Controller` (`self.GetOwner`) :!pure true))
    (`self.SERVER Load Skill Data`)))

(event `CLIENT Load Skill Data`
  (params (`Unlocked Skills` :type "Array of /Game/UltimateSurvivalPack/Blueprints/Structs/S_SkillDatabase Structure (by ref)") (`Current Skill Abilities` :type "/Game/UltimateSurvivalPack/Blueprints/Structs/S_CurrentSkills Structure") (`Survivor Skill Data` :type "/Game/UltimateSurvivalPack/Blueprints/Structs/S_SkillDataSave Structure (by ref)") (`Agility Skill Data` :type "/Game/UltimateSurvivalPack/Blueprints/Structs/S_SkillDataSave Structure (by ref)") (`Power Skill Data` :type "/Game/UltimateSurvivalPack/Blueprints/Structs/S_SkillDataSave Structure (by ref)"))
  (bind (_skillpoints _experience _level) (break `/Game/UltimateSurvivalPack/Blueprints/Structs/S_SkillDataSave` `Survivor Skill Data`))
  (bind (_skillpoints_2 _experience_2 _level_2) (break `/Game/UltimateSurvivalPack/Blueprints/Structs/S_SkillDataSave` `Agility Skill Data`))
  (bind (_skillpoints_3 _experience_3 _level_3) (break `/Game/UltimateSurvivalPack/Blueprints/Structs/S_SkillDataSave` `Power Skill Data`))
  ;[1 1 1] Set  General Data
  (set `self.Unlocked Skills` `Unlocked Skills`)
  (set `self.Current Skill Abilities` `Current Skill Abilities`)
  ;[1 1 1] Set Survivor Data
  (set `self.Survivor Skill Points` _skillpoints)
  (set `self.Survivor Experience Points` _experience)
  (set `self.Survivor Level` _level)
  ;[1 1 1] Set Agility Data
  (set `self.Agility Skill Points` _skillpoints_2)
  (set `self.Agility Experience Points` _experience_2)
  (set `self.Agility Level` _level_2)
  ;[1 1 1] Set Power Data
  (set `self.Power Skill Points` _skillpoints_3)
  (set `self.Power Experience Points` _experience_3)
  (set `self.Power Level` _level_3))

(fn `Can Be Skill Unlocked?`
  (params (Skill :type "/Game/UltimateSurvivalPack/Blueprints/Structs/S_SkillDatabase Structure"))
  (returns (Success :type Boolean))
  (locals (`Skill Data L` :type "/Game/UltimateSurvivalPack/Blueprints/Structs/S_SkillTreeMaster Structure"))
  (bind _returnvalue (`|GetDataTableRow` Skill_Datatable_2_D181672E433FE4C5D62BCE8220CD4861 Skill_SkillID_5_12955B8D4AB128D1578E878E30765AA1)
    (:`then`
      (bind _output_get (set `local.Skill Data L` _returnvalue))
      (bind ((`ParentSkill_2_019301794AA1CD45BF83C9A36E99CB69` _parentskill) (`SkillSettings_5_2784FA144838FB861B8955ACE1560BFB` _skillsettings)) (break `/Game/UltimateSurvivalPack/Blueprints/Structs/S_SkillTreeMaster` _output_get))
      ;[1 1 1] Does The Skill have Parent Skill ? If Not just skip first Branch.
      (`/Engine/EditorBlueprintResources/StandardMacros.IsValid` (`.Datatable_2_D181672E433FE4C5D62BCE8220CD4861` (break `/Game/UltimateSurvivalPack/Blueprints/Structs/S_SkillDatabase` _parentskill))
        (:`Is Valid`
          ;[1 0.3594 0.3594] Is Parent Skill Unlocked ?
          (if (`KismetArrayLibrary.Array_Contains` (`self.Unlocked Skills`) _parentskill)
            ;[1 0.3594 0.3594] Is Skill Already Unlocked ?
            (if (not (`KismetArrayLibrary.Array_Contains` (`self.Unlocked Skills`) (`local.Skill`))) :!label _label
              (bind (_skilltype _skillpointsrequired) (break `/Game/UltimateSurvivalPack/Blueprints/Structs/S_Skill_Settings` _skillsettings))
              ;[1 0.3594 0.3594] Does Player Has Enought Skill Points ?
              (if (>= (select `/Game/UltimateSurvivalPack/Blueprints/Enum/E_SkillType` _skilltype :`NewEnumerator0` (`self.Survivor Skill Points`) :`NewEnumerator1` (`self.Agility Skill Points`) :`NewEnumerator2` (`self.Power Skill Points`)) _skillpointsrequired)
                ;[0.3696 1 0.141] Success
                (return true)
                (else
                  _)))))
        (:`Is Not Valid`
          (goto _label)))
      ;[1 0.1302 0.1302] Unsuccess
      (return false))))

(fn `Get Level Experience Range`
  (params (`Skill type` :type "/Game/UltimateSurvivalPack/Blueprints/Enum/E_SkillType Enum" :default "NewEnumerator0"))
  (returns (ReturnValue :type Integer))
  (return (select `/Game/UltimateSurvivalPack/Blueprints/Enum/E_SkillType` (`local.Skill Type`) :`NewEnumerator0` (`self.Survivor Level Experience Range`) :`NewEnumerator1` (`self.Agility Level Experience Range`) :`NewEnumerator2` (`self.Power Level Experience Range`))))

(fn `Get Level Information`
  (params (`Skill Type` :type "/Game/UltimateSurvivalPack/Blueprints/Enum/E_SkillType Enum" :default "NewEnumerator0") (Level :type Integer))
  (returns (`Maximum Total XP` :type Integer) (`Minimum Total XP` :type Integer))
  (bind _returnvalue (`KismetMathLibrary.FTrunc` (* (- (`local.Level`) 1) (* (`self.Get Level Experience Range` (`local.Skill Type`)) (* (`local.Level`) 0.5)))))
  (return (+ _returnvalue (* (`self.Get Level Experience Range` (`local.Skill Type`)) (`local.Level`))) _returnvalue))

(fn `Get Player Pawn`
  (returns (ReturnValue :type "Pawn Object Reference"))
  (bind _ascontroller (cast `Controller` (`self.GetOwner`)))
  (return (`Controller.K2_GetPawn` _ascontroller)))

(fn `Get Skill Level`
  (params (`Skill Type` :type "/Game/UltimateSurvivalPack/Blueprints/Enum/E_SkillType Enum" :default "NewEnumerator0"))
  (returns (ReturnValue :type Integer))
  (return (select `/Game/UltimateSurvivalPack/Blueprints/Enum/E_SkillType` `Skill Type` :`NewEnumerator0` (`self.Survivor Level`) :`NewEnumerator1` (`self.Agility Level`) :`NewEnumerator2` (`self.Power Level`))))

(fn `Get Skill Maximum Level`
  (params (`Skill Type` :type "/Game/UltimateSurvivalPack/Blueprints/Enum/E_SkillType Enum" :default "NewEnumerator0"))
  (returns (ReturnValue :type Integer))
  (return (select `/Game/UltimateSurvivalPack/Blueprints/Enum/E_SkillType` `Skill Type` :`NewEnumerator0` (`self.Survivor Maximum Level`) :`NewEnumerator1` (`self.Agility Maximum Level`) :`NewEnumerator2` (`self.Power Maximum Level`))))

(fn `Get Skill Points`
  (params (`Skill Type` :type "/Game/UltimateSurvivalPack/Blueprints/Enum/E_SkillType Enum" :default "NewEnumerator0"))
  (returns (ReturnValue :type Integer))
  (return (select `/Game/UltimateSurvivalPack/Blueprints/Enum/E_SkillType` `Skill Type` :`NewEnumerator0` (`self.Survivor Skill Points`) :`NewEnumerator1` (`self.Agility Skill Points`) :`NewEnumerator2` (`self.Power Skill Points`))))

(fn `Get Total Experience Points`
  (params (`Skill Type` :type "/Game/UltimateSurvivalPack/Blueprints/Enum/E_SkillType Enum" :default "NewEnumerator0"))
  (returns (ReturnValue :type Integer))
  (return (select `/Game/UltimateSurvivalPack/Blueprints/Enum/E_SkillType` (`local.Skill Type`) :`NewEnumerator0` (`self.Survivor Experience Points`) :`NewEnumerator1` (`self.Agility Experience Points`) :`NewEnumerator2` (`self.Power Experience Points`))))

(fn `Save Player Data`
  (bind _ascontroller (cast `Controller` (`self.GetOwner`)))
  (`/Game/UltimateSurvivalPack/Blueprints/Components/BP_MasterInventoryComponent.Save Player Data` (`/Game/UltimateSurvivalPack/Blueprints/BFL_UMSPack.Get Inventory Component` _ascontroller))
  (return))

(fn `Set Skill Experience Points`
  (params (`Skill Type` :type "/Game/UltimateSurvivalPack/Blueprints/Enum/E_SkillType Enum" :default "NewEnumerator0") (`Experience Points` :type Integer))
  (switch `/Game/UltimateSurvivalPack/Blueprints/Enum/E_SkillType` `Skill Type`
    (:`NewEnumerator0`
      (set `self.Survivor Experience Points` `Experience Points`))
    (:`NewEnumerator1`
      (set `self.Agility Experience Points` `Experience Points`))
    (:`NewEnumerator2`
      (set `self.Power Experience Points` `Experience Points`)))
  (return))

(fn `Set Skill Level`
  (params (`Skill Type` :type "/Game/UltimateSurvivalPack/Blueprints/Enum/E_SkillType Enum" :default "NewEnumerator0") (Level :type Integer))
  (switch `/Game/UltimateSurvivalPack/Blueprints/Enum/E_SkillType` `Skill Type`
    (:`NewEnumerator0`
      (set `self.Survivor Level` Level))
    (:`NewEnumerator1`
      (set `self.Agility Level` Level))
    (:`NewEnumerator2`
      (set `self.Power Level` Level)))
  (return))

(fn `Set Skill Points`
  (params (`Skill Type` :type "/Game/UltimateSurvivalPack/Blueprints/Enum/E_SkillType Enum" :default "NewEnumerator0") (`Skill Points` :type Integer))
  (switch `/Game/UltimateSurvivalPack/Blueprints/Enum/E_SkillType` `Skill Type`
    (:`NewEnumerator0`
      (set `self.Survivor Skill Points` `Skill Points`))
    (:`NewEnumerator1`
      (set `self.Agility Skill Points` `Skill Points`))
    (:`NewEnumerator2`
      (set `self.Power Skill Points` `Skill Points`)))
  (return))

(fn `Update Experience`
  (params (`Skill Type` :type "/Game/UltimateSurvivalPack/Blueprints/Enum/E_SkillType Enum" :default "NewEnumerator0") (`Experience Points` :type Integer))
  (bind _skill_type (`local.Skill Type`))
  (bind _skill_type_2 (`local.Skill Type`))
  (bind _skill_type_3 (`local.Skill Type`))
  (bind _skill_type_4 (`local.Skill Type`))
  (bind _skill_type_5 (`local.Skill Type`))
  (bind _returnvalue (`self.Get Skill Level` _skill_type_2))
  (if (!= `Experience Points` 0)
    ;[0.3707 1 0.7436] Add Experience Points
    (`self.Set Skill Experience Points` (`local.Skill Type`) (`KismetMathLibrary.Clamp` (+ (`self.Get Total Experience Points` (`local.Skill Type`)) (`local.Experience Points`)) (`.Minimum Total XP` (`self.Get Level Information` _skill_type_3 (`self.Get Skill Level` _skill_type_3))) (`self.Get Level Information` _skill_type (`self.Get Skill Maximum Level` _skill_type))))
    ;[0.4748 1 0.1691] Check For Level Up
    (if (>= (`self.Get Total Experience Points` _skill_type_4) (`self.Get Level Information` _skill_type_4 _returnvalue)) :!label _label
      (if (< _returnvalue (`self.Get Skill Maximum Level` _skill_type_2))
        (`self.Set Skill Level` (`local.Skill Type`) (+ (`KismetMathLibrary.Clamp` (`self.Get Skill Level` _skill_type_5) 1 (`self.Get Skill Maximum Level` _skill_type_5)) 1))
        (`self.Event On Level Up` (`local.Skill Type`))
        (goto _label)
        (else
          _)))
    ;[1 1 1] Return
    (return)
    (else
      ;[1 1 1] Return
      (return))))

(fn `Update Skill Abilities`
  (params (Skill :type "/Game/UltimateSurvivalPack/Blueprints/Structs/S_SkillTreeMaster Structure"))
  (returns (`Current Skill Abilities` :type "/Game/UltimateSurvivalPack/Blueprints/Structs/S_CurrentSkills Structure"))
  (locals (`New Value | Bool` :type Boolean) (`New Value | Float` :type "Float (double-precision)"))
  (for _array_element (`.SkillsToUnlock_14_8F7E4E0F426802BBA71579A8473897C8` (break `/Game/UltimateSurvivalPack/Blueprints/Structs/S_SkillTreeMaster` Skill))
    (bind (_skillabilitytochange _newvaluebool _newvaluefloat) (break `/Game/UltimateSurvivalPack/Blueprints/Structs/S_SkillToUnlock` _array_element))
    (set `local.New Value | Bool` _newvaluebool)
    (set `local.New Value | Float` _newvaluefloat)
    (switch `/Game/UltimateSurvivalPack/Blueprints/Enum/E_SkillAbility` _skillabilitytochange
      (:`NewEnumerator0`
        ;[1 1 1] Replace Meele Damage Multiplier
        (setmembers `/Game/UltimateSurvivalPack/Blueprints/Structs/S_CurrentSkills` :`StructRef` (`self.Current Skill Abilities`) :`Meele Damage Multiplier` (`local.New Value | Float`)))
      (:`NewEnumerator6`
        ;[1 1 1] Set Hunger Speed
        (setmembers `/Game/UltimateSurvivalPack/Blueprints/Structs/S_CurrentSkills` :`StructRef` (`self.Current Skill Abilities`) :`Hunger Speed Multiplier` (`local.New Value | Float`)))
      (:`NewEnumerator7`
        ;[1 1 1] Set Thirst Speed
        (setmembers `/Game/UltimateSurvivalPack/Blueprints/Structs/S_CurrentSkills` :`StructRef` (`self.Current Skill Abilities`) :`Thirst Speed Multiplier` (`local.New Value | Float`)))
      (:`NewEnumerator8`
        ;[1 1 1] Set Damage Resistance
        (setmembers `/Game/UltimateSurvivalPack/Blueprints/Structs/S_CurrentSkills` :`StructRef` (`self.Current Skill Abilities`) :`Damage Resistance Multiplier` (`local.New Value | Float`)))
      (:`NewEnumerator9`
        ;[1 1 1] Set Stamina
        (setmembers `/Game/UltimateSurvivalPack/Blueprints/Structs/S_CurrentSkills` :`StructRef` (`self.Current Skill Abilities`) :`Stamina` (`local.New Value | Float`)))
      (:`NewEnumerator10`
        ;[1 1 1] Set Stamina
        (setmembers `/Game/UltimateSurvivalPack/Blueprints/Structs/S_CurrentSkills` :`StructRef` (`self.Current Skill Abilities`) :`Fall Damage Resistance` (`local.New Value | Float`)))))
  ;[1 1 1] Return
  (return (`self.Current Skill Abilities`)))