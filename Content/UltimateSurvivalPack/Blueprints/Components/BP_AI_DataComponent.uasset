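; AI data component for enemies that tracks health, per-player damage, death rewards and combat targets.
; Point damage lowers health and records each player's share; death grants proportional XP and skill points, rolls item drops and reports to the enemy camp.
; Perception filters by team and feeds sight, noise and spot stimuli into targets or Blackboard investigation.
; A looping timer prunes lost targets, rechecks line-of-sight and selects the nearest.
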(event `self.ReceiveBeginPlay`
  ;[0 0 0] Begin Play
  (`KismetSystemLibrary.Delay` 0.1) ; Load Delay
  (bind _asw_health_bar (cast `/Game/UltimateSurvivalPack/Widget/W_Health_Bar` (`WidgetComponent.GetUserWidgetObject` (`/Game/UltimateSurvivalPack/Blueprints/BFL_UMSPack.Get Enemy Nametag` (`self.GetOwner`)))))
  (set `/Game/UltimateSurvivalPack/Widget/W_Health_Bar.Component Reference` self _asw_health_bar))

(event `On Death`
  (bind _enemycamp (`self.EnemyCamp`))
  ;[0 0 0] On Death Events
  (set `self.Is Alive` false)
  (`self.Reward Players`)
  (`/Engine/EditorBlueprintResources/StandardMacros.IsValid` _enemycamp
    (:`Is Valid`
      (`self.Send Information To Camp`)
      (`/Game/UltimateSurvivalPack/Blueprints/BP_EnemyCamp.On Member Dead` _enemycamp))))

(event `Widget Visibility`
  (params (Visibility :type "/Game/UltimateSurvivalPack/Blueprints/Enum/E_Visibility Enum" :default "NewEnumerator0"))
  (bind _returnvalue (`self.GetOwner`))
  ;[0 0 0] Show/Hide Enemy Info Widget
  (`/Engine/EditorBlueprintResources/StandardMacros.IsValid` _returnvalue
    (:`Is Valid`
      (`SceneComponent.SetVisibility` (`/Game/UltimateSurvivalPack/Blueprints/BFL_UMSPack.Get Enemy Nametag` _returnvalue) (select `/Game/UltimateSurvivalPack/Blueprints/Enum/E_Visibility` Visibility :`NewEnumerator0` true) false))))

(event `On Point Damage`
  (params (Damage :type "Float (double-precision)") (DamageType :type "DamageType Object Reference") (InstigatedBy :type "Controller Object Reference") (DamageCauser :type "Actor Object Reference") (Hit :type "HitResult Structure"))
  ;[0 0 0] Handling Damage
  (if (`self.Is Alive`)
    (`self.Add to database` Damage InstigatedBy) ; Should be done before function "Handle Damage"
    (cast `/Game/UltimateSurvivalPack/Blueprints/BP_PlayerController` InstigatedBy
      (:`then`
        (cast `/Game/UltimateSurvivalPack/Blueprints/DamageType/DT_Vehicle` DamageType
          (:`then`
            _)
          (:`CastFailed`
            (`/Game/UltimateSurvivalPack/Blueprints/Components/BP_PlayerInventoryComponent.Spawn Damage Widget` (`/Game/UltimateSurvivalPack/Blueprints/BFL_UMSPack.Get Inventory Component` InstigatedBy) (`SceneComponent.K2_GetComponentLocation` (`/Game/UltimateSurvivalPack/Blueprints/BFL_UMSPack.Get Enemy Nametag` (`self.GetOwner`))) (`KismetMathLibrary.FClamp` Damage 0.0 9999.0) (`.HitBoneName` (`GameplayStatics.BreakHitResult` Hit))))))
      (:`CastFailed`
        _))
    (bind _health (`self.Handle Damage` Damage))
    ;;[0.1 0.1 0.1] Calling Event On Death
    (if (<= _health 0.0)
      (`self.On Death`))))

(event `Reward Players`
  (bind _returnvalue (`self.GetOwner`))
  (bind (_returnvalue_roll _returnvalue_pitch _returnvalue_yaw) (`KismetMathLibrary.BreakRotator` (`Actor.K2_GetActorRotation` _returnvalue)))
  ;[0.08459 1 0] Adding experience points to the player depending on his damage
  (`|ExecutionSequence`
    (:`then_0`
      (for (_array_element _array_index) (`self.Player Database`)
        (bind _leveling_component (`/Game/UltimateSurvivalPack/Blueprints/BFL_UMSPack.Get Leveling Component` _array_element))
        (`/Engine/EditorBlueprintResources/StandardMacros.IsValid` _leveling_component
          (:`Is Valid`
            (bind _returnvalue_2 (/ (`|GetArrayItem` (`self.Player Damage Database`) _array_index) (`self.Maximum Health`)))
            (bind _returnvalue_3 (`KismetMathLibrary.FTrunc` (* _returnvalue_2 (`KismetMathLibrary.Conv_IntToDouble` (`self.Experience Reward`)))))
            (`/Game/UltimateSurvivalPack/Blueprints/Components/BP_Player_ExperienceComponent.Add Experience` _leveling_component _returnvalue_3 true (make `/Game/UltimateSurvivalPack/Blueprints/Structs/S_Notification` (`KismetStringLibrary.Concat_StrStr` (`KismetStringLibrary.Conv_NameToString` (`self.Name`)) " Elimination Reward") (`KismetStringLibrary.Concat_StrStr` "+ " (`KismetStringLibrary.Conv_IntToString` _returnvalue_3) " XP")))
            (bind _returnvalue_4 (`KismetMathLibrary.FTrunc` (* _returnvalue_2 (`KismetMathLibrary.Conv_IntToDouble` (`self.Power Points Reward`)))))
            ;;[0 0 0] Add Skill Experience Points
            (if (> _returnvalue_4 0)
              (bind _returnvalue_5 (`/Game/UltimateSurvivalPack/Blueprints/BFL_UMSPack.Get Skill Component` _array_element))
              (`/Game/UltimateSurvivalPack/Blueprints/Components/BP_SkillTreeComponent.Add Experience` _returnvalue_5 "NewEnumerator2" _returnvalue_4))
            (bind _returnvalue_6 (`KismetMathLibrary.FTrunc` (* _returnvalue_2 (`KismetMathLibrary.Conv_IntToDouble` (`self.Agility Points Reward`)))))
            (if (> _returnvalue_6 0)
              (`/Game/UltimateSurvivalPack/Blueprints/Components/BP_SkillTreeComponent.Add Experience` _returnvalue_5 "NewEnumerator1" _returnvalue_6))))))
    (:`then_1`
      (for _array_element_2 (`self.Items to Drop`)
        (bind (_itemid _minimumamount _maximumamount _chanceofspawning) (break `/Game/UltimateSurvivalPack/Blueprints/Structs/S_DropItem` _array_element_2))
        (if (<= (`KismetMathLibrary.RandomFloatInRange` 0.0 100.0) _chanceofspawning)
          (`|SpawnActorFromClass` "/Game/UltimateSurvivalPack/Blueprints/BP_InventoryItem.BP_InventoryItem_C" (`KismetMathLibrary.MakeTransform` (`Actor.K2_GetActorLocation` _returnvalue) (`KismetMathLibrary.MakeRotator` 0.0 0.0 _returnvalue_yaw)) "AdjustIfPossibleButAlwaysSpawn" "OverrideRootScale" null (make `/Game/UltimateSurvivalPack/Blueprints/Structs/S_InventoryItem` _itemid (`KismetMathLibrary.Clamp` (`KismetMathLibrary.RandomIntegerInRange` _minimumamount _maximumamount) 1 999999)) null null))))))

(event `On Perception Updated`
  (params (Actor :type "Actor Object Reference") (Simulus :type "AIStimulus Structure"))
  (`self.Perception Updated` Actor Simulus))

(fn `Add Enemy Target`
  (params (`New Target` :type "Actor Object Reference (by ref)"))
  (bind _new_target (`local.New Target`))
  (bind _combat_check_time (`self.Combat Check Time`))
  (if (`Actor.HasAuthority` (`self.GetOwner`))
    (`/Engine/EditorBlueprintResources/StandardMacros.IsValid` `New Target`
      (:`Is Valid`
        ;[1 1 1] Is not already in targets
        (if (not (`KismetArrayLibrary.Array_Contains` (`self.Enemy Targets`) (`local.New Target`)))
          ;[1 1 1] Is alive (if implements player interface)
          (if (`KismetSystemLibrary.DoesImplementInterface` _new_target "/Game/UltimateSurvivalPack/Blueprints/Interface/BPI_Player.BPI_Player_C")
            (bind _is_alive (message `/Game/UltimateSurvivalPack/Blueprints/Interface/BPI_Player.Is Alive` _new_target))
            (if _is_alive
              (if (<= (`KismetArrayLibrary.Array_Length` (`self.Enemy Targets`)) 0) :!label _label
                ;[1 1 1] Set checking Timer
                (if (`KismetSystemLibrary.K2_IsTimerActiveHandle` (`self.Combat Timer Handle`))
                  (`KismetSystemLibrary.K2_ClearAndInvalidateTimerHandle` (`self.Combat Timer Handle`)))
                (bind _returnvalue (`KismetSystemLibrary.K2_SetTimer` null "CheckForCombat" (`KismetMathLibrary.Abs` _combat_check_time) true (* _combat_check_time -1.0)))
                (set `self.Combat Timer Handle` _returnvalue))
              ;[1 1 1] Add to Enemy Targets
              (`KismetArrayLibrary.Array_AddUnique` (`self.Enemy Targets`) (`local.New Target`))
              (`BlackboardComponent.SetValueAsEnum` (`AIBlueprintHelperLibrary.GetBlackboard` (`self.GetOwner`)) "Action" 0))
            (else
              (goto _label))))))))

(fn `Add To Database`
  (params (Damage :type "Float (double-precision)") (`Damage Causer` :type "Controller Object Reference"))
  (bind _returnvalue (`KismetArrayLibrary.Array_Find` (`self.Player Database`) `Damage Causer`))
  (bind _returnvalue_2 (`KismetMathLibrary.FClamp` (`KismetMathLibrary.Conv_IntToDouble` (`KismetMathLibrary.FTrunc` Damage)) 0.0 (`self.Health`)))
  (cast `PlayerController` `Damage Causer`)
  (if (`KismetArrayLibrary.Array_Contains` (`self.Player Database`) `Damage Causer`)
    ;[0 0 0] Replacing Existing Damage
    (`KismetArrayLibrary.Array_Set` (`self.Player Damage Database`) _returnvalue (+ (`|GetArrayItem` (`self.Player Damage Database`) _returnvalue) _returnvalue_2))
    (else
      ;[0 0 0] Adding Player To Array
      (`KismetArrayLibrary.Array_Add` (`self.Player Database`) `Damage Causer`)
      (`KismetArrayLibrary.Array_Add` (`self.Player Damage Database`) _returnvalue_2))))

(fn `BB Update Target`
  (params (`New Target` :type "Actor Object Reference"))
  ;[1 1 1] Comment
  (bind _ascharacter (cast `Character` (`self.GetOwner`)))
  (`BlackboardComponent.SetValueAsObject` (`AIBlueprintHelperLibrary.GetBlackboard` (`AIBlueprintHelperLibrary.GetAIController` _ascharacter)) "Target" (`local.New Target`))
  ;[1 1 1] On Target Call
  (message `/Game/UltimateSurvivalPack/Blueprints/Interface/BPI_AI.On Target Updated` (`self.GetOwner`)))

(fn `Check For Visibility`
  (params (Actor :type "Actor Object Reference"))
  (returns (Return :type Boolean))
  (bind (_outhit _returnvalue) (`KismetSystemLibrary.LineTraceSingle` (`Actor.K2_GetActorLocation` (`self.GetOwner`)) (`Actor.K2_GetActorLocation` Actor) "TraceTypeQuery5"))
  (if _returnvalue
    (`KismetArrayLibrary.Array_AddUnique` (`self.Visually Sensed Actors`) (`local.Actor`))
    (return false)
    (else
      (return true))))

(fn `CheckForCombat`
  (locals (`L Current Shortest Target Distance` :type "Float (double-precision)" :default 9999999.0) (`L Current Target Distance` :type "Float (double-precision)" :default 0.0) (`L Current Target` :type "Actor Object Reference") (`L Array` :type "Array of Actor Object Reference") (`L Targets` :type "Array of Actor Object Reference"))
  ;[1 1 1] Has Any Targets
  (if (> (`KismetArrayLibrary.Array_Length` (`self.Enemy Targets`)) 0)
    (bind _output_get (set `local.L Array` (`self.Visually Sensed Actors`)))
    (for _array_element _output_get
      (`/Engine/EditorBlueprintResources/StandardMacros.IsValid` _array_element
        (:`Is Valid`
          (bind _return (`self.Check For Visibility` _array_element))
          (if _return
            (`KismetArrayLibrary.Array_AddUnique` (`self.Enemy Targets`) _array_element)
            (`BlackboardComponent.SetValueAsEnum` (`AIBlueprintHelperLibrary.GetBlackboard` (`self.GetOwner`)) "Action" 0)
            (`KismetArrayLibrary.Array_RemoveItem` (`self.Visually Sensed Actors`) _array_element :!label _label)))
        (:`Is Not Valid`
          (goto _label))))
    ;[1 1 1] Check for Targets and their distances, if not valid, remove
    (bind _output_get_2 (set `local.L Targets` (`self.Enemy Targets`)))
    (for _array_element_2 _output_get_2
      (`/Engine/EditorBlueprintResources/StandardMacros.IsValid` _array_element_2
        (:`Is Valid`
          ;;[1 1 1] Is alive (if implements player interface)
          (if (`KismetSystemLibrary.DoesImplementInterface` _array_element_2 "/Game/UltimateSurvivalPack/Blueprints/Interface/BPI_Player.BPI_Player_C")
            (bind _is_alive (message `/Game/UltimateSurvivalPack/Blueprints/Interface/BPI_Player.Is Alive` _array_element_2))
            (if _is_alive
              (bind _output_get_3 (set `local.L Current Target Distance` (`Actor.GetDistanceTo` (`self.GetOwner`) _array_element_2) :!label _label_2))
              (if (not (> _output_get_3 (`self.Target Lost Distance`)))
                (if (< _output_get_3 (`local.L Current Shortest Target Distance`))
                  (set `local.L Current Shortest Target Distance` (`local.L Current Target Distance`))
                  (set `local.L Current Target` _array_element_2))
                (else
                  (`self.Remove Enemy Target` _array_element_2 :!label _label_3)))
              (else
                (goto _label_3)))
            (else
              (goto _label_2))))
        (:`Is Not Valid`
          (goto _label_3))))
    ;[1 1 1] Update New Target
    (if (!= (`local.L Current Target`) (`self.Current Enemy Target`))
      (bind _output_get_4 (set `self.Current Enemy Target` (`local.L Current Target`)))
      (`self.BB Update Target` _output_get_4))))

(fn `Handle Damage`
  (params (Damage :type "Float (double-precision)"))
  (returns (Health :type "Float (double-precision)"))
  ;[0 0 0] Applying Damage
  (bind _output_get (set `self.Health` (`KismetMathLibrary.FClamp` (- (`self.Health`) (`KismetMathLibrary.Conv_IntToDouble` (`KismetMathLibrary.FTrunc` Damage))) 0.0 (`self.Health`))))
  ;[1 1 1] Call On death to Character if health <= 0
  (if (<= _output_get 0.0)
    (message `/Game/UltimateSurvivalPack/Blueprints/Interface/BPI_AI.On Dead` (`self.GetOwner`)))
  (return _output_get))

(fn `Perception Updated`
  (params (Actor :type "Actor Object Reference") (Stimulus :type "AIStimulus Structure"))
  (locals (`L Target` :type "Actor Object Reference") (`L Reacheable Locatiojn` :type "Vector Structure" :default (0.0 0.0 0.0)))
  (bind _returnvalue (`AIBlueprintHelperLibrary.GetBlackboard` (`self.GetOwner`)))
  (bind _returnvalue_2 (`AIBlueprintHelperLibrary.GetBlackboard` (`self.GetOwner`)))
  ;[1 1 1] Switch Based On Vehicle
  (bind _asbp_buggy (cast `/Game/UltimateSurvivalPack/Blueprints/VehicleBP/BP_Buggy` Actor)
    (:`then`
      (bind _asplayer_controller (cast `PlayerController` (`Pawn.GetController` _asbp_buggy)))
      (bind _output_get (set `local.L Target` (`/Game/UltimateSurvivalPack/Blueprints/Components/BP_PlayerInventoryComponent.Human Player Character` (`/Game/UltimateSurvivalPack/Blueprints/BFL_UMSPack.Get Inventory Component` _asplayer_controller)))))
    (:`CastFailed`
      (set `local.L Target` (`local.Actor`))))
  (bind _team_id (message `/Game/UltimateSurvivalPack/Blueprints/Interface/BPI_InventorySystem.Get Team ID` _output_get))
  (if (and (!= _team_id (`self.Team ID`)) (!= _team_id 0))
    (switch `name` (`.Tag` (break `AIStimulus` Stimulus))
      (:`None`
        ;[1 1 1] Check for Visual Sense
        (bind _return (`self.Check For Visibility` (`local.L Target`)))
        (if _return
          (`self.Add Enemy Target` (`local.L Target`) :!label _label)))
      (:`Noise`
        (if (< (`KismetMathLibrary.Vector_Distance` (`Actor.K2_GetActorLocation` (`self.GetOwner`)) (`.StimulusLocation` (break `AIStimulus` (`local.Stimulus`)))) 750.0)
          (goto _label)
          (else
            (`self.Current Enemy Target`
              (:`then`)
              (:`else`
                ;[1 1 1] Set Hear Sense
                (`BlackboardComponent.SetValueAsEnum` _returnvalue "Action" 1)
                (`BlackboardComponent.SetValueAsVector` _returnvalue "Action Location" (`.StimulusLocation` (break `AIStimulus` (`local.Stimulus`)))))))))
      (:`Enemy Spot`
        (`self.Current Enemy Target`
          (:`then`)
          (:`else`
            ;[1 1 1] Set Hear Sense
            (set `local.L Reacheable Locatiojn` (`NavigationSystemV1.K2_GetRandomReachablePointInRadius` (`Actor.K2_GetActorLocation` (`local.Actor`)) 500.0 null null))
            (`BlackboardComponent.SetValueAsEnum` _returnvalue_2 "Action" 1)
            (`BlackboardComponent.SetValueAsVector` _returnvalue_2 "Action Location" (`local.L Reacheable Locatiojn`))))))))

(fn `Remove Enemy Target`
  (params (`Target to Remove` :type "Actor Object Reference (by ref)"))
  (if (`Actor.HasAuthority` (`self.GetOwner`))
    ;[1 1 1] If contains, check if is current, update target and remove it from Array
    (if (`KismetArrayLibrary.Array_Contains` (`self.Enemy Targets`) `Target to Remove`)
      (`KismetArrayLibrary.Array_RemoveItem` (`self.Enemy Targets`) (`local.Target to Remove`))
      (if (== (`self.Current Enemy Target`) (`local.Target to Remove`))
        (`self.BB Update Target` null))
      ;[1 1 1] If empty, clear and invalidate timer
      (if (<= (`KismetArrayLibrary.Array_Length` (`self.Enemy Targets`)) 0)
        (`KismetSystemLibrary.K2_ClearAndInvalidateTimerHandle` (`self.Combat Timer Handle`))))))

(fn `Send Information To Camp`
  (bind _enemycamp (`self.EnemyCamp`))
  (bind _playerdamagedatabase (`/Game/UltimateSurvivalPack/Blueprints/BP_EnemyCamp.PlayerDamageDatabase` (`self.EnemyCamp`)))
  (for (_array_element _array_index) (`self.Player Database`)
    (if (`KismetArrayLibrary.Array_Contains` (`/Game/UltimateSurvivalPack/Blueprints/BP_EnemyCamp.PlayerDatabase` (`self.EnemyCamp`)) _array_element)
      (bind _returnvalue (`KismetArrayLibrary.Array_Find` (`/Game/UltimateSurvivalPack/Blueprints/BP_EnemyCamp.PlayerDatabase` (`self.EnemyCamp`)) _array_element))
      (bind _output (`|GetArrayItem` (`self.Player Damage Database`) _array_index))
      ;[0.4896 0.05952 0] Replacing damage value
      (`KismetArrayLibrary.Array_Set` _playerdamagedatabase _returnvalue (+ (`|GetArrayItem` _playerdamagedatabase _returnvalue) _output))
      (else
        ;[0.2341 0.4167 0] Creating value
        (`KismetArrayLibrary.Array_Add` (`/Game/UltimateSurvivalPack/Blueprints/BP_EnemyCamp.PlayerDatabase` _enemycamp) _array_element)
        (`KismetArrayLibrary.Array_Add` (`/Game/UltimateSurvivalPack/Blueprints/BP_EnemyCamp.PlayerDamageDatabase` _enemycamp) _output)))))