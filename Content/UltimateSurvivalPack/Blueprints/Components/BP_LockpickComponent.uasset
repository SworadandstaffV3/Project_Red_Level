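; An actor component that makes its owner a pickable lock, tracking the locked state and the player currently picking it.
; On BeginPlay, only the authority rolls a random unlock angle within a half-circle range.
; CanLockpick requires a lockpick item and a free lock, notifying the player otherwise, and also reports whether it is unlocked.
; ToggleLockpicking claims a free lock for a controller and opens that client's lockpick through its inventory component.
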(event `self.ReceiveBeginPlay`
  ;[1 1 1] Initialize
  (`self.Initialize Lockpick Component`))

(event `Initialize Lockpick Component`
  ;[1 1 1] Generate Random Unlock Location
  (if (`Actor.HasAuthority` (`self.GetOwner`))
    (set `self.Unlock Angle` (`KismetMathLibrary.RandomFloatInRange` -90.0 90.0))))

(event `Toggle Lockpicking`
  (params (Controller :type "Controller Object Reference"))
  ;[1 1 1] Toggle Lockpick
  (`/Engine/EditorBlueprintResources/StandardMacros.IsValid` (`self.Current Lockpicking Player`)
    (:`Is Not Valid`
      (bind _output_get (set `self.Current Lockpicking Player` Controller))
      (`/Game/UltimateSurvivalPack/Blueprints/Components/BP_PlayerInventoryComponent.CLIENT Open Lockpick` (`/Game/UltimateSurvivalPack/Blueprints/BFL_UMSPack.Get Inventory Component` _output_get) self))))

(fn `Can Lockpick`
  (params (Player :type "Controller Object Reference"))
  (returns (Return :type Boolean) (`Is Unlocked` :type Boolean))
  (bind _missioncomponent (`/Game/UltimateSurvivalPack/Blueprints/BFL_UMSPack.Get Mission Component` Player))
  (if (>= (`/Game/UltimateSurvivalPack/Blueprints/Components/BP_MasterInventoryComponent.Find Item by ID` (`/Game/UltimateSurvivalPack/Blueprints/BFL_UMSPack.Get Inventory Component` Player) "Lockpick") 0)
    ;[1 1 1] Lockpick Conditions
    (`/Engine/EditorBlueprintResources/StandardMacros.IsValid` (`self.Current Lockpicking Player`)
      (:`Is Valid`
        (`/Game/UltimateSurvivalPack/Blueprints/Components/BP_MissionComponent.CLIENT Add Notification` _missioncomponent (make `/Game/UltimateSurvivalPack/Blueprints/Structs/S_Notification` "Cannot Lockpick" "Lock is already being lockpicked"))
        (return false (not (`self.Locked`))))
      (:`Is Not Valid`
        (if (`self.Locked`)
          (return true false)
          (else
            (return false true)))))
    (else
      (`/Game/UltimateSurvivalPack/Blueprints/Components/BP_MissionComponent.CLIENT Add Notification` _missioncomponent (make `/Game/UltimateSurvivalPack/Blueprints/Structs/S_Notification` "No Lockpick" "You need a lockpick"))
      (return false (not (`self.Locked`))))))