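; Base inventory component for the survival pack, holding a slot array created on the authority with helpers for item and free-space lookups.
; AddItem splits amounts into full stacks, partial-stack top-ups and a remainder, writing slots once space is found.
; Server events forward use and swap requests; player inventories send changed indexes to the client to refresh UI slots.
; Remove, use, swap and save are empty stubs here.
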(event `SERVER Use Item`
  (params (`At Index` :type Integer) (`From Inventory` :type "/Game/UltimateSurvivalPack/Blueprints/Components/BP_MasterInventoryComponent Object Reference"))
  ;[1 1 1] Request Use Item
  (`self.Use Item Call` `At Index` `From Inventory`))

(event `SERVER Swap Items`
  (params (`From Index` :type Integer) (`From Inventory` :type "/Game/UltimateSurvivalPack/Blueprints/Components/BP_MasterInventoryComponent Object Reference") (`To Index` :type Integer) (`To Inventory` :type "/Game/UltimateSurvivalPack/Blueprints/Components/BP_MasterInventoryComponent Object Reference"))
  ;[1 1 1] Request Swap Items
  (`self.Swap Items` `From Index` `From Inventory` `To Index` `To Inventory`))

(event `CLIENT Update Inventory and Slots`
  (params (Inventory :type "Array of /Game/UltimateSurvivalPack/Blueprints/Structs/S_InventoryItem Structure (by ref)") (`Indexes to Update` :type "Array of Integer"))
  ;[1 1 1] Local update Inventory and Slots
  (set `self.Inventory` Inventory)
  ;;[1 1 1] Is array not empty
  (if (> (`KismetArrayLibrary.Array_Length` `Indexes to Update`) 0)
    ;;[1 1 1] Update slots at indexes in ui
    (for _array_element `Indexes to Update`
      (`/Game/UltimateSurvivalPack/Widget/W_Inventory.Update Slot` (`self.Get Local Player Inventory UI`) _array_element false))
    (`self.Local On Inventory Updated`)))

(fn `Add Item`
  (params (Item :type "/Game/UltimateSurvivalPack/Blueprints/Structs/S_InventoryItem Structure"))
  (returns (Success :type Boolean))
  (locals (`L Current Item Data` :type "/Game/UltimateSurvivalPack/Blueprints/Structs/S_InventoryItemData Structure") (`L New Amount` :type Integer :default 0) (`L Current Index` :type Integer :default 0) (`L Queued Amount` :type Integer) (`L Maped Index Amounts` :type "Map of Integer to Object Object Reference") (`L Free Indexes` :type "Array of Integer") (`L Stacks` :type Integer :default 0) (`L Indexes to Update` :type "Array of Integer") (`L Current Amount` :type Integer))
  (bind (_bisvalid _item_data) (`/Game/UltimateSurvivalPack/Blueprints/BFL_Inventory.Get Item Data from ID` Item_ID_2_1F4451EE4759095BA0D31BB237483A5E))
  (bind (_item_id _item_amount _item_cachedindex _item_inventoryreference _item_custominteger _item_durability _item_additionaldata) (break `/Game/UltimateSurvivalPack/Blueprints/Structs/S_InventoryItem` (`local.Item`)))
  (bind _item_id_2 (break `/Game/UltimateSurvivalPack/Blueprints/Structs/S_InventoryItem` (`local.Item`)))
  (bind _l_maped_index_amounts (`local.L Maped Index Amounts`))
  (bind (_item_id_3 _item_amount_2 _item_cachedindex_2 _item_inventoryreference_2 _item_custominteger_2 _item_durability_2 _item_additionaldata_2) (break `/Game/UltimateSurvivalPack/Blueprints/Structs/S_InventoryItem` (`local.Item`)))
  (bind _l_maped_index_amounts_2 (`local.L Maped Index Amounts`))
  (bind (_item_id_4 _item_amount_3 _item_cachedindex_3 _item_inventoryreference_3 _item_custominteger_3 _item_durability_3 _item_additionaldata_3) (break `/Game/UltimateSurvivalPack/Blueprints/Structs/S_InventoryItem` (`local.Item`)))
  (bind _l_free_indexes (`local.L Free Indexes`))
  (bind (_item_id_5 _item_amount_4 _item_cachedindex_4 _item_inventoryreference_4 _item_custominteger_4 _item_durability_4 _item_additionaldata_4) (break `/Game/UltimateSurvivalPack/Blueprints/Structs/S_InventoryItem` (`local.Item`)))
  (bind ((`MaximumStack_21_39EA4E634AD2ADBC0EA36C92000AFBC7` _maximumstack)) (break `/Game/UltimateSurvivalPack/Blueprints/Structs/S_InventoryItemData` (`local.L Current Item Data`)))
  (bind _found_indexes (`self.Find Item Indexes from ID` _item_id_2))
  (bind _returnvalue (- _maximumstack (`local.L Current Amount`)))
  (bind _returnvalue_2 (<= (`local.L Queued Amount`) _returnvalue))
  (bind (_remainder _returnvalue_3) (`KismetMathLibrary.FMod` (`KismetMathLibrary.Conv_IntToDouble` (`local.L Queued Amount`)) (`KismetMathLibrary.Conv_IntToDouble` (`.MaximumStack_21_39EA4E634AD2ADBC0EA36C92000AFBC7` (break `/Game/UltimateSurvivalPack/Blueprints/Structs/S_InventoryItemData` (`local.L Current Item Data`))))))
  (bind _output_get (set `local.L Queued Amount` Item_Amount_5_1F2975454CE296A7C7033BA39535256F))
  ;[1 1 1] Is Valid
  (if (> _output_get 0)
    (if _bisvalid
      (set `local.L Current Item Data` _item_data)
      ;[1 1 1] Is Stackable Item
      (if (> (`.MaximumStack_21_39EA4E634AD2ADBC0EA36C92000AFBC7` (break `/Game/UltimateSurvivalPack/Blueprints/Structs/S_InventoryItemData` (`local.L Current Item Data`))) 1)
        (if (> _returnvalue_3 0)
          (set `local.L Stacks` (- _returnvalue_3 1))
          (for _ (range (+ (`local.L Stacks`) 1))
            (bind _array_index (`self.Find Free Space` (`local.L Free Indexes`)))
            (if (> _array_index -1)
              (`KismetArrayLibrary.Array_AddUnique` (`local.L Free Indexes`) _array_index)
              (set `local.L Queued Amount` (- (`local.L Queued Amount`) (`.MaximumStack_21_39EA4E634AD2ADBC0EA36C92000AFBC7` (break `/Game/UltimateSurvivalPack/Blueprints/Structs/S_InventoryItemData` (`local.L Current Item Data`))))))))
        (if (> (`KismetArrayLibrary.Array_Length` _found_indexes) 0)
          ;[1 1 1] Loop through found indexes
          (for _array_element _found_indexes
            (bind (_output_id _output_amount) (break `/Game/UltimateSurvivalPack/Blueprints/Structs/S_InventoryItem` (`|GetArrayItem` (`self.Inventory`) _array_element)))
            ;[1 1 1] Add amount
            (if (< _output_amount (`.MaximumStack_21_39EA4E634AD2ADBC0EA36C92000AFBC7` (break `/Game/UltimateSurvivalPack/Blueprints/Structs/S_InventoryItemData` (`local.L Current Item Data`))))
              (`BlueprintMapLibrary.Map_Add` (`local.L Maped Index Amounts`) _array_element _output_amount)))
          (bind _keys (`BlueprintMapLibrary.Map_Keys` _l_maped_index_amounts_2))
          (for _array_element_2 _keys
            (if (<= (`local.L Queued Amount`) 0)
              (`BlueprintMapLibrary.Map_Remove` (`local.L Maped Index Amounts`) _array_element_2)
              (else
                (set `local.L Current Amount` (`BlueprintMapLibrary.Map_Find` _l_maped_index_amounts_2 _array_element_2))
                (`BlueprintMapLibrary.Map_Add` (`local.L Maped Index Amounts`) _array_element_2 (select `bool` _returnvalue_2 :`false` _maximumstack :`true` (+ (`local.L Current Amount`) (`local.L Queued Amount`))))
                (set `local.L Queued Amount` (- (`local.L Queued Amount`) (select `bool` _returnvalue_2 :`false` _returnvalue :`true` (`local.L Queued Amount`))))))))
        (if (> (`local.L Queued Amount`) 0)
          (bind _array_index_2 (`self.Find Free Space` (`local.L Free Indexes`)))
          (if (> _array_index_2 -1)
            (`KismetArrayLibrary.Array_Set` (`self.Inventory`) _array_index_2 (make `/Game/UltimateSurvivalPack/Blueprints/Structs/S_InventoryItem` _item_id_5 (`local.L Queued Amount`) _array_index_2 self _item_custominteger_4 _item_durability_4 _item_additionaldata_4))
            (`KismetArrayLibrary.Array_AddUnique` (`local.L Indexes to Update`) _array_index_2)
            (else
              (return false))))
        (if (> (`KismetArrayLibrary.Array_Length` _l_free_indexes) 0)
          (for _array_element_3 _l_free_indexes
            (`KismetArrayLibrary.Array_Set` (`self.Inventory`) _array_element_3 (make `/Game/UltimateSurvivalPack/Blueprints/Structs/S_InventoryItem` _item_id_4 (`.MaximumStack_21_39EA4E634AD2ADBC0EA36C92000AFBC7` (break `/Game/UltimateSurvivalPack/Blueprints/Structs/S_InventoryItemData` (`local.L Current Item Data`))) _array_element_3 self _item_custominteger_3 _item_durability_3 _item_additionaldata_3))
            (`KismetArrayLibrary.Array_AddUnique` (`local.L Indexes to Update`) _array_element_3)))
        (bind _keys_2 (`BlueprintMapLibrary.Map_Keys` _l_maped_index_amounts))
        (if (> (`KismetArrayLibrary.Array_Length` _keys_2) 0)
          (for _array_element_4 _keys_2
            (`KismetArrayLibrary.Array_Set` (`self.Inventory`) _array_element_4 (make `/Game/UltimateSurvivalPack/Blueprints/Structs/S_InventoryItem` _item_id_3 (`BlueprintMapLibrary.Map_Find` _l_maped_index_amounts _array_element_4) _array_element_4 self _item_custominteger_2 _item_durability_2 _item_additionaldata_2))
            (`KismetArrayLibrary.Array_AddUnique` (`local.L Indexes to Update`) _array_element_4)))
        (cast `/Game/UltimateSurvivalPack/Blueprints/Components/BP_PlayerInventoryComponent` self
          (:`then`
            (`self.CLIENT Update Inventory and Slots` (`self.Inventory`) (`local.L Indexes to Update`)))
          (:`CastFailed`
            _))
        (return true)
        (else
          ;[1 1 1] Has found Free Space
          (bind _array_index_3 (`self.Find Free Space` (`|MakeArray`)))
          (bind _output_get_2 (set `local.L Current Index` _array_index_3))
          (if (>= _output_get_2 0)
            (`KismetArrayLibrary.Array_Set` (`self.Inventory`) _output_get_2 (make `/Game/UltimateSurvivalPack/Blueprints/Structs/S_InventoryItem` _item_id _item_amount _output_get_2 self _item_custominteger _item_durability _item_additionaldata))
            (`KismetArrayLibrary.Array_AddUnique` (`local.L Indexes to Update`) _output_get_2)
            (cast `/Game/UltimateSurvivalPack/Blueprints/Components/BP_PlayerInventoryComponent` self
              (:`then`
                (`self.CLIENT Update Inventory and Slots` (`self.Inventory`) (`local.L Indexes to Update`)))
              (:`CastFailed`
                _))
            (return true)
            (else
              (`KismetSystemLibrary.PrintString` "Inventory is Full" true true (struct :`R` 1.0 :`G` 0.229378 :`B` 0.349274 :`A` 1.0) 5.0)
              (return false)))))
      (else
        _)))
  (return false))

(fn `Create Inventory`
  (if (`Actor.HasAuthority` (`self.GetOwner`))
    (`KismetArrayLibrary.Array_Clear` (`self.Inventory`))
    (for _index (range (`self.Inventory Size`))
      (`KismetArrayLibrary.Array_Set` (`self.Inventory`) _index (make `/Game/UltimateSurvivalPack/Blueprints/Structs/S_InventoryItem` "None" 0 _index self) true))))

(fn `Find Free Space`
  (params (Exceptions :type "Array of Integer (by ref)"))
  (returns (`Array Index` :type Integer))
  (for (_array_element _array_index) (`self.Inventory`)
    (if (and (not (`KismetArrayLibrary.Array_Contains` Exceptions _array_index)) (== (`.ID_2_1F4451EE4759095BA0D31BB237483A5E` (break `/Game/UltimateSurvivalPack/Blueprints/Structs/S_InventoryItem` _array_element)) "None"))
      (return _array_index)))
  (return -1))

(fn `Find Free Space for Item`
  (params (`Item ID` :type Name) (`Limit Finder to Index` :type Integer :default -1) (Exceptions :type "Array of Integer"))
  (returns (`Found Space` :type Integer))
  (locals (`L Data` :type "/Game/UltimateSurvivalPack/Blueprints/Structs/S_InventoryItemData Structure") (`L Found Free Amount` :type Integer))
  (bind (_bisvalid _item_data) (`/Game/UltimateSurvivalPack/Blueprints/BFL_Inventory.Get Item Data from ID` `Item ID`))
  (bind ((`MaximumStack_21_39EA4E634AD2ADBC0EA36C92000AFBC7` _maximumstack)) (break `/Game/UltimateSurvivalPack/Blueprints/Structs/S_InventoryItemData` (`local.L Data`)))
  (bind _returnvalue (`KismetArrayLibrary.Array_LastIndex` (`self.Inventory`)))
  (if _bisvalid
    (set `local.L Data` _item_data)
    (for _index (range (+ (select `bool` (> `Limit Finder to Index` -1) :`false` _returnvalue :`true` (`KismetMathLibrary.Clamp` `Limit Finder to Index` 0 _returnvalue)) 1))
      ;[1 1 1] Search for Stacks and Free Slots
      (if (not (`KismetArrayLibrary.Array_Contains` Exceptions _index))
        (bind ((`ID_2_1F4451EE4759095BA0D31BB237483A5E` _id) (`Amount_5_1F2975454CE296A7C7033BA39535256F` _amount)) (break `/Game/UltimateSurvivalPack/Blueprints/Structs/S_InventoryItem` (`|GetArrayItem` (`self.Inventory`) _index)))
        (if (== _id (`local.Item ID`))
          (set `local.L Found Free Amount` (+ (`local.L Found Free Amount`) (- _maximumstack _amount)))
          (elif (== _id "None")
            (set `local.L Found Free Amount` (+ (`local.L Found Free Amount`) _maximumstack))))))
    (return (`local.L Found Free Amount`))
    (else
      (return -1))))

(fn `Find Free Space for Item Amount`
  (params (`Item ID` :type Name) (Amount :type Integer) (`Limit Finder to Index` :type Integer :default -1) (Exceptions :type "Array of Integer"))
  (returns (`Found Indexes` :type "Array of Integer"))
  (locals (`L Data` :type "/Game/UltimateSurvivalPack/Blueprints/Structs/S_InventoryItemData Structure") (`L Found Free Amount` :type Integer) (`L Found Indexes` :type "Array of Integer"))
  (bind (_bisvalid _item_data) (`/Game/UltimateSurvivalPack/Blueprints/BFL_Inventory.Get Item Data from ID` `Item ID`))
  (bind ((`MaximumStack_21_39EA4E634AD2ADBC0EA36C92000AFBC7` _maximumstack)) (break `/Game/UltimateSurvivalPack/Blueprints/Structs/S_InventoryItemData` (`local.L Data`)))
  (bind _returnvalue (`KismetArrayLibrary.Array_LastIndex` (`self.Inventory`)))
  (if _bisvalid
    (set `local.L Data` _item_data)
    (for _index (range (+ (select `bool` (> `Limit Finder to Index` -1) :`false` _returnvalue :`true` (`KismetMathLibrary.Clamp` `Limit Finder to Index` 0 _returnvalue)) 1))
      ;[1 1 1] Search for Stacks and Free Slots
      (if (not (`KismetArrayLibrary.Array_Contains` Exceptions _index))
        (bind ((`ID_2_1F4451EE4759095BA0D31BB237483A5E` _id) (`Amount_5_1F2975454CE296A7C7033BA39535256F` _amount)) (break `/Game/UltimateSurvivalPack/Blueprints/Structs/S_InventoryItem` (`|GetArrayItem` (`self.Inventory`) _index)))
        (if (== _id (`local.Item ID`))
          (set `local.L Found Free Amount` (+ (`local.L Found Free Amount`) (- _maximumstack _amount)))
          (`KismetArrayLibrary.Array_AddUnique` (`local.L Found Indexes`) _index :!label _label)
          (if (>= (`local.L Found Free Amount`) (`local.Amount`))
            (return (`local.L Found Indexes`)))
          (elif (== _id "None")
            (set `local.L Found Free Amount` (+ (`local.L Found Free Amount`) _maximumstack))
            (goto _label)))))
    (return)
    (else
      (return))))

(fn `Find Item by ID`
  (params (`Item ID` :type "Name (by ref)"))
  (returns (`Array Index` :type Integer))
  (for (_array_element _array_index) (`self.Inventory`)
    (if (== (break `/Game/UltimateSurvivalPack/Blueprints/Structs/S_InventoryItem` _array_element) `Item ID`)
      (return _array_index)))
  (return -1))

(fn `Find Item Indexes from ID`
  (params (`Item ID` :type Name))
  (returns (`Found Indexes` :type "Array of Integer"))
  (locals (`L Found Indexes` :type "Array of Integer"))
  (for _array_element (`self.Inventory`)
    (if (== (break `/Game/UltimateSurvivalPack/Blueprints/Structs/S_InventoryItem` _array_element) (`local.Item ID`))
      (`KismetArrayLibrary.Array_AddUnique` (`local.L Found Indexes`) (`.CachedIndex_8_8C45C80D4D5FE5E3EA32ABA4B5107184` (break `/Game/UltimateSurvivalPack/Blueprints/Structs/S_InventoryItem` _array_element)))))
  (return (`local.L Found Indexes`)))

(fn `Get Local Player Inventory UI`
  (returns (W_Inventory :type "/Game/UltimateSurvivalPack/Widget/W_Inventory Object Reference"))
  (bind _returnvalue (`self.GetOwner`))
  (bind _hud (`/Game/UltimateSurvivalPack/Blueprints/Components/BP_MissionComponent.HUD` (`/Game/UltimateSurvivalPack/Blueprints/BFL_UMSPack.Get Mission Component` _returnvalue)))
  (if (`Controller.IsLocalController` (cast `Controller` _returnvalue :!pure true))
    (`/Engine/EditorBlueprintResources/StandardMacros.IsValid` _hud
      (:`Is Valid`
        (return (`/Game/UltimateSurvivalPack/Widget/W_InventoryHUD.W_Inventory` (`/Game/UltimateSurvivalPack/Widget/W_HUD.W_InventoryHUD` _hud))))
      (:`Is Not Valid`
        _)))
  (return null))

(fn `Has Any Items in Inventory`
  (returns (Has :type Boolean))
  (locals (`L Has` :type Boolean))
  (for _array_element (`self.Inventory`)
    (if (!= (break `/Game/UltimateSurvivalPack/Blueprints/Structs/S_InventoryItem` _array_element) "None")
      (set `local.L Has` true)
      (break)))
  (return (`local.L Has`)))

(fn `Is Caller Local`
  (returns (`Is Local` :type Boolean))
  (bind _ascontroller (cast `Controller` (`self.GetOwner`))
    (:`then`
      (if (`Controller.IsLocalController` _ascontroller)
        (return true)
        (else
          (return false))))
    (:`CastFailed`
      (return false))))

(fn `Local On Inventory Updated`)

(fn `Remove Item`
  (params (`At Index` :type Integer) (Amount :type Integer) (`From Inventory` :type "/Game/UltimateSurvivalPack/Blueprints/Components/BP_MasterInventoryComponent Object Reference")))

(fn `Save Player Data`)

(fn `Swap Items`
  (params (`From Index` :type Integer) (`From Inventory` :type "/Game/UltimateSurvivalPack/Blueprints/Components/BP_MasterInventoryComponent Object Reference (by ref)") (`To Index` :type Integer) (`To Inventory` :type "/Game/UltimateSurvivalPack/Blueprints/Components/BP_MasterInventoryComponent Object Reference (by ref)"))
  (locals (`L Cached From` :type "/Game/UltimateSurvivalPack/Blueprints/Structs/S_InventoryItem Structure") (`L Cached To` :type "/Game/UltimateSurvivalPack/Blueprints/Structs/S_InventoryItem Structure")))

(fn `Use Item Call`
  (params (`At Index` :type Integer) (`From Inventory` :type "/Game/UltimateSurvivalPack/Blueprints/Components/BP_MasterInventoryComponent Object Reference")))