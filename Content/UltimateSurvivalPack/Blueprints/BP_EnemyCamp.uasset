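; Enemy camp actor that spawns enemies when a player enters its activation sphere and shows a "Restricted area" notification on local overlap.
; Once all spawned members die, it awards XP and skill points by damage share, notifies its target component and re-arms after a delay.
; Players leaving an inactive camp trigger a timed reset of enemies and respawnable actors.
; Editor events gather spawners and respawnables within the activation radius.
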(event `self.ReceiveBeginPlay`
  (bind _activation_collision (`self.Activation collision`))
  ;[0 0 0] Refresh collision
  (`PrimitiveComponent.SetCollisionEnabled` _activation_collision "NoCollision")
  (`KismetSystemLibrary.Delay` 0.2)
  (`PrimitiveComponent.SetCollisionEnabled` _activation_collision "QueryOnly"))

(event `Exec Enemy Camp`
  ;[0.1818 0.4948 0.1652] Execute Enemy Camp
  (if (not (`self.Defeated?`))
    (set `self.Active?` true)
    (for _array_element (`self.Spawners`)
      (`/Game/UltimateSurvivalPack/Blueprints/BP_Spawner.Spawn` _array_element self))))

(event `On Enemy Camp Defeated`
  ;[1 0.177 0.187] On Enemy Camp Defeated
  (`KismetSystemLibrary.Delay` 1.0) ; Effect Delay
  (`self.Reward Players`)
  (set `self.Defeated?` true)
  (set `self.Active?` false)
  (`self.Reset Defeated State`))

(event `On Member Dead`
  ;[0.4115 0 0] On Member Dead
  (for _array_element (`self.Spawners`)
    (bind _is_alive (`self.Is Enemy Alive` (`/Game/UltimateSurvivalPack/Blueprints/BP_Spawner.Spawned Actor` _array_element)))
    (if _is_alive
      (break)))
  (if (not _is_alive)
    (`self.On Enemy Camp Defeated`)))

(event `Reward Players`
  ;[0.2761 1 0] Reward Player
  (for (_array_element _array_index) (`self.PlayerDatabase`)
    (bind _leveling_component (`/Game/UltimateSurvivalPack/Blueprints/BFL_UMSPack.Get Leveling Component` _array_element))
    (`/Engine/EditorBlueprintResources/StandardMacros.IsValid` _leveling_component
      (:`Is Valid`
        (bind _returnvalue (/ (`|GetArrayItem` (`self.PlayerDamageDatabase`) _array_index) (`self.Global Enemy Health`)))
        (bind _returnvalue_2 (`KismetMathLibrary.FTrunc` (* _returnvalue (`KismetMathLibrary.Conv_IntToDouble` (`self.Experience Reward`)))))
        (`/Game/UltimateSurvivalPack/Blueprints/Components/BP_Player_ExperienceComponent.Add Experience` _leveling_component _returnvalue_2 true (make `/Game/UltimateSurvivalPack/Blueprints/Structs/S_Notification` (`KismetStringLibrary.Concat_StrStr` (`self.Name`) " Defeated Reward") (`KismetStringLibrary.Concat_StrStr` "+" (`KismetStringLibrary.Conv_IntToString` _returnvalue_2) " XP")))
        (bind _returnvalue_3 (`KismetMathLibrary.FTrunc` (* _returnvalue (`KismetMathLibrary.Conv_IntToDouble` (`self.Survivor Points`)))))
        (if (> _returnvalue_3 0)
          (`/Game/UltimateSurvivalPack/Blueprints/Components/BP_SkillTreeComponent.Add Experience` (`/Game/UltimateSurvivalPack/Blueprints/BFL_UMSPack.Get Skill Component` _array_element) "NewEnumerator0" _returnvalue_3))
        (`/Game/UltimateSurvivalPack/Blueprints/Components/BP_TargetComponent.Interacted` (`self.BP_TargetComponent`) _array_element)))))

(event `Stop Reset`
  (bind _reset_timer_handle (`self.Reset Timer Handle`))
  ;[1 1 1] Stop Reset Timer
  (if (`KismetSystemLibrary.K2_IsValidTimerHandle` _reset_timer_handle)
    (`KismetSystemLibrary.K2_ClearAndInvalidateTimerHandle` _reset_timer_handle)))

(event `self.Activation collision.OnComponentBeginOverlap`
  (params (OverlappedComponent :type "PrimitiveComponent Object Reference") (OtherActor :type "Actor Object Reference") (OtherComp :type "PrimitiveComponent Object Reference") (OtherBodyIndex :type Integer) (bFromSweep :type Boolean) (SweepResult :type "HitResult Structure (by ref)"))
  ;[0.01116 0.04167 0] Activate Camp
  (bind _ascharacter (cast `Character` OtherActor))
  (`/Engine/EditorBlueprintResources/StandardMacros.IsValid` (`/Game/UltimateSurvivalPack/Blueprints/BFL_UMSPack.Get Player Component` _ascharacter)
    (:`Is Valid`
      (if (`self.Active?`)
        (`self.Stop Reset`)
        (elif (<= (`KismetArrayLibrary.Array_Length` (`PrimitiveComponent.GetOverlappingActors` (`self.Activation collision`) "/Game/UltimateSurvivalPack/Blueprints/ThirdPersonCharacter.ThirdPersonCharacter_C")) 1)
          (`self.Exec Enemy Camp`))))))

(event `self.Activation collision.OnComponentEndOverlap`
  (params (OverlappedComponent :type "PrimitiveComponent Object Reference") (OtherActor :type "Actor Object Reference") (OtherComp :type "PrimitiveComponent Object Reference") (OtherBodyIndex :type Integer))
  ;[0.151 0 0] Deactive
  (bind _ascharacter (cast `Character` OtherActor))
  (`/Engine/EditorBlueprintResources/StandardMacros.IsValid` (`/Game/UltimateSurvivalPack/Blueprints/BFL_UMSPack.Get Player Component` _ascharacter)
    (:`Is Valid`
      (if (not (`self.Active?`))
        (`self.Reset Camp`)))))

(event `/Game/UltimateSurvivalPack/Blueprints/Interface/BPI_InventorySystem.Local Overlap`
  (params (Overlap :type Boolean))
  ;[0 0 0] Add Notify "Restricted Area"
  (if Overlap
    (`/Game/UltimateSurvivalPack/Blueprints/Components/BP_MissionComponent.CLIENT Add Notification` (`/Game/UltimateSurvivalPack/Blueprints/BFL_UMSPack.Get Mission Component` (`GameplayStatics.GetPlayerController` 0)) (make `/Game/UltimateSurvivalPack/Blueprints/Structs/S_Notification` "Restricted area" "Be aware of your surroundings"))))

(event `Detect Spawners`
  ;[1 0.3359 0] Editor Events
  (bind _outactors (`GameplayStatics.GetAllActorsOfClass` "/Game/UltimateSurvivalPack/Blueprints/BP_Spawner.BP_Spawner_C"))
  (for _array_element _outactors
    (if (<= (`self.GetDistanceTo` _array_element) (`SphereComponent.SphereRadius` (`self.Activation collision`)))
      (`KismetArrayLibrary.Array_AddUnique` (`self.Spawners`) _array_element))))

(event `Delete Spawners`
  ;[1 0.3359 0] Editor Events
  (`KismetArrayLibrary.Array_Clear` (`self.Spawners`)))

(event `Detect Respawnable Actors`
  ;[1 0.3359 0] Editor Events
  (bind _outactors (`GameplayStatics.GetAllActorsWithInterface` "/Game/UltimateSurvivalPack/Blueprints/Interface/BPI_Spawning.BPI_Spawning_C"))
  (for _array_element _outactors
    (if (<= (`self.GetDistanceTo` _array_element) (`SphereComponent.SphereRadius` (`self.Activation collision`)))
      (`KismetArrayLibrary.Array_AddUnique` (`self.Actors to Reset`) _array_element))))

(event `Delete Respawnable Actors`
  ;[1 0.3359 0] Editor Events
  (`KismetArrayLibrary.Array_Clear` (`self.Actors to Reset`)))

(event `Reset Camp`
  ;[0 0 0] Reset variables
  (bind _returnvalue (`KismetSystemLibrary.K2_SetTimerDelegate` (delegate `Reset`) 1.0))
  (set `self.Reset Timer Handle` _returnvalue)
  (`PrimitiveComponent.SetCollisionEnabled` (`self.Activation collision`) "NoCollision")
  (`PrimitiveComponent.SetCollisionEnabled` (`self.Area Collision`) "NoCollision"))

(event `Reset`
  ;[0 0 0] Reset variables
  (set `self.Active?` false)
  (set `self.Global Enemy Health` 0.0)
  (`KismetArrayLibrary.Array_Clear` (`self.PlayerDatabase`))
  (`KismetArrayLibrary.Array_Clear` (`self.PlayerDamageDatabase`))
  (for _array_element (`self.Spawners`)
    (bind _spawned_actor (`/Game/UltimateSurvivalPack/Blueprints/BP_Spawner.Spawned Actor` _array_element)
      (:`then`
        (`self.K2_DestroyActor` _spawned_actor))
      (:`else`)))
  (`PrimitiveComponent.SetCollisionEnabled` (`self.Activation collision`) "QueryOnly")
  (`PrimitiveComponent.SetCollisionEnabled` (`self.Area Collision`) "QueryOnly")
  (for _array_element_2 (`self.Actors to Reset`)
    (`/Engine/EditorBlueprintResources/StandardMacros.IsValid` _array_element_2
      (:`Is Valid`
        (message `/Game/UltimateSurvivalPack/Blueprints/Interface/BPI_Spawning.Request Respawn` _array_element_2)))))

(event `Reset Defeated State`
  ;[1 1 1] Reset Defeated State
  (`KismetSystemLibrary.Delay` (`self.Respawn Delay`))
  (set `self.Defeated?` false))

(fn `Get Interaction Data`
  (returns (`Interaction Text` :type Text))
  (return ""))

(fn `Get Team ID`
  (returns (`Team ID` :type Byte))
  (return 0))

(fn `Is Enemy Alive`
  (params (Actor :type "Actor Object Reference"))
  (returns (`Is Alive` :type Boolean))
  (`/Engine/EditorBlueprintResources/StandardMacros.IsValid` Actor
    (:`Is Valid`
      (return (`/Game/UltimateSurvivalPack/Blueprints/Components/BP_AI_DataComponent.Is Alive` (`self.GetComponentByClass` Actor "/Game/UltimateSurvivalPack/Blueprints/Components/BP_AI_DataComponent.BP_AI_DataComponent_C"))))
    (:`Is Not Valid`
      (return false))))

(fn `Local Can Overlap`
  (returns (Success :type Boolean))
  (bind _sphereradius (`SphereComponent.SphereRadius` (`self.Area Collision`)))
  (return (< (`self.GetSquaredDistanceTo` (`Controller.K2_GetPawn` (`GameplayStatics.GetPlayerController` 0))) (* _sphereradius _sphereradius))))

(fn `UserConstructionScript`
  (bind (_target_information_targettype _target_information_uniqueid _target_information_amount _target_information_marker) (break `/Game/UltimateSurvivalPack/Blueprints/Structs/S_TargetInformation` (`/Game/UltimateSurvivalPack/Blueprints/Components/BP_TargetComponent.Target Information` (`self.BP_TargetComponent`))))
  ;[1 1 1] Collision Contruction
  (`SphereComponent.SetSphereRadius` (`self.Area Collision`) (`self.Area Radius`) true)
  (`SphereComponent.SetSphereRadius` (`self.Activation collision`) (`self.Activation Distance`) true)
  ;[1 1 1] Setup Target Information
  (set `/Game/UltimateSurvivalPack/Blueprints/Components/BP_TargetComponent.Target Information` (make `/Game/UltimateSurvivalPack/Blueprints/Structs/S_TargetInformation` _target_information_targettype (`self.Unique ID`) _target_information_amount _target_information_marker self) (`self.BP_TargetComponent`)))