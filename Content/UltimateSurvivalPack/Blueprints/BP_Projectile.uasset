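; Projectile actor that ignores collision with its instigator and reacts to entering water.
; On the server, Tick runs a small sphere trace at its location to detect BP_Water.
; A water hit spawns a Niagara splash and sound, lowers the ProjectileMovement speed limit to simulate drag, and disables Tick so detection stops.
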(event `self.ReceiveBeginPlay`
  (`PrimitiveComponent.IgnoreActorWhenMoving` (`self.Sphere`) (`self.Instigator`) true))

(event `self.ReceiveTick`
  (params (DeltaSeconds :type "Float (single-precision)"))
  (bind _returnvalue (`self.K2_GetActorLocation`))
  (`/Engine/EditorBlueprintResources/ActorMacros.Switch Has Authority`
    (:`Authority`
      (bind (_outhit _returnvalue_2) (`KismetSystemLibrary.SphereTraceSingleForObjects` _returnvalue _returnvalue 5.0 (`|MakeArray` "ObjectTypeQuery7" :!type "EObjectTypeQuery Enum")))
      (if _returnvalue_2
        (bind (_bblockinghit _binitialoverlap _time _distance _location _impactpoint _normal _impactnormal _physmat _hitactor) (`GameplayStatics.BreakHitResult` _outhit))
        (cast `/Game/UltimateSurvivalPack/Blueprints/BP_Water` _hitactor)
        (`self.On Water Hit` _impactpoint)))))

(event `On Water Hit`
  (params (Location :type "Vector Structure"))
  ;[0.3102 1 0.4051] Water Effects
  (`NiagaraFunctionLibrary.SpawnSystemAtLocation` "/Game/UltimateSurvivalPack/Demo/Particles/Niagara/NS_WaterSplash_Big.NS_WaterSplash_Big" Location)
  (`GameplayStatics.SpawnSoundAtLocation` "/Game/UltimateSurvivalPack/Demo/Audio/SFX/CUE_WaterSplash.CUE_WaterSplash" Location (struct) 1.0 1.0 0.0 "/Game/UltimateSurvivalPack/Blueprints/Attenuation/SA_Footsteps.SA_Footsteps" null)
  (set `ProjectileMovementComponent.InitialSpeed` 800.0 (`self.ProjectileMovement`))
  (set `ProjectileMovementComponent.MaxSpeed` 800.0 (`self.ProjectileMovement`))
  (`self.SetActorTickEnabled` false))

(fn `UserConstructionScript`)