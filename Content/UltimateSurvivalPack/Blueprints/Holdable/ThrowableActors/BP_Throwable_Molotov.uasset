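; Throwable Molotov actor that starts a fire where it lands.
; On a hit of its object mesh, the server ignores Characters and surfaces too steep to count as floor, judged by the impact normal's Z.
; A valid ground hit spawns BP_Fire at the actor's location and destroys the Molotov, so wall and character hits leave it intact.
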(event `self.ReceiveBeginPlay`
  (`parent.ReceiveBeginPlay`))

(event `self.ObjectMesh.OnComponentHit`
  (params (HitComponent :type "PrimitiveComponent Object Reference") (OtherActor :type "Actor Object Reference") (OtherComp :type "PrimitiveComponent Object Reference") (NormalImpulse :type "Vector Structure") (Hit :type "HitResult Structure (by ref)"))
  (`/Engine/EditorBlueprintResources/ActorMacros.Switch Has Authority`
    (:`Authority`
      (cast `Character` OtherActor ; Ignore Character
        (:`CastFailed`
          ;[1 1 1] Filter Walls
          (if (>= (.z (`.ImpactNormal` (`GameplayStatics.BreakHitResult` Hit))) 0.5)
            ;[1 1 1] Spawn Fire
            (`|SpawnActorFromClass` "/Game/UltimateSurvivalPack/Blueprints/Holdable/Others/BP_Fire.BP_Fire_C" (`KismetMathLibrary.MakeTransform` (`self.K2_GetActorLocation`)) "Undefined" "OverrideRootScale" null null)
            ;[1 1 1] Destroy Actor
            (`self.K2_DestroyActor`)))))))

(fn `UserConstructionScript`
  (`parent.UserConstructionScript`))