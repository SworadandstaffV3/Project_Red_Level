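; Thrown spear projectile that damages what it hits, sticks there and can be picked up back into the inventory.
; Launches along ThrowVelocity via ProjectileMovement, ignoring its instigator.
; On stop it stops replicating, applies server-only melee point damage, attaches to the hit component or bone and enables interaction with custom-depth highlighting.
; Water hits spawn splash effects, lower the projectile's speed limits and disable actor tick.
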(event `self.ReceiveBeginPlay`
  (bind _projectilemovement (`self.ProjectileMovement`))
  (bind _returnvalue (`KismetMathLibrary.VSize` (`self.Throw Velocity`)))
  ;[1 0.2448 0.2448] Simulate Phyiscs and Add Velocity
  (`PrimitiveComponent.IgnoreActorWhenMoving` (`self.ObjectMesh`) (`self.Instigator`) true)
  (set `ProjectileMovementComponent.InitialSpeed` _returnvalue _projectilemovement)
  (set `ProjectileMovementComponent.MaxSpeed` _returnvalue _projectilemovement)
  (set `MovementComponent.Velocity` (`self.Throw Velocity`) _projectilemovement))

(event `/Game/UltimateSurvivalPack/Blueprints/Interface/BPI_InventorySystem.On Interacted`
  (params (Executor :type "Controller Object Reference"))
  (if (`self.Can be Interacted`)
    (`/Game/UltimateSurvivalPack/Blueprints/Components/BP_MasterInventoryComponent.Add Item` (`/Game/UltimateSurvivalPack/Blueprints/BFL_UMSPack.Get Inventory Component` Executor) (make `/Game/UltimateSurvivalPack/Blueprints/Structs/S_InventoryItem` "Spear" 1))
    (`self.K2_DestroyActor`)))

(event `self.ProjectileMovement.OnProjectileStop`
  (params (ImpactResult :type "HitResult Structure (by ref)"))
  (bind (_bblockinghit _binitialoverlap _time _distance _location _impactpoint _normal _impactnormal _physmat _hitactor _hitcomponent _hitbonename) (`GameplayStatics.BreakHitResult` ImpactResult))
  (bind _objectmesh (`self.ObjectMesh`))
  (set `self.Can be Interacted` true)
  (`self.SetReplicates` false)
  (`PrimitiveComponent.SetCollisionResponseToAllChannels` _objectmesh "ECR_Ignore")
  (`PrimitiveComponent.SetCollisionResponseToChannel` _objectmesh "ECC_Visibility" "ECR_Block")
  (`/Engine/EditorBlueprintResources/ActorMacros.Switch Has Authority`
    (:`Authority`
      (`GameplayStatics.ApplyPointDamage` _hitactor 35.0 (- _impactpoint (`self.K2_GetActorLocation` (`self.Instigator`))) ImpactResult (cast `Controller` (`self.GetOwner`) :!pure true) self "/Game/UltimateSurvivalPack/Blueprints/DamageType/DT_Melee.DT_Melee_C"))
    (:`Remote`
      _))
  (`self.K2_AttachToComponent` _hitcomponent _hitbonename "KeepWorld" "KeepWorld" "KeepWorld"))

(event `/Game/UltimateSurvivalPack/Blueprints/Interface/BPI_InventorySystem.Toggle Selected`
  (params (Toggle :type Boolean))
  (bind _objectmesh (`self.ObjectMesh`))
  (bind _objectmesh_2 (`self.ObjectMesh`))
  (if (`self.Can be Interacted`)
    (if Toggle
      (`PrimitiveComponent.SetRenderCustomDepth` _objectmesh_2 true)
      (`PrimitiveComponent.SetCustomDepthStencilValue` _objectmesh_2 1)
      (else
        (`PrimitiveComponent.SetRenderCustomDepth` _objectmesh false :!label _label)
        (`PrimitiveComponent.SetCustomDepthStencilValue` _objectmesh 0)))
    (else
      (goto _label))))

(event `self.On Water Hit`
  (params (Location :type "Vector Structure"))
  (`NiagaraFunctionLibrary.SpawnSystemAtLocation` "/Game/UltimateSurvivalPack/Demo/Particles/Niagara/NS_WaterSplash_Big.NS_WaterSplash_Big" Location)
  (`GameplayStatics.SpawnSoundAtLocation` "/Game/UltimateSurvivalPack/Demo/Audio/SFX/CUE_WaterSplash.CUE_WaterSplash" Location (struct) 1.0 1.0 0.0 "/Game/UltimateSurvivalPack/Blueprints/Attenuation/SA_Footsteps.SA_Footsteps" null)
  (set `ProjectileMovementComponent.InitialSpeed` 100.0 (`self.ProjectileMovement`))
  (set `ProjectileMovementComponent.MaxSpeed` 250.0 (`self.ProjectileMovement`))
  (`self.SetActorTickEnabled` false))

(fn `Get Interaction Data`
  (returns (`Interaction Text` :type Text))
  (return (select `bool` (`self.Can be Interacted`) :`true` "Pick up Spear." :!type "Text")))

(fn `Get Team ID`
  (returns (`Team ID` :type Byte))
  (return 0))

(fn `Local Can Overlap`
  (returns (Success :type Boolean))
  (return false))

(fn `UserConstructionScript`
  (`parent.UserConstructionScript`))