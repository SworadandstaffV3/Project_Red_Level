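; Holdable hammer that lets a player remove placed buildings, showing privileged cupboard zones to the local owner while it exists.
; A per-tick camera sphere trace shows the hammer widget over non-harvestable building actors.
; Holding primary action runs the widget's fill animation and timer, then requests destruction on the server.
; The server checks cupboard privilege, allowing removal when no cupboard is found, then notifies and multicasts a sound.
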(event `self.ReceiveBeginPlay`
  (bind _returnvalue (`self.GetOwner`))
  (`parent.ReceiveBeginPlay`)
  ;[1 1 1] Is Local
  (`/Engine/EditorBlueprintResources/StandardMacros.IsValid` _returnvalue
    (:`Is Valid`
      (bind _ascontroller (cast `Controller` _returnvalue))
      (if (`Controller.IsLocalController` _ascontroller)
        ;[1 1 1] Set Cupboard Zone Visibility
        (bind _outactors (`GameplayStatics.GetAllActorsOfClass` "/Game/UltimateSurvivalPack/Blueprints/Buildings/Final/BP_Cupboard.BP_Cupboard_C"))
        (for _array_element _outactors
          (if (`KismetArrayLibrary.Array_Contains` (`/Game/UltimateSurvivalPack/Blueprints/Buildings/Final/BP_Cupboard.Privilege Players` _array_element) (`/Game/UltimateSurvivalPack/Blueprints/Components/BP_PlayerComponent.Player Unique ID` (`/Game/UltimateSurvivalPack/Blueprints/BFL_UMSPack.Get Player Component` (`self.Instigator`))))
            (`SceneComponent.SetVisibility` (`/Game/UltimateSurvivalPack/Blueprints/Buildings/Final/BP_Cupboard.Zone` _array_element) true false)))))))

(event `self.ReceiveTick`
  (params (DeltaSeconds :type "Float (single-precision)"))
  (bind _returnvalue (`GameplayStatics.GetPlayerCameraManager` 0))
  (bind _widget (`self.Widget`))
  (bind _timer (`self.Timer`))
  (bind _returnvalue_2 (`PlayerCameraManager.GetCameraLocation` _returnvalue))
  (if (`self.Is Owner Local`)
    (bind (_outhit _returnvalue_3) (`KismetSystemLibrary.SphereTraceSingle` _returnvalue_2 (+ _returnvalue_2 (* (`KismetMathLibrary.GetForwardVector` (`PlayerCameraManager.GetCameraRotation` _returnvalue)) (`/Game/UltimateSurvivalPack/Blueprints/Components/BP_PlayerInventoryComponent.Interaction Distance` (`/Game/UltimateSurvivalPack/Blueprints/BFL_UMSPack.Get Inventory Component` (`GameplayStatics.GetPlayerController` 0))))) 3.0 "TraceTypeQuery1" true))
    (set `self.Hit` _outhit)
    (if _returnvalue_3
      (bind (_bblockinghit _binitialoverlap _time _distance _location _impactpoint _normal _impactnormal _physmat _hitactor) (`GameplayStatics.BreakHitResult` _outhit))
      (`/Engine/EditorBlueprintResources/StandardMacros.IsValid` (`self.GetComponentByClass` _hitactor "/Game/UltimateSurvivalPack/Blueprints/Buildings/Parent/BP_BuildingComponent.BP_BuildingComponent_C")
        (:`Is Valid`
          (cast `/Game/UltimateSurvivalPack/Blueprints/Buildings/Harvestable/Parent/BP_Harvestable` _hitactor
            (:`then`
              (`/Engine/EditorBlueprintResources/StandardMacros.IsValid` _widget :!label _label
                (:`Is Valid`
                  (`Widget.RemoveFromParent` _widget)
                  (set `self.Widget` null)
                  (if (`KismetSystemLibrary.K2_IsValidTimerHandle` _timer)
                    (`KismetSystemLibrary.K2_ClearAndInvalidateTimerHandle` _timer)))))
            (:`CastFailed`
              (`/Engine/EditorBlueprintResources/StandardMacros.IsValid` (`self.Widget`)
                (:`Is Not Valid`
                  (bind _returnvalue_4 (`|CreateWidget` "/Game/UltimateSurvivalPack/Widget/W_HammerInformation.W_HammerInformation_C"))
                  (bind _output_get (set `self.Widget` _returnvalue_4))
                  (`UserWidget.AddToViewport` _output_get 0))))))
        (:`Is Not Valid`
          (goto _label)))
      (else
        (goto _label)))))

(event `/Game/UltimateSurvivalPack/Blueprints/Interface/BPI_Player.Primary Action`
  (params (Pressed :type Boolean))
  (`self.Toggle Time` Pressed))

(event `self.ReceiveDestroyed`
  (bind _returnvalue (`self.GetOwner`))
  (bind _widget (`self.Widget`))
  (`/Engine/EditorBlueprintResources/StandardMacros.IsValid` _widget
    (:`Is Valid`
      (`Widget.RemoveFromParent` _widget)
      (set `self.Widget` null))
    (:`Is Not Valid`
      _))
  (`/Engine/EditorBlueprintResources/StandardMacros.IsValid` _returnvalue
    (:`Is Valid`
      (bind _ascontroller (cast `Controller` _returnvalue))
      (if (`Controller.IsLocalController` _ascontroller)
        ;[1 1 1] Set Cupboard Zone Visibility
        (bind _outactors (`GameplayStatics.GetAllActorsOfClass` "/Game/UltimateSurvivalPack/Blueprints/Buildings/Final/BP_Cupboard.BP_Cupboard_C"))
        (for _array_element _outactors
          (if (`KismetArrayLibrary.Array_Contains` (`/Game/UltimateSurvivalPack/Blueprints/Buildings/Final/BP_Cupboard.Privilege Players` _array_element) (`/Game/UltimateSurvivalPack/Blueprints/Components/BP_PlayerComponent.Player Unique ID` (`/Game/UltimateSurvivalPack/Blueprints/BFL_UMSPack.Get Player Component` (`self.Instigator`))))
            (`SceneComponent.SetVisibility` (`/Game/UltimateSurvivalPack/Blueprints/Buildings/Final/BP_Cupboard.Zone` _array_element) false false)))))))

(event `Toggle Time`
  (params (Toggle :type Boolean))
  (bind _widget (`self.Widget`))
  (bind _timer (`self.Timer`))
  (`/Engine/EditorBlueprintResources/StandardMacros.IsValid` (`self.Widget`)
    (:`Is Valid`
      (if Toggle
        (`/Game/UltimateSurvivalPack/Widget/W_HammerInformation.Play Animation` _widget)
        (if (not (`KismetSystemLibrary.K2_IsValidTimerHandle` (`self.Timer`)))
          (bind _returnvalue (`KismetSystemLibrary.K2_SetTimerDelegate` (delegate `Destroy Building`) (`WidgetAnimation.GetEndTime` (`/Game/UltimateSurvivalPack/Widget/W_HammerInformation.FillAnimation` _widget))))
          (set `self.Timer` _returnvalue))
        (else
          (`/Game/UltimateSurvivalPack/Widget/W_HammerInformation.Stop Animation` (`self.Widget`))
          (if (`KismetSystemLibrary.K2_IsValidTimerHandle` _timer)
            (`KismetSystemLibrary.K2_ClearAndInvalidateTimerHandle` _timer)))))))

(event `Destroy Building`
  (bind (_bblockinghit _binitialoverlap _time _distance _location _impactpoint _normal _impactnormal _physmat _hitactor) (`GameplayStatics.BreakHitResult` (`self.Hit`)))
  (`/Engine/EditorBlueprintResources/StandardMacros.IsValid` _hitactor
    (:`Is Valid`
      (`self.SERVER Destroy Building` _hitactor))))

(event `SERVER Destroy Building`
  (params (`Destroy Building` :type "Actor Object Reference"))
  (bind _assurvival_gamemode (cast `/Game/UltimateSurvivalPack/Blueprints/SurvivalGamemode` (`GameplayStatics.GetGameMode`)))
  (bind (_value _returnvalue) (`BlueprintMapLibrary.Map_Find` (`/Game/UltimateSurvivalPack/Blueprints/SurvivalGamemode.Building Actors` _assurvival_gamemode) (`/Game/UltimateSurvivalPack/Blueprints/Buildings/Parent/BP_BuildingComponent.Cupboard ID` (`self.GetComponentByClass` `Destroy Building` "/Game/UltimateSurvivalPack/Blueprints/Buildings/Parent/BP_BuildingComponent.BP_BuildingComponent_C"))))
  (if _returnvalue
    (`/Engine/EditorBlueprintResources/StandardMacros.IsValid` _value
      (:`Is Valid`
        (bind _asbp_cupboard (cast `/Game/UltimateSurvivalPack/Blueprints/Buildings/Final/BP_Cupboard` _value)
          (:`then`
            (if (`KismetArrayLibrary.Array_Contains` (`/Game/UltimateSurvivalPack/Blueprints/Buildings/Final/BP_Cupboard.Privilege Players` _asbp_cupboard) (`/Game/UltimateSurvivalPack/Blueprints/Components/BP_PlayerComponent.Player Unique ID` (`/Game/UltimateSurvivalPack/Blueprints/BFL_UMSPack.Get Player Component` (`self.Instigator`))))
              (`/Engine/EditorBlueprintResources/StandardMacros.IsValid` `Destroy Building` :!label _label_2
                (:`Is Valid`
                  (`self.K2_DestroyActor` `Destroy Building`)
                  (`self.K2_DestroyActor` `Destroy Building`)
                  (`/Game/UltimateSurvivalPack/Blueprints/Components/BP_Player_ExperienceComponent.CLIENT Add Notification` (`/Game/UltimateSurvivalPack/Blueprints/BFL_UMSPack.Get Leveling Component` (`GameplayStatics.GetPlayerController` 0)) (make `/Game/UltimateSurvivalPack/Blueprints/Structs/S_Notification` "Building Removed" "Building has been Removed"))
                  (`self.MULTICAST Play Destroy Effect`)))))
          (:`CastFailed`
            (goto _label_2))))
      (:`Is Not Valid`
        (goto _label_2)))
    (else
      (goto _label_2))))

(event `MULTICAST Play Destroy Effect`
  (`GameplayStatics.PlaySoundAtLocation` "/Game/UltimateSurvivalPack/Demo/Audio/Impact/WAV_BuildingDestroyed.WAV_BuildingDestroyed" (`self.K2_GetActorLocation`) (struct) 1.0 1.0 0.0 "/Game/UltimateSurvivalPack/Blueprints/Attenuation/SA_Footsteps.SA_Footsteps" null null))

(fn `UserConstructionScript`
  (`parent.UserConstructionScript`))