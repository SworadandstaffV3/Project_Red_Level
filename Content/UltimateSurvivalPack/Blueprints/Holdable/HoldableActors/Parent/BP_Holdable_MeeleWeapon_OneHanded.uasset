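; Parent Blueprint for one-handed melee weapons, handling networked attacks and blocking.
; Primary action checks durability and spends stamina, then the server gates a multicast of alternating montages by an action delay.
; A separate local attack request triggers a server sphere trace, applying skill-scaled damage once per actor and wearing durability.
; Aiming toggles shielding with a camera offset; blocked hits play effects, cost double durability and drop the shield at zero.
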(event `/Game/UltimateSurvivalPack/Blueprints/Interface/BPI_Player.Primary Action`
  (params (Pressed :type Boolean))
  (bind (_item_data_id _item_data_amount _item_data_cachedindex) (break `/Game/UltimateSurvivalPack/Blueprints/Structs/S_InventoryItem` (`self.Item Data`)))
  ;[1 1 1] Primary Action
  (if Pressed
    (if (and (not (`self.Is Shielding`)) (`/Game/UltimateSurvivalPack/Blueprints/Components/BP_PlayerInventoryComponent.Has Durability` (`/Game/UltimateSurvivalPack/Blueprints/BFL_UMSPack.Get Inventory Component` (`self.GetOwner`)) _item_data_cachedindex))
      (`/Engine/EditorBlueprintResources/StandardMacros.DoOnce` false :!label _label
        (:`Completed`
          (bind _returnvalue (`/Game/UltimateSurvivalPack/Blueprints/Components/BP_PlayerInventoryComponent.Decerase Stamina` (`/Game/UltimateSurvivalPack/Blueprints/BFL_UMSPack.Get Inventory Component` (`self.GetOwner`)) 15.0))
          (if _returnvalue
            (`self.SERVER Attack`)
            (else
              (goto _label :!via `Reset`))))))))

(event `Reset`
  ;[1 1 1] Primary Action
  (goto _label :!via `Reset`))

(event `Mutlicast Block Effect`
  (bind _returnvalue (`SceneComponent.K2_GetComponentLocation` (`self.Item Mesh`)))
  ;[1 1 1] Block Effect
  (`NiagaraFunctionLibrary.SpawnSystemAtLocation` "/Game/UltimateSurvivalPack/Demo/Particles/Niagara/NS_BlockedHit.NS_BlockedHit" _returnvalue)
  (`GameplayStatics.SpawnSoundAtLocation` "/Game/UltimateSurvivalPack/Demo/Audio/Impact/CUE_BlockedHit.CUE_BlockedHit" _returnvalue (struct) 1.0 1.0 0.0 "/Game/UltimateSurvivalPack/Blueprints/Attenuation/SA_Footsteps.SA_Footsteps" null))

(event `SERVER Attack`
  (bind _returnvalue (`self.GetOwner`))
  (bind (_item_data_id _item_data_amount _item_data_cachedindex) (break `/Game/UltimateSurvivalPack/Blueprints/Structs/S_InventoryItem` (`self.Item Data`)))
  ;[1 1 1] Has Desired Durability
  (if (`/Game/UltimateSurvivalPack/Blueprints/Components/BP_PlayerInventoryComponent.Has Durability` (`/Game/UltimateSurvivalPack/Blueprints/BFL_UMSPack.Get Inventory Component` _returnvalue) _item_data_cachedindex)
    ;[1 1 1] Action Delay
    (`/Engine/EditorBlueprintResources/StandardMacros.DoOnce` false :!label _label_2
      (:`Completed`
        (`|ExecutionSequence`
          (:`then_0`
            (`self.MULTICAST Attack`))
          (:`then_1`
            (`KismetSystemLibrary.Delay` (`self.Action Delay`))
            (`self.Reset` :!label _label_3)
            (goto _label_2 :!via `Reset`)))))
    (else
      (`/Game/UltimateSurvivalPack/Blueprints/Components/BP_MissionComponent.CLIENT Add Notification` (`/Game/UltimateSurvivalPack/Blueprints/BFL_UMSPack.Get Mission Component` _returnvalue) (make `/Game/UltimateSurvivalPack/Blueprints/Structs/S_Notification` "Melee Weapon" "You do not have enough durability to attack"))
      (goto _label_3))))

(event `MULTICAST Attack`
  ;[1 1 1] Play Attack on MULTICAST
  (bind _ascharacter (cast `Character` (`self.GetInstigator`)))
  (`/Engine/EditorBlueprintResources/StandardMacros.FlipFlop`
    (:`A`
      (`Character.PlayAnimMontage` _ascharacter (`self.Attack Montage 01`) 1.0 "None"))
    (:`B`
      (`Character.PlayAnimMontage` _ascharacter (`self.Attack Montage 02`) 1.0 "None")))
  (if (`Pawn.IsLocallyControlled` _ascharacter)
    (`PlayerController.ClientStartCameraShake` :`self` (`GameplayStatics.GetPlayerController` 0) :`Shake` "/Game/UltimateSurvivalPack/Blueprints/Other/Attack_CameraShake.Attack_CameraShake_C")))

(event `On Shielding Hit`
  (bind (_item_data_id _item_data_amount _item_data_cachedindex) (break `/Game/UltimateSurvivalPack/Blueprints/Structs/S_InventoryItem` (`self.Item Data`)))
  (bind _returnvalue (`/Game/UltimateSurvivalPack/Blueprints/BFL_UMSPack.Get Inventory Component` (`self.GetOwner`)))
  ;[1 1 1] On shielding hit (Called from server damage handled, Playerinventorycomponent)
  (`/Game/UltimateSurvivalPack/Blueprints/Components/BP_PlayerInventoryComponent.Decerase Durability` _returnvalue _item_data_cachedindex (* (`self.Minus Durability`) 2.0))
  (`self.Mutlicast Block Effect`)
  (if (<= (`.Durability_17_EACE862B4A67C4626DE918B12D7D20BB` (break `/Game/UltimateSurvivalPack/Blueprints/Structs/S_InventoryItem` (`|GetArrayItem` (`/Game/UltimateSurvivalPack/Blueprints/Components/BP_MasterInventoryComponent.Inventory` _returnvalue) _item_data_cachedindex))) 0.0)
    (`self.SERVER Set Shielding` false)))

(event `/Game/UltimateSurvivalPack/Blueprints/Interface/BPI_Player.Local Request Attack`
  ;[1 1 1] Local Attack Request
  (if (`self.Is Owner Local`)
    (`self.SERVER Init Attack`)))

(event `SERVER Set Shielding`
  (params (`Is Shielding` :type Boolean))
  (bind (_item_data_id _item_data_amount _item_data_cachedindex) (break `/Game/UltimateSurvivalPack/Blueprints/Structs/S_InventoryItem` (`self.Item Data`)))
  ;[1 1 1] Server set shielding, if no durability force disable
  (if `Is Shielding`
    (if (> (`.Durability_17_EACE862B4A67C4626DE918B12D7D20BB` (break `/Game/UltimateSurvivalPack/Blueprints/Structs/S_InventoryItem` (`|GetArrayItem` (`/Game/UltimateSurvivalPack/Blueprints/Components/BP_MasterInventoryComponent.Inventory` (`/Game/UltimateSurvivalPack/Blueprints/BFL_UMSPack.Get Inventory Component` (`self.GetOwner`))) _item_data_cachedindex))) 0.0)
      (set `self.Is Shielding` `Is Shielding` :!label _label_4)
      (else
        (set `self.Is Shielding` false)))
    (else
      (goto _label_4)))
  (`self.CLIENT On Shielding` (`self.Is Shielding`)))

(event `/Game/UltimateSurvivalPack/Blueprints/Interface/BPI_Player.Aiming Action`
  (params (Toggle :type Boolean))
  ;[1 1 1] Toggle Shielding
  (`parent.Aiming Action` Toggle)
  (`self.SERVER Set Shielding` Toggle))

(event `SERVER Init Attack`
  ;[1 1 1] Init Attack
  (`self.Apply Damage`))

(event `CLIENT On Shielding`
  (params (Condition :type Boolean))
  ;[1 1 1] Client on Shielding change
  (if Condition
    (message `/Game/UltimateSurvivalPack/Blueprints/Interface/BPI_Player.Start Aiming` (`self.Instigator`) (0.0 70.0 10.0) 220.0)
    (else
      (message `/Game/UltimateSurvivalPack/Blueprints/Interface/BPI_Player.Stop Aiming` (`self.Instigator`)))))

(fn `Apply Damage`
  (locals (`L Hit Actors` :type "Array of Actor Object Reference") (`L Damaged` :type Boolean))
  (bind _returnvalue (`self.GetInstigator`))
  (bind _returnvalue_2 (`self.K2_GetActorLocation`))
  (bind (_item_data_id _item_data_amount _item_data_cachedindex) (break `/Game/UltimateSurvivalPack/Blueprints/Structs/S_InventoryItem` (`self.Item Data`)))
  (bind _returnvalue_3 (+ (`self.K2_GetActorLocation` _returnvalue) (* (`self.GetActorForwardVector` _returnvalue) 90.0)))
  (bind _outhits (`KismetSystemLibrary.SphereTraceMulti` _returnvalue_3 _returnvalue_3 90.0 "TraceTypeQuery1" false (`|MakeArray` (`self.GetInstigator`) :!type "Actor Object Reference")))
  (for _array_element _outhits
    (bind (_bblockinghit _binitialoverlap _time _distance _location _impactpoint _normal _impactnormal _physmat _hitactor) (`GameplayStatics.BreakHitResult` _array_element))
    (if (not (`KismetArrayLibrary.Array_Contains` (`local.L Hit Actors`) _hitactor))
      (`GameplayStatics.ApplyPointDamage` _hitactor (* (`.MeeleDamageMultiplier_2_AFBC246445B8D9BF2BBABD91EA2F11A8` (break `/Game/UltimateSurvivalPack/Blueprints/Structs/S_CurrentSkills` (`/Game/UltimateSurvivalPack/Blueprints/Components/BP_SkillTreeComponent.Current Skill Abilities` (`/Game/UltimateSurvivalPack/Blueprints/BFL_UMSPack.Get Skill Component` (`self.GetOwner`))))) (`self.Damage`)) (`KismetMathLibrary.Normal` (- (`self.K2_GetActorLocation` _hitactor) (`self.K2_GetActorLocation` (`self.Instigator`)))) (`GameplayStatics.MakeHitResult` false false 0.0 0.0 _returnvalue_2 _returnvalue_2) (`self.GetInstigatorController`) self (`self.Damage Type`))
      (`KismetArrayLibrary.Array_Add` (`local.L Hit Actors`) _hitactor)
      (if (`Actor.bCanBeDamaged` _hitactor)
        (set `local.L Damaged` true))))
  (if (`local.L Damaged`)
    (if (> (`KismetArrayLibrary.Array_Length` (`local.L Hit Actors`)) 0)
      (`/Game/UltimateSurvivalPack/Blueprints/Components/BP_PlayerInventoryComponent.Decerase Durability` (`/Game/UltimateSurvivalPack/Blueprints/BFL_UMSPack.Get Inventory Component` (`self.GetOwner`)) _item_data_cachedindex (`self.Minus Durability`))))
  (return))

(fn `UserConstructionScript`
  (`parent.UserConstructionScript`))