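; Explosion actor that deals area damage, pushes physics objects and plays a positional sound when spawned, then destroys itself shortly after its particle effect ends.
; On authority it emits an AI noise and sphere-traces for targets, applying point damage once per actor with linear distance falloff, credited to its owner.
; Pawns behind world-static geometry are spared, while other actors skip that check.
; Actor scale drives both damage and impulse radius.
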(event `self.ReceiveBeginPlay`
  (`/Engine/EditorBlueprintResources/ActorMacros.Switch Has Authority`
    (:`Authority`
      (`self.Apply Explosion Damage`)
      (`self.MakeNoise` 1.0 null (`self.K2_GetActorLocation`) 3000.0 "Noise"))
    (:`Remote`
      _))
  ;[1 1 1] Fire Impulse
  (`RadialForceComponent.FireImpulse` (`self.RadialForce`))
  (`GameplayStatics.SpawnSoundAtLocation` "/Game/UltimateSurvivalPack/Demo/Audio/Explosion/CUE_Explosion.CUE_Explosion" (`self.K2_GetActorLocation`) (struct) 1.0 1.0 0.0 "/Game/UltimateSurvivalPack/Blueprints/Attenuation/SA_Explosion.SA_Explosion" null))

(event `self.ParticleSystem.OnSystemFinished`
  (params (PSystem :type "ParticleSystemComponent Object Reference"))
  ;[1 1 1] Remove Actor After Emitter Finished
  (`KismetSystemLibrary.Delay` 1.0)
  (`self.K2_DestroyActor`))

(fn `Apply Explosion Damage`
  (locals (`L ActorList` :type "Array of Actor Object Reference"))
  (bind _returnvalue (`self.K2_GetActorLocation`))
  (bind _returnvalue_x (`KismetMathLibrary.BreakVector` (`self.GetActorScale3D`)))
  (bind _returnvalue_x_2 (`KismetMathLibrary.BreakVector` (`self.GetActorScale3D`)))
  (bind (_outhits _returnvalue_2) (`KismetSystemLibrary.SphereTraceMulti` _returnvalue _returnvalue (* _returnvalue_x_2 100.0) "TraceTypeQuery3"))
  (if _returnvalue_2
    (for _array_element _outhits
      (bind (_bblockinghit _binitialoverlap _time _distance _location _impactpoint _normal _impactnormal _physmat _hitactor) (`GameplayStatics.BreakHitResult` _array_element))
      (if (not (`KismetArrayLibrary.Array_Contains` (`local.L ActorList`) _hitactor))
        (cast `Pawn` _hitactor
          (:`then`
            ;[1 1 1] Is Actor Behind Wall?
            (bind (_outhit _returnvalue_3) (`KismetSystemLibrary.LineTraceSingleForObjects` (`self.K2_GetActorLocation`) (+ (`self.K2_GetActorLocation` _hitactor) (0.0 0.0 10.0)) (`|MakeArray` "ObjectTypeQuery1" :!type "EObjectTypeQuery Enum")))
            (if (not _returnvalue_3)
              (`GameplayStatics.ApplyPointDamage` _hitactor (`KismetMathLibrary.Conv_IntToDouble` (`KismetMathLibrary.FTrunc` (* (- 1.0 (`KismetMathLibrary.FClamp` (/ (`self.GetDistanceTo` _hitactor self) (* _returnvalue_x 100.0)))) 300.0))) (`KismetMathLibrary.Normal` (- (`self.K2_GetActorLocation` _hitactor) (`self.K2_GetActorLocation`))) (`GameplayStatics.MakeHitResult` false) (cast `Controller` (`self.GetOwner`) :!pure true) (`self.GetOwner`) "/Game/UltimateSurvivalPack/Blueprints/DamageType/DT_Explosion.DT_Explosion_C" :!label _label)
              (`KismetArrayLibrary.Array_Add` (`local.L ActorList`) _hitactor)))
          (:`CastFailed`
            (goto _label)))))
    (return)))

(fn `UserConstructionScript`
  (bind _returnvalue_x (`KismetMathLibrary.BreakVector` (`self.GetActorScale3D`)))
  (set `RadialForceComponent.Radius` (* _returnvalue_x 110.0) (`self.RadialForce`)))