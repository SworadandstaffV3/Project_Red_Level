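; BP_Spawner is a spawn point that creates an enemy for an Enemy Camp at its own transform.
; Its Spawn event only spawns when no valid SpawnedActor exists, so each spawner holds one enemy at a time.
; It links the enemy's BP_AI_DataComponent to the camp and adds its health to the camp's GlobalEnemyHealth, which is used to divide rewards between players.
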(event `Spawn`
  (params (`Enemy Camp` :type "/Game/UltimateSurvivalPack/Blueprints/BP_EnemyCamp Object Reference"))
  ;[0 0 0] Spawn Enemy
  (`/Engine/EditorBlueprintResources/StandardMacros.IsValid` (`self.Spawned Actor`)
    (:`Is Not Valid`
      (bind _returnvalue (`|SpawnActorFromClass` (`self.Enemy`) (`self.GetTransform`) "AdjustIfPossibleButAlwaysSpawn" "OverrideRootScale" null null))
      (bind _output_get (set `self.Spawned Actor` _returnvalue))
      (`/Engine/EditorBlueprintResources/StandardMacros.IsValid` _output_get
        (:`Is Valid`
          (bind _returnvalue_2 (`self.GetComponentByClass` _output_get "/Game/UltimateSurvivalPack/Blueprints/Components/BP_AI_DataComponent.BP_AI_DataComponent_C"))
          (set `/Game/UltimateSurvivalPack/Blueprints/Components/BP_AI_DataComponent.EnemyCamp` `Enemy Camp` _returnvalue_2)
          ;;[0.375 0.147 0.02891] Needed for Enemy Camp to divide reward between each players
          (set `/Game/UltimateSurvivalPack/Blueprints/BP_EnemyCamp.Global Enemy Health` (+ (`/Game/UltimateSurvivalPack/Blueprints/Components/BP_AI_DataComponent.Health` _returnvalue_2) (`/Game/UltimateSurvivalPack/Blueprints/BP_EnemyCamp.Global Enemy Health` `Enemy Camp`)) `Enemy Camp`))))))

(fn `UserConstructionScript`)