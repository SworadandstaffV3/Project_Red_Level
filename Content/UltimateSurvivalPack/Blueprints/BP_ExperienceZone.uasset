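; BP_ExperienceZone is a box trigger that periodically grants skill experience to characters standing inside it.
; On the server, overlap events add and remove each character's controller in PlayersInZone.
; A looping timer starts when none is running, fires every Delay seconds and is cleared when the zone empties.
; Each tick passes the configured Category and experience amount to every tracked controller's skill component.
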(event `self.Box.OnComponentEndOverlap`
  (params (OverlappedComponent :type "PrimitiveComponent Object Reference") (OtherActor :type "Actor Object Reference") (OtherComp :type "PrimitiveComponent Object Reference") (OtherBodyIndex :type Integer))
  (bind _players_in_zone (`self.Players In Zone`))
  (bind _ascharacter (cast `Character` OtherActor))
  (`/Engine/EditorBlueprintResources/ActorMacros.Switch Has Authority`
    (:`Authority`
      (`KismetArrayLibrary.Array_RemoveItem` _players_in_zone (`Pawn.GetController` _ascharacter))
      (if (<= (`KismetArrayLibrary.Array_Length` _players_in_zone) 0)
        (`KismetSystemLibrary.K2_ClearAndInvalidateTimerHandle` (`self.XP Timer`))))))

(event `self.Box.OnComponentBeginOverlap`
  (params (OverlappedComponent :type "PrimitiveComponent Object Reference") (OtherActor :type "Actor Object Reference") (OtherComp :type "PrimitiveComponent Object Reference") (OtherBodyIndex :type Integer) (bFromSweep :type Boolean) (SweepResult :type "HitResult Structure (by ref)"))
  (bind _ascharacter (cast `Character` OtherActor))
  (`/Engine/EditorBlueprintResources/ActorMacros.Switch Has Authority`
    (:`Authority`
      (`KismetArrayLibrary.Array_Add` (`self.Players In Zone`) (`Pawn.GetController` _ascharacter))
      (if (not (`KismetSystemLibrary.K2_IsValidTimerHandle` (`self.XP Timer`)))
        (bind _returnvalue (`KismetSystemLibrary.K2_SetTimerDelegate` (delegate `Add Experience Timer`) (`self.Delay`) true))
        (set `self.XP Timer` _returnvalue)))))

(event `Add Experience Timer`
  (for _array_element (`self.Players In Zone`)
    (`/Game/UltimateSurvivalPack/Blueprints/Components/BP_SkillTreeComponent.Add Experience` (`/Game/UltimateSurvivalPack/Blueprints/BFL_UMSPack.Get Skill Component` _array_element) (`self.Category`) (`self.Add Experience`))))

(fn `UserConstructionScript`)