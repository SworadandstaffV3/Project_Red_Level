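; Placement ghost for the wooden wall in the building system, whose five mesh segments follow the ground height individually.
; Each segment runs a short vertical WorldStatic line trace, with debug drawing, and snaps to the hit height or resets to zero.
; Placement passes only if the parent condition and all five traces succeed, though segments adjust either way.
; Custom rotation applies the current rotation directly, and the additive offset is zero.
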(fn `Additive Vector`
  (params (`Additive Vector` :type "Vector Structure"))
  (returns (`Additive Vector` :type "Vector Structure"))
  (return (0.0 0.0 0.0)))

(fn `Custom Condition Pass`
  (params (Hit :type "HitResult Structure") (`Locked Location` :type Boolean))
  (returns (Return :type Boolean))
  (bind _return (`parent.Custom Condition Pass` Hit false)) ; Is Build Type = Building?
  (if _return
    (bind _return_2 (`self.Do Height Trace` (`self.StaticMesh5`)))
    (bind _return_3 (`self.Do Height Trace` (`self.StaticMesh4`)))
    (bind _return_4 (`self.Do Height Trace` (`self.StaticMesh3`)))
    (bind _return_5 (`self.Do Height Trace` (`self.StaticMesh2`)))
    (bind _return_6 (`self.Do Height Trace` (`self.StaticMesh1`)))
    (return (and _return_6 _return_5 _return_4 _return_3 _return_2))
    (else
      (`self.Do Height Trace` (`self.StaticMesh5`))
      (`self.Do Height Trace` (`self.StaticMesh4`))
      (`self.Do Height Trace` (`self.StaticMesh3`))
      (`self.Do Height Trace` (`self.StaticMesh2`))
      (`self.Do Height Trace` (`self.StaticMesh1`))
      (return false))))

(fn `Custom Rotation`
  (params (Hit :type "HitResult Structure") (`Current Rotation` :type "Rotator Structure") (`Socket Rotation` :type "Rotator Structure") (`Locked Location` :type Boolean) (`Rotation Mode` :type "/Game/UltimateSurvivalPack/Blueprints/Enum/E_RotationMode Enum" :default "NewEnumerator0"))
  (`self.K2_SetActorRotation` `Current Rotation`)
  (return))

(fn `Do Height Trace`
  (params (Component :type "StaticMeshComponent Object Reference"))
  (returns (Return :type Boolean))
  (bind (_returnvalue_x _returnvalue_y _returnvalue_z) (`KismetMathLibrary.BreakVector` (`self.K2_GetActorLocation`)))
  (bind (_returnvalue_x_2 _returnvalue_y_2) (`KismetMathLibrary.BreakVector` (`SceneComponent.K2_GetComponentLocation` Component)))
  (bind (_relativelocation_x _relativelocation_y) (`KismetMathLibrary.BreakVector` (`SceneComponent.RelativeLocation` Component)))
  (bind _returnvalue (`KismetMathLibrary.MakeVector` _returnvalue_x_2 _returnvalue_y_2 _returnvalue_z))
  (bind (_outhit _returnvalue_2) (`KismetSystemLibrary.LineTraceSingleForObjects` :`Start` (+ _returnvalue (0.0 0.0 125.0)) :`End` (- _returnvalue (0.0 0.0 125.0)) :`ObjectTypes` (`|MakeArray` "ObjectTypeQuery1" :!type "EObjectTypeQuery Enum") :`DrawDebugType` "ForOneFrame"))
  (if _returnvalue_2
    (`SceneComponent.K2_SetRelativeLocation` Component (`KismetMathLibrary.MakeVector` _relativelocation_x _relativelocation_y (- (.z (`.ImpactPoint` (`GameplayStatics.BreakHitResult` _outhit))) (.z (`self.K2_GetActorLocation`)))) false false)
    (return true)
    (else
      (`SceneComponent.K2_SetRelativeLocation` Component (`KismetMathLibrary.MakeVector` _relativelocation_x _relativelocation_y) false false)
      (return false))))

(fn `UserConstructionScript`
  (`parent.UserConstructionScript`))