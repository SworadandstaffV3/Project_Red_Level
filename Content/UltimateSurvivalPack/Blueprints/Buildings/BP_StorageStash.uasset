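; BP_StorageStash is an interactable storage building that gives players access to a chest inventory, prompted as "Open Stash".
; On interaction it registers the executor's inventory component with its chest inventory component, then tells that component to open the stash's inventory.
; Selection toggles custom depth and stencil on the chest mesh for highlighting.
; It reports a fixed team ID and disallows local overlap.
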(event `/Game/UltimateSurvivalPack/Blueprints/Interface/BPI_InventorySystem.On Interacted`
  (params (Executor :type "Controller Object Reference"))
  (bind _returnvalue (`/Game/UltimateSurvivalPack/Blueprints/BFL_UMSPack.Get Inventory Component` Executor))
  (bind _bp_chestinventorycomponent (`self.BP_ChestInventoryComponent`))
  (`KismetArrayLibrary.Array_AddUnique` (`/Game/UltimateSurvivalPack/Blueprints/Components/BP_ChestInventoryComponent.Controlling Components` (`self.BP_ChestInventoryComponent`)) _returnvalue)
  (`/Game/UltimateSurvivalPack/Blueprints/Components/BP_PlayerInventoryComponent.Open Chest Inventory` _returnvalue _bp_chestinventorycomponent true (`/Game/UltimateSurvivalPack/Blueprints/Components/BP_MasterInventoryComponent.Inventory` _bp_chestinventorycomponent)))

(event `/Game/UltimateSurvivalPack/Blueprints/Interface/BPI_InventorySystem.Toggle Selected`
  (params (Toggle :type Boolean))
  (bind _chest (`self.Chest`))
  (bind _chest_2 (`self.Chest`))
  (if Toggle
    (`PrimitiveComponent.SetRenderCustomDepth` _chest_2 true)
    (`PrimitiveComponent.SetCustomDepthStencilValue` _chest_2 1)
    (else
      (`PrimitiveComponent.SetRenderCustomDepth` _chest false)
      (`PrimitiveComponent.SetCustomDepthStencilValue` _chest 0))))

(fn `Get Interaction Data`
  (returns (`Interaction Text` :type Text))
  (return "Open Stash"))

(fn `Get Team ID`
  (returns (`Team ID` :type Byte))
  (return 0))

(fn `Local Can Overlap`
  (returns (Success :type Boolean))
  (return false))

(fn `UserConstructionScript`)