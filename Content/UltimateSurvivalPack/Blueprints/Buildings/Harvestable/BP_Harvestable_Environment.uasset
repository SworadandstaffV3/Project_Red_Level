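; Environment harvestable that players interact with to collect items and that regrows after a delay.
; Interacting while not growing drops the data-defined items, awards skill experience to the executor, and starts a timer from the first stage's growth time.
; The replicated IsGrowing flag's RepNotify clears the mesh during regrowth and restores the first-stage mesh afterwards.
; Net dormancy is flushed on each state change to push replication.
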(event `self.ReceiveBeginPlay`
  ;[1 1 1] Begin Play Load
  (if (not (`self.Is Growing`))
    (`self.Load Stage` 0)
    (else
      (`StaticMeshComponent.SetStaticMesh` (`self.StaticMesh`) null))))

(event `/Game/UltimateSurvivalPack/Blueprints/Interface/BPI_InventorySystem.On Interacted`
  (params (Executor :type "Controller Object Reference"))
  ;[1 1 1] On Interacted
  (if (not (`self.Is Growing`))
    ;;[1 1 1] Drop Items
    (`self.Drop Items` (`.ItemsToDrop_11_D6FCA423474F33007BCD3FB01B4B586E` (break `/Game/UltimateSurvivalPack/Blueprints/Structs/S_HarvestableData` (`self.Harvestable Data`))))
    ;;[1 1 1] Add Skill Epxperience
    (`/Game/UltimateSurvivalPack/Blueprints/Components/BP_SkillTreeComponent.Add Experience` (`/Game/UltimateSurvivalPack/Blueprints/BFL_UMSPack.Get Skill Component` Executor) "NewEnumerator0" 75)
    ;;[1 1 1] Update And Replicate
    (set `self.Is Growing` true)
    (`self.FlushNetDormancy`)
    (`KismetSystemLibrary.Delay` (`KismetMathLibrary.Conv_IntToDouble` (`.GrowthTime_5_B8A89A414F14770DA75F77A924154985` (break `/Game/UltimateSurvivalPack/Blueprints/Structs/S_HarvestableStages` (`|GetArrayItem` (`.HarvestableStages_3_6500A21C48D3CEBEB49AFA8AF2653873` (break `/Game/UltimateSurvivalPack/Blueprints/Structs/S_HarvestableData` (`self.Harvestable Data`))))))))
    (set `self.Is Growing` false)
    (`self.FlushNetDormancy`)))

(fn `OnRep_Is Growing`
  (if (`self.Is Growing`)
    (`StaticMeshComponent.SetStaticMesh` (`self.StaticMesh`) null)
    (else
      (`StaticMeshComponent.SetStaticMesh` (`self.StaticMesh`) (`.Mesh_2_0A8788E245A70711D7885D99C17B05F7` (break `/Game/UltimateSurvivalPack/Blueprints/Structs/S_HarvestableStages` (`|GetArrayItem` (`.HarvestableStages_3_6500A21C48D3CEBEB49AFA8AF2653873` (break `/Game/UltimateSurvivalPack/Blueprints/Structs/S_HarvestableData` (`self.Harvestable Data`))))))))))

(fn `UserConstructionScript`
  (`parent.UserConstructionScript`))