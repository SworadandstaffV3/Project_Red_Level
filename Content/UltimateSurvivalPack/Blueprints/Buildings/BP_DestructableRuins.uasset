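; BP_DestructableRuins is a building ruins actor that shatters as soon as it begins play, using a destructible mesh assigned in the construction script.
; It replaces every material slot with one dynamic instance of M_TransparentRuins, then applies damage and impulse at the actor's location.
; A timeline animates that material's Opacity parameter, so all slots change transparency together.
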(event `self.ReceiveBeginPlay`
  (bind _returnvalue (`self.K2_GetActorLocation`))
  (bind _returnvalue_2 (`KismetMaterialLibrary.CreateDynamicMaterialInstance` "/Game/UltimateSurvivalPack/Demo/Material/Environment/M_TransparentRuins.M_TransparentRuins"))
  (bind _output_get (set `self.Dynamic Material` _returnvalue_2))
  (for _index (range (`PrimitiveComponent.GetNumMaterials` (`self.Destructible`)))
    (`PrimitiveComponent.SetMaterial` (`self.Destructible`) _index _output_get))
  (`DestructibleComponent.ApplyDamage` (`self.Destructible`) 100.0 _returnvalue _returnvalue 200.0)
  (bind (_direction _alpha) (`Timeline|Timeline_0` :`NewTime` 0.0)
    (:`Update`
      (`MaterialInstanceDynamic.SetScalarParameterValue` (`self.Dynamic Material`) "Opacity" _alpha))))

(fn `UserConstructionScript`
  (`DestructibleComponent.SetDestructibleMesh` (`self.Destructible`) (`self.Destructible Mesh`)))