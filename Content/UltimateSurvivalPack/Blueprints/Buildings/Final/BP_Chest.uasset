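; BP_Chest is an interactable storage chest, apparently for the building system.
; Interacting registers the player's inventory component as a controller of the chest's inventory component and opens that inventory.
; Selection toggles custom-depth highlighting and plays or reverses a timeline that tilts the chest part.
; An optional cupboard-based access check exists but is left unconnected, so interaction is unrestricted.
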(event `/Game/UltimateSurvivalPack/Blueprints/Interface/BPI_InventorySystem.On Interacted`
  (params (Executor :type "Controller Object Reference"))
  (bind _returnvalue (`/Game/UltimateSurvivalPack/Blueprints/BFL_UMSPack.Get Inventory Component` Executor))
  (bind _bp_chestinventorycomponent (`self.BP_ChestInventoryComponent`))
  ;[0.3083 0.573 1] On Interacted
  (`KismetArrayLibrary.Array_AddUnique` (`/Game/UltimateSurvivalPack/Blueprints/Components/BP_ChestInventoryComponent.Controlling Components` (`self.BP_ChestInventoryComponent`)) _returnvalue)
  (`/Game/UltimateSurvivalPack/Blueprints/Components/BP_PlayerInventoryComponent.Open Chest Inventory` _returnvalue _bp_chestinventorycomponent true (`/Game/UltimateSurvivalPack/Blueprints/Components/BP_MasterInventoryComponent.Inventory` _bp_chestinventorycomponent)))

(event `/Game/UltimateSurvivalPack/Blueprints/Interface/BPI_InventorySystem.Toggle Selected`
  (params (Toggle :type Boolean))
  (bind _chestpart (`self.ChestPart`))
  (bind _chestpart_2 (`self.ChestPart`))
  ;[1 1 1] On Selected
  (`self.Toggle Chest` Toggle)
  (if Toggle
    (`PrimitiveComponent.SetRenderCustomDepth` _chestpart_2 true)
    (`PrimitiveComponent.SetRenderCustomDepth` (`self.Chest`) true)
    (`PrimitiveComponent.SetCustomDepthStencilValue` _chestpart_2 1)
    (`PrimitiveComponent.SetCustomDepthStencilValue` (`self.Chest`) 1)
    (else
      (`PrimitiveComponent.SetRenderCustomDepth` _chestpart false)
      (`PrimitiveComponent.SetRenderCustomDepth` (`self.Chest`) false)
      (`PrimitiveComponent.SetCustomDepthStencilValue` _chestpart 0)
      (`PrimitiveComponent.SetCustomDepthStencilValue` (`self.Chest`) 0))))

(event `Toggle Chest`
  (params (Toggle :type Boolean))
  ;[1 1 1] Chest Open Animation
  (if Toggle
    (bind (_direction _alpha) (`Timeline|Animation` :!label _label)
      (:`Update`
        (`SceneComponent.K2_SetRelativeRotation` (`self.ChestPart`) (`KismetMathLibrary.MakeRotator` 0.0 (* _alpha 15.0)) false false)))
    (else
      (goto _label :!via `Reverse`))))

(fn `Get Interaction Data`
  (returns (`Interaction Text` :type Text))
  (return "Open Chest"))

(fn `Get Team ID`
  (returns (`Team ID` :type Byte))
  (return 0))

(fn `Local Can Overlap`
  (returns (Success :type Boolean))
  (return false))

(fn `UserConstructionScript`)