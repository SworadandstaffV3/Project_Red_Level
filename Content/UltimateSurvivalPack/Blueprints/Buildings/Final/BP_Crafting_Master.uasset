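; BP_Crafting_Master is the master Blueprint for interactable crafting stations in the survival pack's buildings.
; On interaction it gets the executor's inventory component and opens crafting on the client with the station's CraftingDataTable.
; Selection toggles custom depth and stencil on the static mesh.
; It supplies an "Open {name}" prompt and always returns false for local overlap.
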(event `/Game/UltimateSurvivalPack/Blueprints/Interface/BPI_InventorySystem.On Interacted`
  (params (Executor :type "Controller Object Reference"))
  ;[1 1 1] On interacted
  (`/Game/UltimateSurvivalPack/Blueprints/Components/BP_PlayerInventoryComponent.CLIENT Open Crafting` (`/Game/UltimateSurvivalPack/Blueprints/BFL_UMSPack.Get Inventory Component` Executor) (`self.Crafting Data Table`)))

(event `/Game/UltimateSurvivalPack/Blueprints/Interface/BPI_InventorySystem.Toggle Selected`
  (params (Toggle :type Boolean))
  (bind _staticmesh (`self.StaticMesh`))
  ;[1 1 1] On Selected
  (if Toggle
    (`PrimitiveComponent.SetRenderCustomDepth` _staticmesh true)
    (`PrimitiveComponent.SetCustomDepthStencilValue` _staticmesh 1)
    (else
      (`PrimitiveComponent.SetRenderCustomDepth` _staticmesh false)
      (`PrimitiveComponent.SetCustomDepthStencilValue` _staticmesh 0))))

(fn `Get Interaction Data`
  (returns (`Interaction Text` :type Text))
  (return (`|FormatText` "Open {name}" (`self.Name`))))

(fn `Local Can Overlap`
  (returns (Success :type Boolean))
  (return false))

(fn `UserConstructionScript`)