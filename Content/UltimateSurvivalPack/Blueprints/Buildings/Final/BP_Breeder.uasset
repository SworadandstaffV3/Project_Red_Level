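; Breeder building that periodically spawns AI animals beside itself in the survival game.
; On the server, a looping timer first fires about five seconds after BeginPlay, then every CheckTime.
; Each tick prunes invalid animals from the tracked list and spawns another if the count is at or below the maximum, so it can reach one over.
; Every spawn costs the breeder fixed internal damage to itself.
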(event `self.ReceiveBeginPlay`
  (bind _check_time_ (`self.Check Time `))
  (`/Engine/EditorBlueprintResources/ActorMacros.Switch Has Authority`
    (:`Authority`
      (`KismetSystemLibrary.K2_SetTimerDelegate` (delegate `Spawn New Animal`) _check_time_ true (+ (* _check_time_ -1.0) 5.0)))))

(event `Spawn New Animal`
  (bind (_returnvalue_roll _returnvalue_pitch _returnvalue_yaw) (`KismetMathLibrary.BreakRotator` (`self.K2_GetActorRotation`)))
  (`self.Check Animal Validity`)
  (if (<= (`KismetArrayLibrary.Array_Length` (`self.Spawned Animals`)) (`self.Maximum Spawned Animals`))
    (bind _returnvalue (`AIBlueprintHelperLibrary.SpawnAIFromClass` (`self.Animal to Spawn`) null (+ (`self.K2_GetActorLocation`) (* (`self.GetActorRightVector`) -100.0) (* (`self.GetActorUpVector`) 25.0)) (`KismetMathLibrary.MakeRotator` 0.0 0.0 _returnvalue_yaw) false null))
    (`KismetArrayLibrary.Array_AddUnique` (`self.Spawned Animals`) _returnvalue)
    (`GameplayStatics.ApplyDamage` self 30.0 null null "/Game/UltimateSurvivalPack/Blueprints/DamageType/DT_InternalDamage.DT_InternalDamage_C")))

(fn `Check Animal Validity`
  (locals (`L Animals` :type "Array of Actor Object Reference"))
  (for _array_element (`self.Spawned Animals`)
    (`/Engine/EditorBlueprintResources/StandardMacros.IsValid` _array_element
      (:`Is Valid`
        (`KismetArrayLibrary.Array_Add` (`local.L Animals`) _array_element))))
  (set `self.Spawned Animals` (`local.L Animals`))
  (return))

(fn `UserConstructionScript`)