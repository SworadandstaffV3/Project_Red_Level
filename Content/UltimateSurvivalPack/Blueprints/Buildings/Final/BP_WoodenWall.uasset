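; BP_WoodenWall is a wooden wall building piece that fits its segments to uneven ground.
; On BeginPlay, each of its five static mesh components runs DoHeightTrace.
; That function line-traces vertically against WorldStatic objects at the component's XY, around the actor's height.
; A hit sets the mesh's relative Z to the impact height; a miss resets it to zero.
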(event `self.ReceiveBeginPlay`
  (`self.Do Height Trace` (`self.StaticMesh5`))
  (`self.Do Height Trace` (`self.StaticMesh4`))
  (`self.Do Height Trace` (`self.StaticMesh3`))
  (`self.Do Height Trace` (`self.StaticMesh2`))
  (`self.Do Height Trace` (`self.StaticMesh1`)))

(fn `Do Height Trace`
  (params (Component :type "StaticMeshComponent Object Reference"))
  (returns (Return :type Boolean))
  (bind (_returnvalue_x _returnvalue_y _returnvalue_z) (`KismetMathLibrary.BreakVector` (`self.K2_GetActorLocation`)))
  (bind (_returnvalue_x_2 _returnvalue_y_2) (`KismetMathLibrary.BreakVector` (`SceneComponent.K2_GetComponentLocation` Component)))
  (bind (_relativelocation_x _relativelocation_y) (`KismetMathLibrary.BreakVector` (`SceneComponent.RelativeLocation` Component)))
  (bind _returnvalue (`KismetMathLibrary.MakeVector` _returnvalue_x_2 _returnvalue_y_2 _returnvalue_z))
  (bind (_outhit _returnvalue_2) (`KismetSystemLibrary.LineTraceSingleForObjects` :`Start` (+ _returnvalue (0.0 0.0 125.0)) :`End` (- _returnvalue (0.0 0.0 125.0)) :`ObjectTypes` (`|MakeArray` "ObjectTypeQuery1" :!type "EObjectTypeQuery Enum") :`DrawDebugType` "ForOneFrame"))
  (if _returnvalue_2
    (`SceneComponent.K2_SetRelativeLocation` Component (`KismetMathLibrary.MakeVector` _relativelocation_x _relativelocation_y (- (.z (`.ImpactPoint` (`GameplayStatics.BreakHitResult` _outhit))) (.z (`self.K2_GetActorLocation`)))) false false)
    (return true)
    (else
      (`SceneComponent.K2_SetRelativeLocation` Component (`KismetMathLibrary.MakeVector` _relativelocation_x _relativelocation_y) false false)
      (return false))))

(fn `UserConstructionScript`
  (`parent.UserConstructionScript`))