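; BP_CarSpawner is a spawner that creates a vehicle of a configurable class at its own location and yaw when a respawn is requested.
; RequestRespawn waits a brief random delay, then, if CarLimit is nonzero, spawns only while the BP_Buggy count does not exceed it; zero means no limit.
; Each vehicle gets random health and a reference back to the spawner, adjusting for collisions but always spawning.
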(event `/Game/UltimateSurvivalPack/Blueprints/Interface/BPI_Spawning.Request Respawn`
  (bind (_returnvalue_roll _returnvalue_pitch _returnvalue_yaw) (`KismetMathLibrary.BreakRotator` (`self.K2_GetActorRotation`)))
  ;[1 1 1] On requested respanw spawn car
  (`KismetSystemLibrary.Delay` (`KismetMathLibrary.RandomFloatInRange` 0.0 0.1))
  (if (!= (`self.Car Limit`) 0)
    (bind _outactors (`GameplayStatics.GetAllActorsOfClass` "/Game/UltimateSurvivalPack/Blueprints/VehicleBP/BP_Buggy.BP_Buggy_C"))
    (if (<= (`KismetArrayLibrary.Array_Length` _outactors) (`KismetMathLibrary.Conv_ByteToInt` (`self.Car Limit`)))
      (`|SpawnActorFromClass` (`self.Vehicle Class`) (`KismetMathLibrary.MakeTransform` (`self.K2_GetActorLocation`) (`KismetMathLibrary.MakeRotator` 0.0 0.0 _returnvalue_yaw)) "AdjustIfPossibleButAlwaysSpawn" "OverrideRootScale" null 30.0 3.0 "" false (`KismetMathLibrary.RandomFloatInRange` 200.0 700.0) 700.0 (-1.0 -1.0 -1.0) self null :!label _label))
    (else
      (goto _label))))

(fn `UserConstructionScript`)