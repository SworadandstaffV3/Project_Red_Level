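; Garage actor that periodically repairs a vehicle parked inside its box trigger.
; Overlap with a vehicle-interface actor claims the single slot and starts a looping timer that adds health through that interface.
; The timer stops when the health call returns false or the vehicle leaves.
; Clients destroy the box, so repair is server-only; on authority, the garage also becomes owner of its VehicleManager child actor.
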(event `self.ReceiveBeginPlay`
  (`/Engine/EditorBlueprintResources/ActorMacros.Switch Has Authority`
    (:`Authority`
      (bind _childactor (`ChildActorComponent.ChildActor` (`self.Vehicle Manager`))
        (:`then`
          (`self.SetOwner` _childactor self))
        (:`else`)))
    (:`Remote`
      (`ActorComponent.K2_DestroyComponent` (`self.Box`)))))

(event `self.Box.OnComponentBeginOverlap`
  (params (OverlappedComponent :type "PrimitiveComponent Object Reference") (OtherActor :type "Actor Object Reference") (OtherComp :type "PrimitiveComponent Object Reference") (OtherBodyIndex :type Integer) (bFromSweep :type Boolean) (SweepResult :type "HitResult Structure (by ref)"))
  (if (`KismetSystemLibrary.DoesImplementInterface` OtherActor "/Game/UltimateSurvivalPack/Blueprints/Interface/BPI_VehicleSystem.BPI_VehicleSystem_C")
    (`self.Vehicle Reference`
      (:`then`)
      (:`else`
        (set `self.Vehicle Reference` OtherActor)
        (bind _returnvalue (`KismetSystemLibrary.K2_SetTimerDelegate` (delegate `Heal Vehicle`) 10.0 true))
        (set `self.Healing Timer Handle` _returnvalue)))))

(event `Heal Vehicle`
  (bind _vehicle_reference (`self.Vehicle Reference`)
    (:`then`
      (bind _success (message `/Game/UltimateSurvivalPack/Blueprints/Interface/BPI_VehicleSystem.Add Health to Vehicle` _vehicle_reference 100.0))
      (if (not _success)
        (`KismetSystemLibrary.K2_ClearAndInvalidateTimerHandle` (`self.Healing Timer Handle`) :!label _label)))
    (:`else`)))

(event `self.Box.OnComponentEndOverlap`
  (params (OverlappedComponent :type "PrimitiveComponent Object Reference") (OtherActor :type "Actor Object Reference") (OtherComp :type "PrimitiveComponent Object Reference") (OtherBodyIndex :type Integer))
  (if (== (`self.Vehicle Reference`) OtherActor)
    (set `self.Vehicle Reference` null)
    (goto _label)))

(fn `UserConstructionScript`)