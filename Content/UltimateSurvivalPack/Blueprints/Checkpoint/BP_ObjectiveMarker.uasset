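; BP_ObjectiveMarker is a checkpoint objective marker Blueprint that hides and shows its markers based on checkpoint overlap.
; Its CheckpointOverlap event loops over the Markers array and skips invalid entries.
; On overlap it plays each visible marker's hide animation forward, and otherwise plays the same animation in reverse on hidden markers to restore them without destroying any.
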(event `self.Checkpoint Overlap`
  (params (`Overlaping?` :type Boolean))
  ;[1 1 1] On Checkpoint Overlap
  (for _array_element (`self.Markers`)
    (if `Overlaping?`
      (`/Engine/EditorBlueprintResources/StandardMacros.IsValid` _array_element
        (:`Is Valid`
          (bind _is_hidden_ (`/Game/UltimateSurvivalPack/Widget/W_Marker.Is Hidden?` _array_element))
          (if (not _is_hidden_)
            (`/Game/UltimateSurvivalPack/Widget/W_Marker.Play Hide Animation` _array_element "Forward" false))))
      (else
        (`/Engine/EditorBlueprintResources/StandardMacros.IsValid` _array_element
          (:`Is Valid`
            (if _is_hidden_
              (`/Game/UltimateSurvivalPack/Widget/W_Marker.Play Hide Animation` _array_element "Reverse" false))))))))

(fn `UserConstructionScript`
  (`parent.UserConstructionScript`))