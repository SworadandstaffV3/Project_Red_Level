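; Footstep anim notify that plays surface-based sounds and effects at a given bone, skipped on dedicated servers.
; A downward multi-trace against WorldDynamic adds a foliage rustle, while a WorldStatic trace picks the footstep cue by physical surface and leaves fading decals on snow and sand.
; The player component's water depth swaps this for splash sound and Niagara in shallow water, and horizontal speed sets the walk/sprint sound parameter.
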(fn `Foliage Hit Filter`
  (params (Hit :type "Array of HitResult Structure"))
  (returns (Foliage :type Boolean))
  (locals (`L Foliage Overlap` :type Boolean))
  (for _array_element Hit
    (if (`|EnumEquality` (`GameplayStatics.GetSurfaceType` _array_element) "SurfaceType3")
      (set `local.L Foliage Overlap` true)
      (return true)))
  (return (`local.L Foliage Overlap`)))

(fn `Received_Notify`
  (params (MeshComp :type "SkeletalMeshComponent Object Reference") (Animation :type "AnimSequenceBase Object Reference"))
  (returns (ReturnValue :type Boolean))
  (locals (`L Bone Location` :type "Vector Structure" :default (0.0 0.0 0.0)) (`L Owner` :type "Actor Object Reference") (`L Hit` :type "HitResult Structure") (`L Player Component` :type "/Game/UltimateSurvivalPack/Blueprints/Components/BP_PlayerComponent Object Reference"))
  (bind _l_hit (`local.L Hit`))
  (bind _returnvalue (`Actor.GetVelocity` (`local.L Owner`)))
  (bind (_returnvalue_roll _returnvalue_pitch _returnvalue_yaw) (`KismetMathLibrary.BreakRotator` (`Actor.K2_GetActorRotation` (`local.L Owner`))))
  (bind (_returnvalue_roll_2 _returnvalue_pitch_2 _returnvalue_yaw_2) (`KismetMathLibrary.BreakRotator` (`KismetMathLibrary.Conv_VectorToRotator` _returnvalue)))
  (if (not (`KismetSystemLibrary.IsDedicatedServer`))
    (bind _output_get (set `local.L Owner` (`ActorComponent.GetOwner` MeshComp)))
    (set `local.L Player Component` (`Actor.GetComponentByClass` _output_get "/Game/UltimateSurvivalPack/Blueprints/Components/BP_PlayerComponent.BP_PlayerComponent_C"))
    (set `local.L Bone Location` (`SceneComponent.GetSocketLocation` MeshComp (`self.Bone Name`)))
    ;[1 1 1] Spawn Foliage Sound
    (bind (_outhits _returnvalue_2) (`KismetSystemLibrary.LineTraceMultiForObjects` (`local.L Bone Location`) (- (`local.L Bone Location`) (0.0 0.0 50.0)) (`|MakeArray` "ObjectTypeQuery2" :!type "EObjectTypeQuery Enum")))
    (if _returnvalue_2
      (bind _foliage (`self.Foliage Hit Filter` _outhits))
      (if _foliage
        (`GameplayStatics.SpawnSoundAtLocation` "/Game/UltimateSurvivalPack/Demo/Audio/SFX/CUE_InFoliage.CUE_InFoliage" (`Actor.K2_GetActorLocation` (`local.L Owner`)) (struct) (`self.Volume Multiplier`) 1.0 0.0 "/Game/UltimateSurvivalPack/Blueprints/Attenuation/SA_Footsteps.SA_Footsteps" null)))
    ;[1 1 1] Spawn Footstep Sound
    (bind (_outhit _returnvalue_3) (`KismetSystemLibrary.LineTraceSingleForObjects` (`local.L Bone Location`) (- (`local.L Bone Location`) (0.0 0.0 50.0)) (`|MakeArray` "ObjectTypeQuery1" :!type "EObjectTypeQuery Enum")))
    (if _returnvalue_3
      (set `local.L Hit` _outhit)
      (`local.L Player Component`
        (:`then`
          ;;[1 0.05729 0.073] Is NOT In Water
          (if (<= (`/Game/UltimateSurvivalPack/Blueprints/Components/BP_PlayerComponent.Water Deepness` (`/Game/UltimateSurvivalPack/Blueprints/BFL_UMSPack.Get Player Component` (`local.L Owner`))) 0.0)
            (bind _returnvalue_4 (`GameplayStatics.SpawnSoundAtLocation` (select `EPhysicalSurface` (`GameplayStatics.GetSurfaceType` _outhit) :`SurfaceType_Default` "/Game/UltimateSurvivalPack/Demo/Audio/Footsteps/Default/CUE_Footsteps_Concrete.CUE_Footsteps_Concrete" :`SurfaceType1` "/Game/UltimateSurvivalPack/Demo/Audio/Footsteps/Grass/CUE_Footsteps_Grass.CUE_Footsteps_Grass" :`SurfaceType2` "/Game/UltimateSurvivalPack/Demo/Audio/Footsteps/Dirt/CUE_Footsteps_Dirt.CUE_Footsteps_Dirt" :`SurfaceType4` "/Game/UltimateSurvivalPack/Demo/Audio/Footsteps/Snow/CUE_Footsteps_Snow.CUE_Footsteps_Snow" :`SurfaceType5` "/Game/UltimateSurvivalPack/Demo/Audio/Footsteps/Snow/CUE_Footsteps_Snow.CUE_Footsteps_Snow" :!type "SoundBase Object Reference") (`local.L Bone Location`) (struct) (`self.Volume Multiplier`) (`self.Pitch Multiplier`) 0.0 "/Game/UltimateSurvivalPack/Blueprints/Attenuation/SA_Footsteps.SA_Footsteps" null :!label _label))
            (`/Engine/EditorBlueprintResources/StandardMacros.IsValid` _returnvalue_4
              (:`Is Valid`
                ;[1 1 1] Set Footstep Type Walk/Sprint
                (`AudioComponent.SetIntParameter` _returnvalue_4 "Footstep" (select `bool` (> (`KismetMathLibrary.VSizeXY` (`Actor.GetVelocity` (`local.L Owner`))) 550.0) :`true` 1))
                ;[1 1 1] Footprint Decal
                (if (`KismetArrayLibrary.Array_Contains` (`|MakeArray` "SurfaceType4" "SurfaceType5" :!type "EPhysicalSurface Enum") (`GameplayStatics.GetSurfaceType` _l_hit))
                  (bind _returnvalue_5 (`GameplayStatics.SpawnDecalAtLocation` "/Game/UltimateSurvivalPack/Demo/Material/M_Footstep.M_Footstep" (3.0 15.0 10.0) (`.ImpactPoint` (`GameplayStatics.BreakHitResult` _l_hit)) (`KismetMathLibrary.MakeRotator` 0.0 -90.0 (- (select `bool` (== _returnvalue (0.0 0.0 0.0)) :`false` _returnvalue_yaw_2 :`true` _returnvalue_yaw) 90.0))))
                  (`/Engine/EditorBlueprintResources/StandardMacros.IsValid` _returnvalue_5
                    (:`Is Valid`
                      (`DecalComponent.SetFadeOut` _returnvalue_5 15.0 1.0 false)
                      (`DecalComponent.SetFadeScreenSize` _returnvalue_5 0.005))
                    (:`Is Not Valid`
                      _))
                  (return true)
                  (else
                    (return true)))))
            (else
              ;[1 1 1] Splash Sound
              (if (`KismetMathLibrary.InRange_FloatFloat` (`/Game/UltimateSurvivalPack/Blueprints/Components/BP_PlayerComponent.Water Deepness` (`/Game/UltimateSurvivalPack/Blueprints/BFL_UMSPack.Get Player Component` (`local.L Owner`))) 0.0 0.3 false false)
                (bind _returnvalue_6 (`GameplayStatics.SpawnSoundAtLocation` "/Game/UltimateSurvivalPack/Demo/Audio/Footsteps/Water/CUE_Footsteps_Water.CUE_Footsteps_Water" (`local.L Bone Location`) (struct) (`self.Volume Multiplier`) (`self.Pitch Multiplier`) 0.0 "/Game/UltimateSurvivalPack/Blueprints/Attenuation/SA_Footsteps.SA_Footsteps" null))
                (`/Engine/EditorBlueprintResources/StandardMacros.IsValid` _returnvalue_6
                  (:`Is Valid`
                    ;[1 1 1] Set Footstep Type Walk/Sprint
                    (`AudioComponent.SetIntParameter` _returnvalue_6 "Footstep" (select `bool` (> (`KismetMathLibrary.VSizeXY` (`Actor.GetVelocity` (`local.L Owner`))) 550.0) :`true` 1))
                    ;[1 1 1] Splash Emitter
                    (`NiagaraFunctionLibrary.SpawnSystemAtLocation` "/Game/UltimateSurvivalPack/Demo/Particles/Niagara/NS_WaterSplash_Small.NS_WaterSplash_Small" (`local.L Bone Location`))))))))
        (:`else`
          (goto _label))))))