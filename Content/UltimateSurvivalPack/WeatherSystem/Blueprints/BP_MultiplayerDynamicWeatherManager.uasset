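; Multiplayer weather manager actor that runs an authority-driven day/night cycle and chance-weighted random weather from a data table.
; A timeline blends current and next weather rows.
; Each tick, that blend and sun-angle curves drive sun, skylight, fog, clouds, sky sphere, day/night audio and a material parameter collection.
; Interface messages announce rain and weather changes to actors (weather also to widgets), while rainy thunder weathers spawn line-traced lightning.
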(fn `Day/Night Cycle`
  (bind _returnvalue (+ (`self.Current Time`) (/ (* (`GameplayStatics.GetWorldDeltaSeconds`) 20.0) (select `bool` (> (.z (`self.GetActorForwardVector` (`self.Sun light`))) 0.0) :`false` (/ (`self.Day Length`) 2.0) :`true` (/ (`self.Night Length`) 2.0)))))
  (`/Engine/EditorBlueprintResources/ActorMacros.Switch Has Authority`
    (:`Authority`
      (if (`self.Animate Day/Night Cycle`)
        (if (> _returnvalue 2400.0)
          ;[1 0.5365 0.5365] Reset Day
          (set `self.Current Time` 0.0)
          (else
            (set `self.Current Time` (`KismetMathLibrary.SelectFloat` 2400.0 _returnvalue (< _returnvalue 0.0)))))))))

(fn `Get Sun Angle Value`
  (returns (ReturnValue :type "Float (double-precision)"))
  (return (`KismetMathLibrary.MapRangeClamped` (.z (`self.GetActorForwardVector` (`self.Sun light`))) -1.0 1.0 1.0)))

(fn `Pick Random Weather`
  (returns (`Weather Row` :type Integer) (`Weather Name` :type Name))
  (locals (`Picked Weather Name` :type Name) (`Picked Weather` :type Integer))
  (bind _weathers (`self.Weathers`))
  (bind _output_get (set `local.Picked Weather` (`KismetMathLibrary.RandomIntegerInRange` 0 (- (`KismetArrayLibrary.Array_Length` _weathers) 1)) :!label _label))
  (bind _output_get_2 (set `local.Picked Weather Name` (`|GetArrayItem` _weathers _output_get)))
  (bind _returnvalue (`|GetDataTableRow` (`self.Weather Data Table`) _output_get_2)
    (:`then`
      (if (>= (`.Chance_6_E81598554F12B0ECF9B480994E6D83FE` (break `/Game/UltimateSurvivalPack/WeatherSystem/Blueprints/Structures/S_Weather` _returnvalue)) (`KismetMathLibrary.RandomFloatInRange` 1e-06 1.0))
        (return (`local.Picked Weather`) (`local.Picked Weather Name`))
        (else
          (goto _label))))))

(fn `Set Audio Elements`
  (bind _night_sound (`self.Night Sound`))
  (bind _returnvalue (`CurveFloat.GetFloatValue` (`self.Audio Curve`) (`self.Get Sun Angle Value`)))
  ;[1 1 1] Set Day Volume
  (`AudioComponent.SetVolumeMultiplier` (`self.Day Sound`) _returnvalue)
  ;[1 1 1] Set Night Volume
  (`AudioComponent.SetVolumeMultiplier` _night_sound (- 1.0 _returnvalue))
  ;[1 0.2604 0.2604] Disable Crickets Sound at Winter
  (`AudioComponent.SetFloatParameter` _night_sound "Cricket Sound" (`self.Switch on Session FLOAT` 1.0 1.0 1.0)))

(fn `Set Elements`
  (bind _sky_light (`self.Sky light`))
  (bind _weather_data_table (`self.Weather Data Table`))
  (bind _sky_sphere (`self.Sky sphere`))
  (bind _volumetric_clouds (`self.Volumetric Clouds`))
  (bind _exponencial_fog (`self.Exponencial Fog`))
  (bind _sun_light (`self.Sun light`))
  (bind _returnvalue (`CurveLinearColor.GetLinearColorValue` (`self.Sun Color Curve`) (`self.Get Sun Angle Value`)))
  (bind (_returnvalue_x _returnvalue_y) (`KismetMathLibrary.BreakVector` (`self.K2_GetActorLocation` _exponencial_fog)))
  (bind _returnvalue_2 (select `/Game/UltimateSurvivalPack/WeatherSystem/Blueprints/Enumeration/E_Shader_Type` (`self.Shader Type`) :`NewEnumerator0` true))
  (bind _component (`ExponentialHeightFog.Component` _exponencial_fog))
  (bind _lightcomponent (`Light.LightComponent` _sun_light))
  (bind _asdirectional_light_component (cast `DirectionalLightComponent` (`Actor.RootComponent` _sun_light) :!pure true))
  (bind _returnvalue_3 (`|GetDataTableRow` _weather_data_table (`|GetArrayItem` (`self.Weathers`) (`self.Actual Weather`)))
    (:`then`
      (bind _returnvalue_4 (`|GetDataTableRow` _weather_data_table (`|GetArrayItem` (`self.Weathers`) (`self.Next Weather`)))
        (:`then`
          ;[0 0 0] Setting FOG elements
          (`/Engine/EditorBlueprintResources/StandardMacros.IsValid` _exponencial_fog
            (:`Is Valid`
              (bind (_fog_fogdensity _fog_fogheigh _fog_fogdaycolor _fog_fognightcolor) (break `/Game/UltimateSurvivalPack/WeatherSystem/Blueprints/Structures/S_Fog` (break `/Game/UltimateSurvivalPack/WeatherSystem/Blueprints/Structures/S_Season_Settings` (`.Weather_29_5A3E01714F3985C9D9080E96ED878B73` (break `/Game/UltimateSurvivalPack/WeatherSystem/Blueprints/Structures/S_Weather` _returnvalue_3)))))
              (bind (_fog_fogdensity_2 _fog_fogheigh_2 _fog_fogdaycolor_2 _fog_fognightcolor_2) (break `/Game/UltimateSurvivalPack/WeatherSystem/Blueprints/Structures/S_Fog` (break `/Game/UltimateSurvivalPack/WeatherSystem/Blueprints/Structures/S_Season_Settings` (`.Weather_29_5A3E01714F3985C9D9080E96ED878B73` (break `/Game/UltimateSurvivalPack/WeatherSystem/Blueprints/Structures/S_Weather` _returnvalue_4)))))
              (`ExponentialHeightFogComponent.SetFogDensity` _component (`self.Blend Between Weathers FLOAT` _fog_fogdensity _fog_fogdensity_2))
              (`self.K2_SetActorLocation` _exponencial_fog (`KismetMathLibrary.MakeVector` _returnvalue_x _returnvalue_y (`self.Blend Between Weathers FLOAT` _fog_fogheigh _fog_fogheigh_2)) false false)
              (`ExponentialHeightFogComponent.SetFogInscatteringColor` _component (`KismetMathLibrary.LinearColorLerp` (`self.Blend Between Weathers COLOR` _fog_fogdaycolor _fog_fogdaycolor_2) (`self.Blend Between Weathers COLOR` _fog_fognightcolor _fog_fognightcolor_2) (`self.Switch On Day/Night` 0.0 1.0 (`self.Day/Night Curve Smooth`)))))
            (:`Is Not Valid`
              _))
          ;[0 0 0] Setting SUN elements
          (`/Engine/EditorBlueprintResources/StandardMacros.IsValid` _sun_light
            (:`Is Valid`
              (`LightComponent.SetLightColor` _lightcomponent _returnvalue true)
              (`LightComponent.SetBloomTint` _lightcomponent (`KismetMathLibrary.Conv_LinearColorToColor` _returnvalue))
              (bind (_sun_sunintensity _sun_sunshaftbloomscale _sun_lightshaftocclusiondarkness) (break `/Game/UltimateSurvivalPack/WeatherSystem/Blueprints/Structures/S_Sun` (break `/Game/UltimateSurvivalPack/WeatherSystem/Blueprints/Structures/S_Season_Settings` (`.Weather_29_5A3E01714F3985C9D9080E96ED878B73` (break `/Game/UltimateSurvivalPack/WeatherSystem/Blueprints/Structures/S_Weather` _returnvalue_3)))))
              (bind (_sun_sunintensity_2 _sun_sunshaftbloomscale_2 _sun_lightshaftocclusiondarkness_2) (break `/Game/UltimateSurvivalPack/WeatherSystem/Blueprints/Structures/S_Sun` (break `/Game/UltimateSurvivalPack/WeatherSystem/Blueprints/Structures/S_Season_Settings` (`.Weather_29_5A3E01714F3985C9D9080E96ED878B73` (break `/Game/UltimateSurvivalPack/WeatherSystem/Blueprints/Structures/S_Weather` _returnvalue_4)))))
              (`LightComponent.SetIntensity` _lightcomponent (`self.Switch On Day/Night` (`self.Blend Between Weathers FLOAT` _sun_sunintensity _sun_sunintensity_2) 0.0 (`self.Day/Night Curve`)))
              ;;[1 0.5208 0.5208] Set Light Shaft Bloom
              (if (`LightComponent.bEnableLightShaftBloom` _lightcomponent)
                (`LightComponent.SetBloomScale` _lightcomponent (`self.Switch On Day/Night` (`self.Blend Between Weathers FLOAT` _sun_sunshaftbloomscale _sun_sunshaftbloomscale_2) 0.0 (`self.Day/Night Curve`))))
              ;;[1 0.7257 0.3557] Light Shaft Occlusion
              (if (`DirectionalLightComponent.bEnableLightShaftOcclusion` _asdirectional_light_component)
                (`DirectionalLightComponent.SetOcclusionMaskDarkness` _asdirectional_light_component (`self.Switch On Day/Night` (`self.Blend Between Weathers FLOAT` _sun_lightshaftocclusiondarkness _sun_lightshaftocclusiondarkness_2) 1.0 (`self.Day/Night Curve`)))))
            (:`Is Not Valid`
              _))
          ;[0 0 0] Setting SKYLIGHT elements
          (`/Engine/EditorBlueprintResources/StandardMacros.IsValid` _sky_light
            (:`Is Valid`
              (bind (_skylight_skylightdayintensity _skylight_skylightnightintensity) (break `/Game/UltimateSurvivalPack/WeatherSystem/Blueprints/Structures/S_Skylight` (break `/Game/UltimateSurvivalPack/WeatherSystem/Blueprints/Structures/S_Season_Settings` (`.Weather_29_5A3E01714F3985C9D9080E96ED878B73` (break `/Game/UltimateSurvivalPack/WeatherSystem/Blueprints/Structures/S_Weather` _returnvalue_3)))))
              (bind (_skylight_skylightdayintensity_2 _skylight_skylightnightintensity_2) (break `/Game/UltimateSurvivalPack/WeatherSystem/Blueprints/Structures/S_Skylight` (break `/Game/UltimateSurvivalPack/WeatherSystem/Blueprints/Structures/S_Season_Settings` (`.Weather_29_5A3E01714F3985C9D9080E96ED878B73` (break `/Game/UltimateSurvivalPack/WeatherSystem/Blueprints/Structures/S_Weather` _returnvalue_4)))))
              (`SkyLightComponent.SetIntensity` (`SkyLight.LightComponent` _sky_light) (`self.Switch On Day/Night` (`self.Blend Between Weathers FLOAT` _skylight_skylightdayintensity _skylight_skylightdayintensity_2) (`self.Blend Between Weathers FLOAT` _skylight_skylightnightintensity _skylight_skylightnightintensity_2) (`self.Skyligth Curve`))))
            (:`Is Not Valid`
              _))
          ;[0 0 0] Setting SKY elements
          (`/Engine/EditorBlueprintResources/StandardMacros.IsValid` _sky_sphere
            (:`Is Valid`
              ;;[1 1 1] Refresh Settings
              (`/Engine/EngineSky/BP_Sky_Sphere.RefreshMaterial` _sky_sphere))
            (:`Is Not Valid`
              _))
          (`/Engine/EditorBlueprintResources/StandardMacros.IsValid` _volumetric_clouds
            (:`Is Valid`
              (bind _returnvalue_5 (`self.Blend Between Weathers FLOAT` (`.CloudDensity_8_B1670AED478D1409362A49922CE1DAF9` (break `/Game/UltimateSurvivalPack/WeatherSystem/Blueprints/Structures/S_Sky` (`.Sky_19_3B4D9DAA4E47B3166336C98CE0CED70A` (break `/Game/UltimateSurvivalPack/WeatherSystem/Blueprints/Structures/S_Season_Settings` (`.Weather_29_5A3E01714F3985C9D9080E96ED878B73` (break `/Game/UltimateSurvivalPack/WeatherSystem/Blueprints/Structures/S_Weather` _returnvalue_3)))))) (`.CloudDensity_8_B1670AED478D1409362A49922CE1DAF9` (break `/Game/UltimateSurvivalPack/WeatherSystem/Blueprints/Structures/S_Sky` (`.Sky_19_3B4D9DAA4E47B3166336C98CE0CED70A` (break `/Game/UltimateSurvivalPack/WeatherSystem/Blueprints/Structures/S_Season_Settings` (`.Weather_29_5A3E01714F3985C9D9080E96ED878B73` (break `/Game/UltimateSurvivalPack/WeatherSystem/Blueprints/Structures/S_Weather` _returnvalue_4))))))))
              ;;[1 1 1] Set Cloud Density
              (`MaterialInstanceDynamic.SetScalarParameterValue` (`self.Volumetric Cloud Dynamic Material`) "Density" _returnvalue_5)
              ;;[1 1 1] Turn Off Clouds On Sky Box And Use Volumetric if Shader = Computer
              (`SceneComponent.SetVisibility` (`VolumetricCloud.VolumetricCloudComponent` _volumetric_clouds) _returnvalue_2 false)
              (`self.SetActorHiddenInGame` _volumetric_clouds (not _returnvalue_2)))
            (:`Is Not Valid`
              _))
          (set `/Engine/EngineSky/BP_Sky_Sphere.Cloud opacity` (* _returnvalue_5 15.0) _sky_sphere)
          ;;[1 1 1] Refresh Settings
          (`/Engine/EngineSky/BP_Sky_Sphere.RefreshMaterial` _sky_sphere)
          ;[0 0 0] Setting Rain Phase
          (set `self.Rain phase` (`self.Blend Between Weathers FLOAT` (`.RainPhase_21_1CA427C74D227035CEFDF8AF180E9159` (break `/Game/UltimateSurvivalPack/WeatherSystem/Blueprints/Structures/S_Weather` _returnvalue_3)) (`.RainPhase_21_1CA427C74D227035CEFDF8AF180E9159` (break `/Game/UltimateSurvivalPack/WeatherSystem/Blueprints/Structures/S_Weather` _returnvalue_4))))
          ;[0 0 0] Setting Parameter Collection For Materials
          (`self.Set Parameter Collections`))))))

(fn `Set Light Rotation`
  (bind _returnvalue (`KismetMathLibrary.MakeRotator` 0.0 (`self.Sun Inclination`)))
  (`self.K2_SetActorRotation` (`self.Sun light`) (`KismetMathLibrary.Conv_VectorToRotator` (`KismetMathLibrary.RotateAngleAxis` (`KismetMathLibrary.RotateAngleAxis` (`KismetMathLibrary.GreaterGreater_VectorRotator` (0.0 0.0 1.0) _returnvalue) (`self.Sun Rotation`) (0.0 0.0 1.0)) (`KismetMathLibrary.MapRangeUnclamped` (`self.Current Time`) 0.0 2400.0 0.0 360.0) (`KismetMathLibrary.RotateAngleAxis` (`KismetMathLibrary.GreaterGreater_VectorRotator` (1.0 0.0 0.0) _returnvalue) (`self.Sun Rotation`) (0.0 0.0 1.0)))) false))

(fn `Set Parameter Collections`
  ;[1 1 1] Set Rain Phase
  (`KismetMaterialLibrary.SetScalarParameterValue` "/Game/UltimateSurvivalPack/ParameterCollection/MPC_DynamicWeatherSystem.MPC_DynamicWeatherSystem" "Rain phase" (`self.Rain phase`))
  ;[1 1 1] Setting Season Phase
  (`KismetMaterialLibrary.SetScalarParameterValue` "/Game/UltimateSurvivalPack/ParameterCollection/MPC_DynamicWeatherSystem.MPC_DynamicWeatherSystem" "Season")
  (bind (_next_weather _actual_weather) (`self.Get DataTable Values` (`self.Weather Data Table`))
    (:`Success`
      (bind _wind_windintensity (break `/Game/UltimateSurvivalPack/WeatherSystem/Blueprints/Structures/S_Wind` (break `/Game/UltimateSurvivalPack/WeatherSystem/Blueprints/Structures/S_Season_Settings` (`.Weather_29_5A3E01714F3985C9D9080E96ED878B73` (break `/Game/UltimateSurvivalPack/WeatherSystem/Blueprints/Structures/S_Weather` _actual_weather)))))
      (bind _wind_windintensity_2 (break `/Game/UltimateSurvivalPack/WeatherSystem/Blueprints/Structures/S_Wind` (break `/Game/UltimateSurvivalPack/WeatherSystem/Blueprints/Structures/S_Season_Settings` (`.Weather_29_5A3E01714F3985C9D9080E96ED878B73` (break `/Game/UltimateSurvivalPack/WeatherSystem/Blueprints/Structures/S_Weather` _next_weather)))))
      (`KismetMaterialLibrary.SetScalarParameterValue` "/Game/UltimateSurvivalPack/ParameterCollection/MPC_DynamicWeatherSystem.MPC_DynamicWeatherSystem" "Wind Intensity" (`self.Blend Between Weathers FLOAT` _wind_windintensity _wind_windintensity_2))
      ;[1 1 1] Setting Ground Wetness
      (`KismetMaterialLibrary.SetScalarParameterValue` "/Game/UltimateSurvivalPack/ParameterCollection/MPC_DynamicWeatherSystem.MPC_DynamicWeatherSystem" "Ground Wetness" (`self.Blend Between Weathers FLOAT` (`.GroundWetness_27_40C2ADBB4142FBAF30EDEAA9C97EE11B` (break `/Game/UltimateSurvivalPack/WeatherSystem/Blueprints/Structures/S_Weather` _actual_weather)) (`.GroundWetness_27_40C2ADBB4142FBAF30EDEAA9C97EE11B` (break `/Game/UltimateSurvivalPack/WeatherSystem/Blueprints/Structures/S_Weather` _next_weather)))))))

(fn `Switch On Day/Night`
  (params (Day :type "Float (double-precision)") (Night :type "Float (double-precision)") (`Alpha Curve` :type "CurveFloat Object Reference"))
  (returns (ReturnValue :type "Float (double-precision)"))
  (return (`KismetMathLibrary.Lerp` Night Day (`KismetMathLibrary.FClamp` (`CurveFloat.GetFloatValue` `Alpha Curve` (`self.Get Sun Angle Value`))))))

(fn `UserConstructionScript`
  ;[0 0 0] In Editor Events
  (`|ExecutionSequence`
    (:`then_0`
      (bind _outrownames (`DataTableFunctionLibrary.GetDataTableRowNames` "/Game/UltimateSurvivalPack/WeatherSystem/Blueprints/DT_Weather.DT_Weather"))
      (set `self.Weathers` _outrownames)
      (if (< (- (`KismetArrayLibrary.Array_Length` (`self.Weathers`)) 1) (`self.Actual Weather`))
        (bind _output_get (set `self.Actual Weather` 0)))
      (set `self.Next Weather` _output_get))
    (:`then_1`
      (bind _returnvalue (`KismetMaterialLibrary.CreateDynamicMaterialInstance` "/Game/UltimateSurvivalPack/WeatherSystem/Materials/Clouds/M_VolumetricClouds.M_VolumetricClouds"))
      (bind _output_get_2 (set `self.Volumetric Cloud Dynamic Material` _returnvalue))
      (`/Engine/EditorBlueprintResources/StandardMacros.IsValid` (`self.Volumetric Clouds`)
        (:`Is Valid`
          (`VolumetricCloudComponent.SetMaterial` (`VolumetricCloud.VolumetricCloudComponent` (`self.Volumetric Clouds`)) _output_get_2))))
    (:`then_3`)
    (:`then_4`
      (`self.Set Light Rotation`)
      (`self.Set Elements`)
      (`self.Calling Event On Rain`)
      (`self.Set Parameter Collections`)
      (`self.Set Audio Elements`))
    (:`then_5`
      ;;[1 1 1] Update Tick Interval
      (`self.SetActorTickInterval` (`self.Update Tick Interval`)))))